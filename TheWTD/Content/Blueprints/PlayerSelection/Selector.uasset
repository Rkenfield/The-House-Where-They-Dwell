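; Selector actor for a player selection screen, a marker labelled with its player number that moves between four slots.
; A/D keys or gamepad left stick step the Selection index with wraparound, repositioning the actor along Y from its starting location.
; Selecting and Selected events unlock or lock movement and swap the marker's material to show its state.
; The construction script writes PlayerNo to the text label.
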(event Custom|Selecting
  ;[1 1 1] Sets material for selector when it is in the selecting state.
  (Variables|Default|SetCanMove true)
  (Rendering|Material|SetMaterial (Variables|Default|GetSelector1) 0 "/Engine/EditorMaterials/Cloth/CameraLitDoubleSided.CameraLitDoubleSided"))

(event Custom|Selected
  ;[1 1 1] Sets material for the selector when it is in the selected state.
  (Variables|Default|SetCanMove false)
  (Rendering|Material|SetMaterial (Variables|Default|GetSelector1) 0 "/Engine/EngineDebugMaterials/VertexColorViewMode_GreenOnly.VertexColorViewMode_GreenOnly"))

(event EventBeginPlay
  ;[1 1 1] Sets the initial position of the selector based on the selection value
  (bind _output_get (Variables|Default|SetInitialLocation (Transformation|GetActorLocation)))
  (Transformation|SetActorLocation (Math|Vector|MakeVector (.x _output_get) (- (.y _output_get) (* (Variables|Default|GetSelection) 1.4e+02)) (.z _output_get)) false false))

(event Input|KeyboardEvents|D
  (params (Key :type Key%20Structure :default "None"))
  (bind _initiallocation (Variables|Default|GetInitialLocation))
  ;[1 1 1] Moving Selector Right and circling back to the beginning after selection value > 3
  (:Pressed
    (if (Variables|Default|GetCanMove)
      (bind _output_get (Variables|Default|SetSelection (+ (Variables|Default|GetSelection) 1)))
      (if (> _output_get 3)
        (Variables|Default|SetSelection 0))
      (Transformation|SetActorLocation (Math|Vector|MakeVector (.x _initiallocation) (- (.y _initiallocation) (* (Variables|Default|GetSelection) 1.4e+02)) (.z _initiallocation)) false false))))

(event Input|GamepadEvents|GamepadLeftStickRight
  (params (Key :type Key%20Structure :default "None"))
  (bind _initiallocation (Variables|Default|GetInitialLocation))
  ;[1 1 1] Moving Selector Right and circling back to the beginning after selection value > 3
  (:Pressed
    (if (Variables|Default|GetCanMove)
      (bind _output_get (Variables|Default|SetSelection (+ (Variables|Default|GetSelection) 1)))
      (if (> _output_get 3)
        (Variables|Default|SetSelection 0))
      (Transformation|SetActorLocation (Math|Vector|MakeVector (.x _initiallocation) (- (.y _initiallocation) (* (Variables|Default|GetSelection) 1.4e+02)) (.z _initiallocation)) false false))))

(event Input|KeyboardEvents|A
  (params (Key :type Key%20Structure :default "None"))
  (bind _initiallocation (Variables|Default|GetInitialLocation))
  ;[1 1 1] Moving Left and circling back to the end when selection value < 0
  (:Pressed
    (if (Variables|Default|GetCanMove)
      (bind _output_get (Variables|Default|SetSelection (- (Variables|Default|GetSelection) 1)))
      (if (< _output_get 0)
        (Variables|Default|SetSelection 3))
      (Transformation|SetActorLocation (Math|Vector|MakeVector (.x _initiallocation) (- (.y _initiallocation) (* (Variables|Default|GetSelection) 1.4e+02)) (.z _initiallocation)) false false))))

(event Input|GamepadEvents|GamepadLeftStickLeft
  (params (Key :type Key%20Structure :default "None"))
  (bind _initiallocation (Variables|Default|GetInitialLocation))
  ;[1 1 1] Moving Left and circling back to the end when selection value < 0
  (:Pressed
    (if (Variables|Default|GetCanMove)
      (bind _output_get (Variables|Default|SetSelection (- (Variables|Default|GetSelection) 1)))
      (if (< _output_get 0)
        (Variables|Default|SetSelection 3))
      (Transformation|SetActorLocation (Math|Vector|MakeVector (.x _initiallocation) (- (.y _initiallocation) (* (Variables|Default|GetSelection) 1.4e+02)) (.z _initiallocation)) false false))))

(fn ConstructionScript
  (Rendering|Components|TextRender|SetText (Variables|Default|GetTextRender1) (Utilities|Text|ToText(Integer) (Variables|Default|GetPlayerNo))))