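; Player controller for the character selection screen, handling join, pick and cancel input for each player.
; Join and confirm go through GM_Selection, with a confirm accepted only if no CharacterIndex entry in the game instance matches the Selector pawn's choice.
; Q clears the player's CharacterIndex slot, reactivates selecting and decrements SelectionCount.
; Gamepad right face button does the same but skips clearing the slot.
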(event Input|ActionEvents|InputActionJoinGame
  (params (Key :type Key%20Structure :default "None"))
  ;[1 1 1] Join Game Input
  (:Pressed
    (bind _asgm_selection (Utilities|Casting|CastToGM_Selection (Game|GetGameMode)))
    (Default|Join _asgm_selection self)))

(event Input|ActionEvents|InputActionInteract
  (params (Key :type Key%20Structure :default "None"))
  (bind _returnvalue (Pawn|GetControlledPawn))
  ;[1 1 1] Checking if player selection has not been made by another player and then assigns selection to player.
  (:Pressed
    (bind _asselector (Utilities|Casting|CastToSelector _returnvalue))
    (bind _asgame_instance_the_wtd (Utilities|Casting|CastToGameInstance_TheWTD (Game|GetGameInstance)))
    (Variables|Default|SetValidSelection true)
    (bind _array_element (Utilities|Array|ForEachLoopwithBreak (Variables|/Game/Blueprints/GameInstance_TheWTD.GameInstance_TheWTD_C|GetCharacterIndex _asgame_instance_the_wtd) :!label _label)
      (:LoopBody
        (if (== _array_element (Variables|/Game/Blueprints/PlayerSelection/Selector.Selector_C|GetSelection _asselector))
          (Variables|Default|SetValidSelection false)
          (goto _label Break)))
      (:Completed
        (if (Variables|Default|GetValidSelection)
          (bind _asselector_2 (Utilities|Casting|CastToSelector _returnvalue))
          (Default|Selected _asselector_2)
          (bind _asgm_selection (Utilities|Casting|CastToGM_Selection (Game|GetGameMode)))
          (Default|Selection _asgm_selection self (Variables|/Game/Blueprints/PlayerSelection/Selector.Selector_C|GetSelection _asselector_2)))))))

(event Input|KeyboardEvents|Q
  (params (Key :type Key%20Structure :default "None"))
  ;[1 1 1] Remove Selection.
  (:Pressed
    (bind _asgame_instance_the_wtd (Utilities|Casting|CastToGameInstance_TheWTD (Game|GetGameInstance)))
    (Utilities|Array|SetArrayElem (Variables|/Game/Blueprints/GameInstance_TheWTD.GameInstance_TheWTD_C|GetCharacterIndex _asgame_instance_the_wtd) (Class|GameplayStatics|GetPlayerControllerID self) -1)
    (bind _asselector (Utilities|Casting|CastToSelector (Pawn|GetControlledPawn)))
    (Default|Selecting _asselector)
    (bind _asgm_selection (Utilities|Casting|CastToGM_Selection (Game|GetGameMode)))
    (Variables|/Game/Blueprints/PlayerSelection/GM_Selection.GM_Selection_C|SetSelectionCount _asgm_selection (- (Variables|/Game/Blueprints/PlayerSelection/GM_Selection.GM_Selection_C|GetSelectionCount _asgm_selection) 1))))

(event Input|GamepadEvents|GamepadFaceButtonRight
  (params (Key :type Key%20Structure :default "None"))
  ;[1 1 1] Remove Selection.
  (:Pressed
    (bind _asselector (Utilities|Casting|CastToSelector (Pawn|GetControlledPawn)))
    (Default|Selecting _asselector)
    (bind _asgm_selection (Utilities|Casting|CastToGM_Selection (Game|GetGameMode)))
    (Variables|/Game/Blueprints/PlayerSelection/GM_Selection.GM_Selection_C|SetSelectionCount _asgm_selection (- (Variables|/Game/Blueprints/PlayerSelection/GM_Selection.GM_Selection_C|GetSelectionCount _asgm_selection) 1))))

(fn ConstructionScript)