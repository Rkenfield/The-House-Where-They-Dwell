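; Purple syringe consumable item that heals the character who uses it.
; Its UseItem override adds a fixed amount to the user's Health, clamps it at a hardcoded maximum, then returns the result of the parent UseItem.
; The event graph holds only disabled default events, and the construction script just calls the parent.
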(event EventBeginPlay
  (|CallParentFunction) ; This node is disabled and will not be called.\nDrag off pins to build functionality.
)

(event Collision|EventActorBeginOverlap
  (params (OtherActor :type Actor%20Object%20Reference))
  (|CallParentFunction OtherActor) ; This node is disabled and will not be called.\nDrag off pins to build functionality.
)

(event EventTick
  (params (DeltaSeconds :type Float%20%28single-precision%29))
  (|CallParentFunction DeltaSeconds) ; This node is disabled and will not be called.\nDrag off pins to build functionality.
)

(fn ConstructionScript
  (|CallParentFunction))

(fn UseItem
  (params (User :type Third%20Person%20Character%20Object%20Reference))
  (bind _output_get (Variables|/Game/Blueprints/Characters/ThirdPersonCharacter.ThirdPersonCharacter_C|SetHealth User (+ (Variables|/Game/Blueprints/Characters/ThirdPersonCharacter.ThirdPersonCharacter_C|GetHealth User) 25.0)))
  (if (>= _output_get 1e+02)
    (Variables|/Game/Blueprints/Characters/ThirdPersonCharacter.ThirdPersonCharacter_C|SetHealth User 1e+02))
  (bind _success (|CallParentFunction User))
  (return _success))