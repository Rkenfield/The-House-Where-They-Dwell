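; Throwable chest armor item Blueprint that applies a passive change to its user's Damage value, likely as armor damage reduction.
; PassiveEffect calls the parent, prints a debug string and halves Damage from its 1.0 baseline by direct assignment.
; RemovePassive calls the parent and resets Damage to that baseline, overwriting any other modifier.
; The event graph holds only disabled stub events.
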(event EventBeginPlay
  (|CallParentFunction) ; This node is disabled and will not be called.\nDrag off pins to build functionality.
)

(event Collision|EventActorBeginOverlap
  (params (OtherActor :type Actor%20Object%20Reference))
  (|CallParentFunction OtherActor) ; This node is disabled and will not be called.\nDrag off pins to build functionality.
)

(event EventTick
  (params (DeltaSeconds :type Float%20%28single-precision%29))
  (|CallParentFunction DeltaSeconds) ; This node is disabled and will not be called.\nDrag off pins to build functionality.
)

(fn ConstructionScript
  (|CallParentFunction))

(fn PassiveEffect
  (params (User :type Third%20Person%20Character%20Object%20Reference))
  (bind _success (|CallParentFunction 0))
  (Development|PrintString "Passive")
  (Variables|/Game/Blueprints/Characters/ThirdPersonCharacter.ThirdPersonCharacter_C|SetDamage User 0.5)
  (return _success))

(fn RemovePassive
  (params (User :type Third%20Person%20Character%20Object%20Reference))
  (|CallParentFunction 0)
  (Variables|/Game/Blueprints/Characters/ThirdPersonCharacter.ThirdPersonCharacter_C|SetDamage User 1.0))