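; BP_Item_NonInventory is an item Blueprint whose passive effect sets the Pregnant Ghost hunting the item's user.
; Its PassiveEffect override finds the Pregnant_Ghost_AIC controller, sets the User as Prey on its controlled ghost pawn, then calls HuntPhase on the controller.
; The parent passive effect runs afterward, only when the pawn cast succeeds.
; The event graph and construction script add no logic of their own.
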(event EventBeginPlay)

(event Collision|EventActorBeginOverlap
  (params (OtherActor :type Actor%20Object%20Reference)))

(event EventTick
  (params (DeltaSeconds :type Float%20%28single-precision%29))
  (|CallParentFunction DeltaSeconds) ; This node is disabled and will not be called.\nDrag off pins to build functionality.
)

(fn ConstructionScript
  (|CallParentFunction))

(fn PassiveEffect
  (params (User :type Third%20Person%20Character%20Object%20Reference))
  (bind _returnvalue (Actor|GetActorOfClass "/Game/Blueprints/AI/Pregnant_Ghost/Pregnant_Ghost_AIC.Pregnant_Ghost_AIC_C"))
  (if (.bSuccess (Utilities|Casting|CastToPregnant_Ghost (Pawn|GetControlledPawn _returnvalue)))
    (Variables|/Game/Blueprints/AI/Pregnant_Ghost/Pregnant_Ghost.Pregnant_Ghost_C|SetPrey (.AsPregnant%20Ghost (Utilities|Casting|CastToPregnant_Ghost (Pawn|GetControlledPawn _returnvalue))) User)
    (Default|HuntPhase _returnvalue)
    (bind _success (|CallParentFunction 0))
    (return _success)))