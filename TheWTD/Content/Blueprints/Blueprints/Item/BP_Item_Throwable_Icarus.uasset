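; BP_Item_Throwable_Icarus is a throwable item that teleports its user to the point where it hits.
; UseItem stores the user, then defers to the parent implementation.
; When the static mesh hits while IsThrown is set, a DoOnce clears the flag, records the hit location and moves the user there with no sweep.
; The DoOnce has no reset, so the teleport fires once per item instance.
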(event OnComponentHit(StaticMesh)
  (params (HitComponent :type Primitive%20Component%20Object%20Reference) (OtherActor :type Actor%20Object%20Reference) (OtherComp :type Primitive%20Component%20Object%20Reference) (NormalImpulse :type Vector :default "0, 0, 0") (Hit :type Hit%20Result%20Structure%20%28by%20ref%29))
  (if (Variables|Default|GetIsThrown)
    (Utilities|FlowControl|DoOnce false
      (:Completed
        (Variables|Default|SetIsThrown false)
        (bind _output_get (Variables|Default|SetThrowLocation (.location Hit)))
        (Transformation|SetActorLocation (Variables|Default|GetUser) _output_get false true)))))

(event EventBeginPlay
  (|CallParentFunction) ; This node is disabled and will not be called.\nDrag off pins to build functionality.
)

(event Collision|EventActorBeginOverlap
  (params (OtherActor :type Actor%20Object%20Reference))
  (|CallParentFunction OtherActor) ; This node is disabled and will not be called.\nDrag off pins to build functionality.
)

(event EventTick
  (params (DeltaSeconds :type Float%20%28single-precision%29))
  (|CallParentFunction DeltaSeconds) ; This node is disabled and will not be called.\nDrag off pins to build functionality.
)

(fn ConstructionScript
  (|CallParentFunction))

(fn UseItem
  (params (User :type Third%20Person%20Character%20Object%20Reference))
  (Variables|Default|SetUser User)
  (bind _success (|CallParentFunction User))
  (return _success))