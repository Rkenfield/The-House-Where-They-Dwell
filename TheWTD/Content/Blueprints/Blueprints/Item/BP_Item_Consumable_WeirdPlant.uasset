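; BP_Item_Consumable_WeirdPlant is a consumable plant item that boosts the throw stat of the character who uses it.
; Its UseItem override adds a large fixed amount to the user's Throw value, then returns the parent item's UseItem result.
; The event graph and construction script add no behavior of their own.
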(event EventBeginPlay
  (|CallParentFunction) ; This node is disabled and will not be called.\nDrag off pins to build functionality.
)

(event Collision|EventActorBeginOverlap
  (params (OtherActor :type Actor%20Object%20Reference))
  (|CallParentFunction OtherActor) ; This node is disabled and will not be called.\nDrag off pins to build functionality.
)

(event EventTick
  (params (DeltaSeconds :type Float%20%28single-precision%29))
  (|CallParentFunction DeltaSeconds) ; This node is disabled and will not be called.\nDrag off pins to build functionality.
)

(fn ConstructionScript
  (|CallParentFunction))

(fn UseItem
  (params (User :type Third%20Person%20Character%20Object%20Reference))
  (Variables|/Game/Blueprints/Characters/ThirdPersonCharacter.ThirdPersonCharacter_C|SetThrow User (+ (Variables|/Game/Blueprints/Characters/ThirdPersonCharacter.ThirdPersonCharacter_C|GetThrow User) 1e+03))
  (bind _success (|CallParentFunction 0))
  (return _success))