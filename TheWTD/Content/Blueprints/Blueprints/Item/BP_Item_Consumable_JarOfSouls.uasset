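; Jar of Souls consumable item that releases one random soul effect when used.
; UseItem rolls a random integer to pick one of eleven soul functions, then calls the parent UseItem.
; Angel sets every ThirdPersonCharacter's Health to full and Demon halves it, affecting all such characters rather than only the user.
; The other souls are placeholders that only print their names.
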(event EventBeginPlay
  (|CallParentFunction) ; This node is disabled and will not be called.\nDrag off pins to build functionality.
)

(event Collision|EventActorBeginOverlap
  (params (OtherActor :type Actor%20Object%20Reference))
  (|CallParentFunction OtherActor) ; This node is disabled and will not be called.\nDrag off pins to build functionality.
)

(event EventTick
  (params (DeltaSeconds :type Float%20%28single-precision%29))
  (|CallParentFunction DeltaSeconds) ; This node is disabled and will not be called.\nDrag off pins to build functionality.
)

(fn ConstructionScript
  (|CallParentFunction))

(fn UseItem
  (params (User :type Third%20Person%20Character%20Object%20Reference))
  (switch int (Math|Random|RandomIntegerinRange 0 10)
    (:0
      (CallFunction|Necromancer))
    (:1
      (CallFunction|Honest))
    (:2
      (CallFunction|Liar))
    (:3
      (CallFunction|Wise))
    (:4
      (CallFunction|Angel))
    (:5
      (CallFunction|Demon))
    (:6
      (CallFunction|Wicked))
    (:7
      (CallFunction|Thieves))
    (:8
      (CallFunction|Spooky))
    (:9
      (CallFunction|Lost))
    (:10
      (CallFunction|Trickster)))
  (bind _success (|CallParentFunction User))
  (return _success))

(fn Necromancer
  (Development|PrintString "Necromancer"))

(fn Honest
  (Development|PrintString "Honest Soul"))

(fn Liar
  (Development|PrintString "Liar's Soul"))

(fn Wise
  (Development|PrintString "Wise Soul"))

(fn Angel
  (bind _outactors (Actor|GetAllActorsOfClass "/Game/Blueprints/Characters/ThirdPersonCharacter.ThirdPersonCharacter_C"))
  (for _array_element _outactors
    (Variables|/Game/Blueprints/Characters/ThirdPersonCharacter.ThirdPersonCharacter_C|SetHealth _array_element 1e+02)))

(fn Demon
  (bind _outactors (Actor|GetAllActorsOfClass "/Game/Blueprints/Characters/ThirdPersonCharacter.ThirdPersonCharacter_C"))
  (for _array_element _outactors
    (Variables|/Game/Blueprints/Characters/ThirdPersonCharacter.ThirdPersonCharacter_C|SetHealth _array_element (/ (Variables|/Game/Blueprints/Characters/ThirdPersonCharacter.ThirdPersonCharacter_C|GetHealth _array_element) 2.0))))

(fn Wicked
  (Development|PrintString "Wicked Soul"))

(fn Thieves
  (Development|PrintString "Thieves Soul"))

(fn Spooky
  (Development|PrintString "Spooky"))

(fn Lost
  (Development|PrintString "Lost"))

(fn Trickster
  (Development|PrintString "Trickster"))