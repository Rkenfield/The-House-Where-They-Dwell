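; Inventory component that stores items in a fixed array of slot structures, sized to NoOfSlots on BeginPlay.
; AddToInventory checks the filled count against a hardcoded limit of four and returns whether the add succeeded.
; CreateStack writes non-stackable items into the first slot matching an empty, zero-quantity structure and increments the count.
; Stacking of stackable items is not implemented.
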(event EventBeginPlay
  ;[1 1 1] Initializes the inventory with required size
  (CallFunction|PrepareInventory))

(event EventTick
  (params (DeltaSeconds :type Float%20%28single-precision%29)))

(fn AddtoInventory
  (params (ContentToAdd :type Slot%20Structure%20Structure))
  ;[1 1 1] Checks if inventory has space to add a new item and if yes, checks if item is to be stacked on an existing slot or added to a new slot.
  (if (< (Variables|Default|GetSlotsFilled) 4)
    (if (not (.isstackable (.itemstructure ContentToAdd)))
      (CallFunction|CreateStack ContentToAdd)
      (LocalVariables|SetAddSuccess true)
      (return (LocalVariables|GetAddSuccess)))
    (else
      (LocalVariables|SetAddSuccess false)
      (return (LocalVariables|GetAddSuccess)))))

(fn CreateStack
  (params (ContentToAdd :type Slot%20Structure%20Structure))
  (bind _inventory (Variables|Default|GetInventory))
  ;[1 1 1] Adding Item to Slot- Finds the first free slot available and adds item to that slot
  (Utilities|Array|SetArrayElem _inventory (Utilities|Array|FindItem _inventory (Utilities|Struct|MakeSlotStructure "(Name_2_6A5FEA534E7C5B6891091A9751937919=NSLOCTEXT(\"[8654E3B44D83D6B0DB71DBA0CD75DF08]\", \"9339194841BA164326F1519822779F04\", \"None\"),IsStackable_5_BE51BD314F210762028380ACF9921B43=True,Thumbnail_8_CB3687484A07D7DD25D3D88C7861C837=None,Description_11_A5E104F147D4EBBD069A19AF25B08BB2=NSLOCTEXT(\"[8654E3B44D83D6B0DB71DBA0CD75DF08]\", \"D599A13E48B83CD8521247854357A9F2\", \"None\"),IsConsumable_14_84465B91483DD2E1AF6CF99AA273FEB5=True,MaxStackSize_21_436777234A098D236EEF2D879F61C9B4=4,Class_20_59146D4D4DAECBF75343ACAD91CCB9D7=None)")) ContentToAdd)
  (Variables|Default|SetSlotsFilled (+ (Variables|Default|GetSlotsFilled) 1)))

(fn PrepareInventory
  ;[1 1 1] Sets the size of the inventory
  (Utilities|Array|Resize (Variables|Default|GetInventory) (Variables|Default|GetNoOfSlots)))