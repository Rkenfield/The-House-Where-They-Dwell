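; Multiplayer game mode that sets up local players and hands each one a playable character.
; On BeginPlay it loops CreatePlayer to add local players with their own controllers, intended to total four.
; SpawnPlayer takes a controller with a valid pawn, uses PlayerCount to select a BP_PlayerChild class, and possesses the instance already in the level.
; Each possession advances PlayerCount, so characters are assigned in join order.
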(event Custom|SpawnPlayer
  (params (Controller :type Player%20Controller%20Object%20Reference))
  ;[1 1 1] SpawnPlayer- Allows each player to take control of one of the playable characters when either '1' (keyboard) or 'Special Left Button' (Gamepad) is pressed
  (Utilities|IsValid (Pawn|GetControlledPawn Controller)
    (:Is%20Valid
      (bind _returnvalue (Actor|GetActorOfClass (Utilities|Select :Index (Variables|Default|GetPlayerCount) :Option%200 "/Game/Blueprints/Characters/BP_PlayerChild1.BP_PlayerChild1_C" :Option%201 "/Game/Blueprints/Characters/BP_PlayerChild2.BP_PlayerChild2_C" :Option%202 "/Game/Blueprints/Characters/BP_PlayerChild3.BP_PlayerChild3_C" :Option%203 "/Game/Blueprints/Characters/BP_PlayerChild4.BP_PlayerChild4_C")))
      (Pawn|Possess Controller _returnvalue)
      (bind _output_get (Variables|Default|SetPlayerCount (+ (Variables|Default|GetPlayerCount) 1))))))

(event EventBeginPlay
  ;[1 1 1] Begin Play- Creates 4 players
  (while (<= (Variables|Default|GetNoOfPlayers) 3)
    (Variables|Default|SetNoOfPlayers (+ (Variables|Default|GetNoOfPlayers) 1))
    (bind _returnvalue (Class|GameplayStatics|CreatePlayer -1))))

(fn ConstructionScript)