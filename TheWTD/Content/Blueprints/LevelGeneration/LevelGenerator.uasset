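; Grid-based level generator that scatters room instances at construction time; room selection by neighbours is unfinished.
; The construction script disables room shadow casting for performance and sizes a flattened MaxX by MaxY tile array, with helpers converting to and from row/column.
; It randomly adds Room2d instances at TileSize spacing, using a Placed flag to skip the tile after each placement.
; The other room components are never populated, and the row/column pass only computes indices.
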(event EventBeginPlay)

(event Collision|EventActorBeginOverlap
  (params (OtherActor :type Actor%20Object%20Reference)))

(event EventTick
  (params (DeltaSeconds :type Float%20%28single-precision%29)))

(fn ConstructionScript
  (bind _maxx (Variables|Default|GetMaxX))
  (bind _maxy (Variables|Default|GetMaxY))
  (bind _maxy_2 (Variables|Default|GetMaxY))
  (bind _tilesize (Variables|Default|GetTileSize))
  (bind _returnvalue (* _maxx _maxy_2))
  ;[1 1 1] disable shadow casting by the floor(helps performance)
  (Rendering|SetCastShadow (Variables|Default|Getroom2ds) false)
  ;[1 1 1] Builds 2d array and sets certain rooms based on rooms around(not finished== need to add more if statements to specify what room needs to be spawned)
  (Utilities|Array|Resize (Variables|Default|GetTileType) _returnvalue)
  (bind _output_get (Variables|Default|Setlength (- _returnvalue 1)))
  (for _index (range 0 _output_get)
    (bind (_rowindex _colindex) (CallFunction|FlattenedtoNormalIndeces _index (Variables|Default|GetMaxY)))
    (Variables|Default|Setrow _rowindex)
    (Variables|Default|Setcol _colindex))
  ;[1 1 1] spawn room based on what number is in array
  (for (_ _array_index) (Variables|Default|GetTileType)
    (if (and (<= (Math|Random|RandomIntegerinRange 1 30) 6) (Math|Boolean|Equal(Boolean) (Variables|Default|Getplaced) false))
      (Components|InstancedStaticMesh|AddInstance (Variables|Default|Getroom2d) (Math|Conversions|ToTransform(Vector) (Math|Vector|MakeVector (Math|Conversions|ToFloat(Integer) (* (/ _array_index _maxy) _tilesize)) (Math|Conversions|ToFloat(Integer) (* (Math|Integer|%(Integer) _array_index _maxy) _tilesize)) 0.0)))
      (Variables|Default|Setplaced true)
      (else
        (Variables|Default|Setplaced false)))))

(fn NormalIndecestoFlattenedIndex
  (params (maxY :type Integer) (rowIndex :type Integer) (colIndex :type Integer))
  (return (+ (* maxY rowIndex) colIndex)))

(fn FlattenedtoNormalIndeces
  (params (FlattenedIndex :type Integer) (MaxY :type Integer))
  (return (/ FlattenedIndex MaxY) (Math|Integer|%(Integer) FlattenedIndex MaxY)))