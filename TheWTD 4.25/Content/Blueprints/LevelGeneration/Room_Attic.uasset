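; Attic room for level generation that spawns its contents and handles the spreading fire as its spider nests are destroyed.
; BeginPlay uses mesh sockets to spawn the door, furniture and tagged nests that reference the room.
; FirePropagation maps the destroyed nest's index to delayed chains of effect activations, adding a final chain once the GameMode's destroyed count reaches maximum.
; It also removes web barriers for phase 3 and activates reverb on overlap.
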(event OnComponentBeginOverlap(VerbVolume)
  (params (OverlappedComponent :type Primitive%20Component%20Object%20Reference) (OtherActor :type Actor%20Object%20Reference) (OtherComp :type Primitive%20Component%20Object%20Reference) (OtherBodyIndex :type Integer) (bFromSweep :type Boolean) (SweepResult :type Hit%20Result%20Structure%20%28by%20ref%29))
  (Class|GameplayStatics|ActivateReverbEffect "/Game/Audio/Reverb/LargeRoom.LargeRoom" "AtticVerb" 0.0 1.0 1.0))

(event Custom|DestroyBarrier
  ;[1 1 1] Destroys the web barrier when phase 3 starts
  (Components|DestroyComponent (Variables|Default|GetDoorBarrier)))

(event Custom|FirePropagation
  (params (DestroyedNest :type Actor%20Object%20Reference))
  ;[1 1 1] "Fire Propagation"
  (for (_array_element _array_index) (Variables|Default|GetNests)
    (if (== DestroyedNest _array_element)
      (switch int _array_index
        (:0
          (bind _array_element_2 (Utilities|CustomLoopwithDelay (Utilities|Array|MakeArray (Variables|Default|GetPF_Nest1_00) (Variables|Default|GetPF_Nest1_01) (Variables|Default|GetPF_Nest1_02) (Variables|Default|GetPF_Nest1_03) (Variables|Default|GetPF_Nest1_04) (Variables|Default|GetPF_Nest1_05) (Variables|Default|GetPF_Nest1_06)) 2.0)
            (:Loop%20Body
              (Components|Activation|SetActive _array_element_2 true false))
            (:Completed
              (Components|Activation|SetActive (Variables|Default|GetNest1_Smoke) true false))))
        (:1
          (bind _array_element_3 (Utilities|CustomLoopwithDelay (Utilities|Array|MakeArray (Variables|Default|GetPF_Nest2_00) (Variables|Default|GetPF_Nest2_01) (Variables|Default|GetPF_Nest2_02) (Variables|Default|GetPF_Nest2_03) (Variables|Default|GetPF_Nest2_04) (Variables|Default|GetPF_Nest2_05) (Variables|Default|GetPF_Nest2_06) (Variables|Default|GetPF_Nest2_07) (Variables|Default|GetPF_Nest2_08) (Variables|Default|GetPF_Nest2_09)) 2.0)
            (:Loop%20Body
              (Components|Activation|SetActive _array_element_3 true false))
            (:Completed
              (Components|Activation|SetActive (Variables|Default|GetNest2_Smoke) true false))))
        (:2
          (bind _array_element_4 (Utilities|CustomLoopwithDelay (Utilities|Array|MakeArray (Variables|Default|GetPF_Nest3_00) (Variables|Default|GetPF_Nest3_01) (Variables|Default|GetPF_Nest3_02) (Variables|Default|GetPF_Nest3_03) (Variables|Default|GetPF_Nest3_04) (Variables|Default|GetPF_Nest3_05) (Variables|Default|GetPF_Nest3_06) (Variables|Default|GetPF_Nest3_07) (Variables|Default|GetPF_Nest3_08) (Variables|Default|GetPF_Nest3_09) (Variables|Default|GetPF_Nest3_010) (Variables|Default|GetPF_Nest3_011) (Variables|Default|GetPF_Nest3_012) (Variables|Default|GetPF_Nest3_013) (Variables|Default|GetPF_Nest3_014) (Variables|Default|GetPF_Nest3_015)) 2.0)
            (:Loop%20Body
              (Components|Activation|SetActive _array_element_4 true false))
            (:Completed
              (Components|Activation|SetActive (Variables|Default|GetNest3_Smoke) true false))))
        (:3
          (bind _array_element_5 (Utilities|CustomLoopwithDelay (Utilities|Array|MakeArray (Variables|Default|GetPF_Nest4_00) (Variables|Default|GetPF_Nest4_01) (Variables|Default|GetPF_Nest4_02) (Variables|Default|GetPF_Nest4_03) (Variables|Default|GetPF_Nest4_04) (Variables|Default|GetPF_Nest4_05) (Variables|Default|GetNest4_Smoke)) 2.0)
            (:Loop%20Body
              (Components|Activation|SetActive _array_element_5 true false))
            (:Completed
              (bind _array_element_6 (Utilities|CustomLoopwithDelay (Utilities|Array|MakeArray (Variables|Default|GetPF_Center_00) (Variables|Default|GetPF_Center_01) (Variables|Default|GetPF_Center_02) (Variables|Default|GetPF_Center_03) (Variables|Default|GetPF_Center_04) (Variables|Default|GetPF_Center_05) (Variables|Default|GetPF_Center_06) (Variables|Default|GetPF_Center_07) (Variables|Default|GetPF_Center_08) (Variables|Default|GetPF_Center_09) (Variables|Default|GetPF_Center_010)) 1.0)
                (:Loop%20Body
                  (Components|Activation|SetActive _array_element_6 true false))
                (:Completed
                  (Components|Activation|SetActive (Variables|Default|GetCenter_Smoke) true false))))))
        (:4
          (bind _array_element_7 (Utilities|CustomLoopwithDelay (Utilities|Array|MakeArray (Variables|Default|GetPF_Nest5_00) (Variables|Default|GetPF_Nest5_01) (Variables|Default|GetPF_Nest5_02) (Variables|Default|GetPF_Nest5_03) (Variables|Default|GetPF_Nest5_04) (Variables|Default|GetPF_Nest5_05) (Variables|Default|GetPF_Nest5_06) (Variables|Default|GetPF_Nest5_07)) 2.0)
            (:Loop%20Body
              (Components|Activation|SetActive _array_element_7 true false))
            (:Completed
              (Components|Activation|SetActive (Variables|Default|GetNest5_Smoke) true false)))))))
  (bind _asbp_wtdgame_mode (Utilities|Casting|CastToBP_WTDGameMode (Game|GetGameMode)))
  (if (== (Variables|/Game/Blueprints/BP_WTDGameMode.BP_WTDGameMode_C|GetDestroyedAtticNests _asbp_wtdgame_mode) (Variables|/Game/Blueprints/BP_WTDGameMode.BP_WTDGameMode_C|GetMaxNoOfAtticNests _asbp_wtdgame_mode))
    (bind _array_element_8 (Utilities|CustomLoopwithDelay (Utilities|Array|MakeArray (Variables|Default|GetPF_Last_00) (Variables|Default|GetPF_Last_01) (Variables|Default|GetPF_Last_02) (Variables|Default|GetPF_Last_03) (Variables|Default|GetPF_Last_04) (Variables|Default|GetPF_Last_05) (Variables|Default|GetPF_Last_06) (Variables|Default|GetPF_Last_07) (Variables|Default|GetPF_Last_08) (Variables|Default|GetPF_Last_09) (Variables|Default|GetLast_Smoke_00)) 1.0)
      (:Loop%20Body
        (Components|Activation|SetActive _array_element_8 true false)))))

(event EventBeginPlay
  (bind _staticmesh (Variables|Default|GetStaticMesh))
  (bind _returnvalue (Transformation|GetAllSocketNames _staticmesh))
  ;[1 1 1] Spawning things at start of game
  (for _array_element _returnvalue
    (if (Utilities|Name|Equal(Name) _array_element "Door1")
      (Game|SpawnActorfromClass "/Game/Blueprints/Blueprints/BP_Door_Attic.BP_Door_Attic_C" (Math|Transform|MakeTransform (.location (Transformation|GetSocketTransform (Variables|Default|GetStaticMesh) _array_element "RTS_World")) (.rotation (Transformation|GetSocketTransform (Variables|Default|GetStaticMesh) _array_element "RTS_World")) "1,1,1") "Undefined" 0 0)
      (for _array_element_2 _returnvalue
        (if (Utilities|Enum|Equal(Enum) (Utilities|String|GetSubstring (Utilities|String|ToString(Name) _array_element_2) 0 4) "Nest")
          (bind _returnvalue_2 (Game|SpawnActorfromClass "/Game/Blueprints/Blueprints/BP_AtticNest.BP_AtticNest_C" (Math|Transform|MakeTransform (.location (Transformation|GetSocketTransform (Variables|Default|GetStaticMesh) _array_element_2 "RTS_World")) (.rotation (Transformation|GetSocketTransform (Variables|Default|GetStaticMesh) _array_element_2 "RTS_World")) "1.200000,1.200000,1.200000") "Undefined" 0 0))
          (Variables|/Game/Blueprints/Blueprints/BP_AtticNest.BP_AtticNest_C|SetAttic_Owner _returnvalue_2 self)
          (Utilities|Array|Add (Variables|/Script/Engine.Actor|GetTags _returnvalue_2) "AtticNest") ; Gives all the nests in the attic a special "AtticNest" tag.
          (Variables|/Game/Blueprints/Blueprints/BP_Nest.BP_Nest_C|SetMaxNofOfSpawnedSpiders _returnvalue_2 2)
          (Utilities|Array|Add (Variables|Default|GetNests) _returnvalue_2)
          (elif (Utilities|Name|Equal(Name) _array_element_2 "Desk1")
            (Game|SpawnActorfromClass "/Game/Blueprints/Blueprints/BP_Desk.BP_Desk_C" (Math|Transform|MakeTransform (.location (Transformation|GetSocketTransform (Variables|Default|GetStaticMesh) _array_element_2 "RTS_World")) (.rotation (Transformation|GetSocketTransform (Variables|Default|GetStaticMesh) _array_element_2 "RTS_World")) "1.700000,1.700000,1.700000") "Undefined" 0 0)
            (elif (Utilities|Name|Equal(Name) _array_element_2 "Dresser1")
              (Game|SpawnActorfromClass "/Game/Blueprints/Blueprints/BP_Dresser.BP_Dresser_C" (Math|Transform|MakeTransform (.location (Transformation|GetSocketTransform (Variables|Default|GetStaticMesh) _array_element_2 "RTS_World")) (.rotation (Transformation|GetSocketTransform (Variables|Default|GetStaticMesh) _array_element_2 "RTS_World")) "1.700000,1.700000,1.700000") "Undefined" 0 0))))))))

(fn ConstructionScript)