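; Storage room piece for level generation that populates itself with a door and candle flames and sets its own reverb.
; On BeginPlay it scans the static mesh sockets, spawns a BP_Door at Door1, then spawns BP_CandleFlame actors at the two flame components, so flames depend on that socket existing.
; Overlapping its box fades in a small-room reverb, leaving outside audio volumes to fade in other reverbs.
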(event OnComponentBeginOverlap(Box)
  (params (OverlappedComponent :type Primitive%20Component%20Object%20Reference) (OtherActor :type Actor%20Object%20Reference) (OtherComp :type Primitive%20Component%20Object%20Reference) (OtherBodyIndex :type Integer) (bFromSweep :type Boolean) (SweepResult :type Hit%20Result%20Structure%20%28by%20ref%29))
  (Class|GameplayStatics|ActivateReverbEffect "/Game/Audio/Reverb/SmallRoom.SmallRoom" "StudyVerb" 0.0 1.0 1.0) ; Will automatically fade into other Reverbs when player hits audio volume outside
)

(event EventBeginPlay
  (for _array_element (Transformation|GetAllSocketNames (Variables|Default|GetStaticMesh))
    (if (Utilities|Name|Equal(Name) _array_element "Door1")
      (Game|SpawnActorfromClass "/Game/Blueprints/Blueprints/BP_Door.BP_Door_C" (Math|Transform|MakeTransform (.location (Transformation|GetSocketTransform (Variables|Default|GetStaticMesh) _array_element "RTS_World")) (.rotation (Transformation|GetSocketTransform (Variables|Default|GetStaticMesh) _array_element "RTS_World")) "1,1,1") "Undefined" 0 0)
      (for _array_element_2 (Utilities|Array|MakeArray (Variables|Default|GetFlame01) (Variables|Default|GetFlame02))
        (Game|SpawnActorfromClass "/Game/Art/Particles/CandleFlame/BP_CandleFlame.BP_CandleFlame_C" (Transformation|GetWorldTransform _array_element_2) "Undefined" 0 0)))))

(fn ConstructionScript)