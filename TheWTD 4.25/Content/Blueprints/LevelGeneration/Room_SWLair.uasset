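; Procedural-level room Blueprint for an attic lair (SWLair) with a webbed door barrier, door and nests.
; On BeginPlay it reads static mesh sockets, spawning BP_Door at Door1 and, within that branch, BP_Nest at each Nest-prefixed socket, tagged AtticNest.
; DestroyBarrier removes the barrier and web components.
; Overlapping the reverb volume activates a large-room reverb under the AtticVerb tag.
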(event OnComponentBeginOverlap(VerbVolume)
  (params (OverlappedComponent :type Primitive%20Component%20Object%20Reference) (OtherActor :type Actor%20Object%20Reference) (OtherComp :type Primitive%20Component%20Object%20Reference) (OtherBodyIndex :type Integer) (bFromSweep :type Boolean) (SweepResult :type Hit%20Result%20Structure%20%28by%20ref%29))
  (Class|GameplayStatics|ActivateReverbEffect "/Game/Audio/Reverb/LargeRoom.LargeRoom" "AtticVerb" 0.0 1.0 1.0))

(event Custom|DestroyBarrier
  (Components|DestroyComponent (Variables|Default|GetDoorBarrier)))

(event EventBeginPlay
  (bind _staticmesh (Variables|Default|GetStaticMesh))
  (bind _returnvalue (Transformation|GetAllSocketNames _staticmesh))
  (for _array_element _returnvalue
    (if (Utilities|Name|Equal(Name) _array_element "Door1")
      (Game|SpawnActorfromClass "/Game/Blueprints/Blueprints/BP_Door.BP_Door_C" (Math|Transform|MakeTransform (.location (Transformation|GetSocketTransform (Variables|Default|GetStaticMesh) _array_element "RTS_World")) (.rotation (Transformation|GetSocketTransform (Variables|Default|GetStaticMesh) _array_element "RTS_World")) "1,1,1") "Undefined" 0 0)
      (for _array_element_2 _returnvalue
        (if (Utilities|Enum|Equal(Enum) (Utilities|String|GetSubstring (Utilities|String|ToString(Name) _array_element_2) 0 4) "Nest")
          (bind _returnvalue_2 (Game|SpawnActorfromClass "/Game/Blueprints/Blueprints/BP_Nest.BP_Nest_C" (Transformation|GetSocketTransform (Variables|Default|GetStaticMesh) _array_element_2 "RTS_World") "Undefined" 0 0))
          (Utilities|Array|Add (Variables|/Script/Engine.Actor|GetTags _returnvalue_2) "AtticNest") ; Gives all the nests in the attic a special "AtticNest" tag.
        )))))

(fn ConstructionScript)