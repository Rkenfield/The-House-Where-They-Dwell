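; Base hallway actor for level generation that sets its mesh from HallwayType and spawns pieces at the mesh's sockets.
; On BeginPlay it spawns Door_or_FilledWall actors at whichever door sockets are flagged as fake.
; CreateRooms, not called within this Blueprint, randomly spawns rooms at one, both or neither room-center socket, skipping fake-door sides.
; Each branch there makes its own random roll, so the outcomes are not equally likely.
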(event EventBeginPlay
  (CallFunction|SetMarkedFilledWalls))

(fn ConstructionScript
  (Components|StaticMesh|SetStaticMesh (Variables|Default|GetStaticMesh) (Variables|Default|GetHallwayType)))

(fn SetMarkedFilledWalls
  (bind _staticmesh (Variables|Default|GetStaticMesh))
  (bind _staticmesh_2 (Variables|Default|GetStaticMesh))
  (bind _staticmesh_3 (Variables|Default|GetStaticMesh))
  (bind _staticmesh_4 (Variables|Default|GetStaticMesh))
  (bind _returnvalue (Transformation|GetSocketTransform _staticmesh "Door1" "RTS_World"))
  (bind _returnvalue_2 (Transformation|GetSocketTransform _staticmesh_2 "Door2" "RTS_World"))
  (bind _returnvalue_3 (Transformation|GetSocketTransform _staticmesh_3 "Door2" "RTS_World"))
  (bind _returnvalue_4 (Transformation|GetSocketTransform _staticmesh_4 "Door1" "RTS_World"))
  (if (Variables|Default|GetSpawnFakeDoorAt1)
    (if (Variables|Default|GetSpawnFakeDoorAt2)
      (Game|SpawnActorfromClass "/Game/Blueprints/LevelGeneration/Door_or_FilledWall.Door_or_FilledWall_C" (Math|Transform|MakeTransform (.location _returnvalue) (.rotation _returnvalue) "1,1,1") "Undefined" 0 0)
      (Game|SpawnActorfromClass "/Game/Blueprints/LevelGeneration/Door_or_FilledWall.Door_or_FilledWall_C" (Math|Transform|MakeTransform (.location _returnvalue_2) (.rotation _returnvalue_2) "1,1,1") "Undefined" 0 0)
      (else
        (Game|SpawnActorfromClass "/Game/Blueprints/LevelGeneration/Door_or_FilledWall.Door_or_FilledWall_C" (Math|Transform|MakeTransform (.location _returnvalue_4) (.rotation _returnvalue_4) "1,1,1") "Undefined" 0 0)))
    (elif (Variables|Default|GetSpawnFakeDoorAt2)
      (Game|SpawnActorfromClass "/Game/Blueprints/LevelGeneration/Door_or_FilledWall.Door_or_FilledWall_C" (Math|Transform|MakeTransform (.location _returnvalue_3) (.rotation _returnvalue_3) "1,1,1") "Undefined" 0 0))))

(fn CreateRooms
  (bind _returnvalue (Math|Random|RandomIntegerinRange 0 3))
  (bind _staticmesh (Variables|Default|GetStaticMesh))
  (bind _staticmesh_2 (Variables|Default|GetStaticMesh))
  (bind _staticmesh_3 (Variables|Default|GetStaticMesh))
  (bind _staticmesh_4 (Variables|Default|GetStaticMesh))
  (bind _returnvalue_2 (Transformation|GetSocketTransform _staticmesh_4 "Room1Center" "RTS_World"))
  (bind _returnvalue_3 (Transformation|GetSocketTransform _staticmesh_3 "Room1Center" "RTS_World"))
  (bind _returnvalue_4 (Transformation|GetSocketTransform _staticmesh_2 "Room2Center" "RTS_World"))
  (bind _returnvalue_5 (Transformation|GetSocketTransform _staticmesh "Room2Center" "RTS_World"))
  (if (not (== _returnvalue 0))
    (if (and (== _returnvalue 1) (Math|Boolean|Equal(Boolean) (Variables|Default|GetSpawnFakeDoorAt1) false))
      (Game|SpawnActorfromClass "/Game/Blueprints/LevelGeneration/Room.Room_C" (Math|Transform|MakeTransform (.location _returnvalue_3) (.rotation _returnvalue_3) "1,1,1") "Undefined" 0 0)
      (elif (and (== _returnvalue 2) (Math|Boolean|Equal(Boolean) (Variables|Default|GetSpawnFakeDoorAt2) false))
        (Game|SpawnActorfromClass "/Game/Blueprints/LevelGeneration/Room.Room_C" (Math|Transform|MakeTransform (.location _returnvalue_4) (.rotation _returnvalue_4) "1,1,1") "Undefined" 0 0)
        (elif (Math|Boolean|ANDBoolean (== _returnvalue 3) (Math|Boolean|Equal(Boolean) (Variables|Default|GetSpawnFakeDoorAt1) false) (Math|Boolean|Equal(Boolean) (Variables|Default|GetSpawnFakeDoorAt2) false))
          (Game|SpawnActorfromClass "/Game/Blueprints/LevelGeneration/Room.Room_C" (Math|Transform|MakeTransform (.location _returnvalue_2) (.rotation _returnvalue_2) "1,1,1") "Undefined" 0 0)
          (Game|SpawnActorfromClass "/Game/Blueprints/LevelGeneration/Room.Room_C" (Math|Transform|MakeTransform (.location _returnvalue_5) (.rotation _returnvalue_5) "1,1,1") "Undefined" 0 0))))))