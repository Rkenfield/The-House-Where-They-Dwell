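; Hallway table decoration for level generation that randomizes its prop and candles on BeginPlay.
; It picks a Deco mesh from an array, then fills the candle slots matching a candelabra, candlestick holder or chamberstick with random candle meshes.
; Candelabra slots each roll for a candle, while the single holders always set one.
; Coin flips trigger actor spawns at Flame sockets, using BP_CandleFlame for single holders but no specified class for the candelabra.
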(event EventBeginPlay
  (bind _returnvalue (Math|Random|RandomInteger 2))
  (bind _returnvalue_2 (Math|Random|RandomInteger 4))
  (bind _candlearray (Variables|Default|GetCandleArray))
  (bind _output (Utilities|Array|Get(acopy) _candlearray _returnvalue_2))
  (Components|StaticMesh|SetStaticMesh (Variables|Default|GetDeco) (Utilities|Array|Get(acopy) (Variables|Default|GetDecoArray) (Math|Random|RandomInteger 3)))
  (if (== (Variables|/Script/Engine.StaticMeshComponent|GetStaticMesh (Variables|Default|GetDeco)) "/Game/Art/AllMeshesGoHERE/Bedroom/CandleStuffs_SM_Candelabra.CandleStuffs_SM_Candelabra")
    (Utilities|FlowControl|Sequence
      (:then_0
        (if (== _returnvalue 0)
          (Components|StaticMesh|SetStaticMesh (Variables|Default|GetCandelabra_Candle01) _output)
          (if (== (Math|Random|RandomInteger 2) 0)
            (Game|SpawnActorfromClass "/Game/Art/Particles/CandleFlame/BP_CandleFlame.BP_CandleFlame_C" (Transformation|GetSocketTransform (Variables|Default|GetCandelabra_Candle01) "Flame" "RTS_World") "Undefined" 0 0))))
      (:then_1
        (if (== _returnvalue 0)
          (Components|StaticMesh|SetStaticMesh (Variables|Default|GetCandelabra_Candle02) _output)
          (if (== (Math|Random|RandomInteger 2) 0)
            (Game|SpawnActorfromClass "/Game/Art/Particles/CandleFlame/BP_CandleFlame.BP_CandleFlame_C" (Transformation|GetSocketTransform (Variables|Default|GetCandelabra_Candle02) "Flame" "RTS_World") "Undefined" 0 0))))
      (:then_2
        (if (== _returnvalue 0)
          (Components|StaticMesh|SetStaticMesh (Variables|Default|GetCandelabra_Candle03) _output)
          (if (== (Math|Random|RandomInteger 2) 0)
            (Game|SpawnActorfromClass "/Game/Art/Particles/CandleFlame/BP_CandleFlame.BP_CandleFlame_C" (Transformation|GetSocketTransform (Variables|Default|GetCandelabra_Candle03) "Flame" "RTS_World") "Undefined" 0 0)))))
    (elif (== (Variables|/Script/Engine.StaticMeshComponent|GetStaticMesh (Variables|Default|GetDeco)) "/Game/Art/AllMeshesGoHERE/Bedroom/CandleStuffs_SM_CandlestickHolder.CandleStuffs_SM_CandlestickHolder")
      (Components|StaticMesh|SetStaticMesh (Variables|Default|GetCandlestick_Candle01) (Utilities|Array|Get(acopy) (Variables|Default|GetCandleArray) (Math|Random|RandomInteger 6)))
      (if (== (Math|Random|RandomInteger 2) 0)
        (Game|SpawnActorfromClass "/Game/Art/Particles/CandleFlame/BP_CandleFlame.BP_CandleFlame_C" (Transformation|GetSocketTransform (Variables|Default|GetCandlestick_Candle01) "Flame" "RTS_World") "Undefined" 0 0))
      (elif (== (Variables|/Script/Engine.StaticMeshComponent|GetStaticMesh (Variables|Default|GetDeco)) "/Game/Art/AllMeshesGoHERE/Bedroom/CandleStuffs_SM_Chamberstick.CandleStuffs_SM_Chamberstick")
        (Components|StaticMesh|SetStaticMesh (Variables|Default|GetChamberstick_Candle01) (Utilities|Array|Get(acopy) (Variables|Default|GetCandleArray) (Math|Random|RandomInteger 6)))
        (if (== (Math|Random|RandomInteger 2) 0)
          (Game|SpawnActorfromClass "/Game/Art/Particles/CandleFlame/BP_CandleFlame.BP_CandleFlame_C" (Transformation|GetSocketTransform (Variables|Default|GetChamberstick_Candle01) "Flame" "RTS_World") "Undefined" 0 0))))))

(fn ConstructionScript)