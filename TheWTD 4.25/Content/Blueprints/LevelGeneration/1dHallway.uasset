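; Procedural level-generation hallway piece with one door socket that caps itself or grows a room when play begins.
; If flagged for a fake door, it spawns a door-or-filled-wall actor at the Door1 socket.
; Otherwise a random roll either places that same plug or spawns a Room at the Room1Center socket.
; New rooms store this hallway as owner and are registered and counted in THWDGameMode.
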(event EventBeginPlay
  (bind _output_get (Variables|Default|SetRoomChoice (Math|Random|RandomIntegerinRange 0 1)))
  (CallFunction|PlugDoor)
  (CallFunction|SpawnRoom _output_get))

(fn ConstructionScript
  (|CallParentFunction))

(fn PlugDoor
  (bind _staticmesh (Variables|Default|GetStaticMesh))
  (bind _returnvalue (Transformation|GetSocketTransform _staticmesh "Door1" "RTS_World"))
  (if (Variables|Default|GetSpawnFakeDoorAt1)
    (Game|SpawnActorfromClass "/Game/Blueprints/LevelGeneration/Door_or_FilledWall_JacobTest.Door_or_FilledWall_JacobTest_C" (Math|Transform|MakeTransform (.location _returnvalue) (.rotation _returnvalue) "1,1,1") "Undefined" 0 0)))

(fn SpawnRoom
  (params (Choice :type Integer))
  (bind _staticmesh (Variables|Default|GetStaticMesh))
  (bind _staticmesh_2 (Variables|Default|GetStaticMesh))
  (bind _returnvalue (Transformation|GetSocketTransform _staticmesh "Room1Center" "RTS_World"))
  (bind _returnvalue_2 (Transformation|GetSocketTransform _staticmesh_2 "Door1" "RTS_World"))
  (if (not (Math|Boolean|Equal(Boolean) (Variables|Default|GetSpawnFakeDoorAt1) true))
    (switch int Choice
      (:0
        (Game|SpawnActorfromClass "/Game/Blueprints/LevelGeneration/Door_or_FilledWall_JacobTest.Door_or_FilledWall_JacobTest_C" (Math|Transform|MakeTransform (.location _returnvalue_2) (.rotation _returnvalue_2) "1,1,1") "Undefined" 0 0))
      (:1
        (bind _returnvalue_3 (Game|SpawnActorfromClass "/Game/Blueprints/LevelGeneration/Room.Room_C" (Math|Transform|MakeTransform (.location _returnvalue) (.rotation _returnvalue) "1,1,1") "Undefined" 0 0))
        (CallFunction|AddRoomtoArray _returnvalue_3)
        (Variables|/Game/Blueprints/LevelGeneration/Room.Room_C|SetRooms%20Owner _returnvalue_3 self)))))

(fn AddRoomtoArray
  (params (RoomToAdd :type Room%20Object%20Reference))
  (bind _asthwdgame_mode (Utilities|Casting|CastToTHWDGameMode (Game|GetGameMode)))
  (Utilities|Array|Add (Variables|/Game/Blueprints/THWDGameMode.THWDGameMode_C|GetRoomsinHouse _asthwdgame_mode) (Utilities|Struct|MakeRooms RoomToAdd))
  (Variables|/Game/Blueprints/THWDGameMode.THWDGameMode_C|SetNumOfRooms _asthwdgame_mode (+ (Variables|/Game/Blueprints/THWDGameMode.THWDGameMode_C|GetNumOfRooms _asthwdgame_mode) 1)))