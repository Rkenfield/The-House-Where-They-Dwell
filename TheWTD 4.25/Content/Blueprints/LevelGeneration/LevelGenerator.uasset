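; Level generator that randomly places rooms on a tile grid in its construction script.
; Checkerboard cells may receive one of five instanced room meshes, whose center and door socket locations are recorded.
; CreateSpanningTree then runs a Prim-style loop over the rooms to build edges, but its nearest-room search is a stub returning zero indices.
; Corridor and hallway functions are empty, and room shadow casting is disabled on most meshes for performance.
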(event EventBeginPlay)

(event Collision|EventActorBeginOverlap
  (params (OtherActor :type Actor%20Object%20Reference)))

(event EventTick
  (params (DeltaSeconds :type Float%20%28single-precision%29)))

(fn ConstructionScript
  (bind _returnvalue (Math|Random|RandomIntegerinRange 0 4))
  (bind _maxx (Variables|Default|GetMaxX))
  (bind _maxy (Variables|Default|GetMaxY))
  (bind _room_1d (Variables|Default|Getroom%201d))
  (bind _room2d (Variables|Default|Getroom2d))
  (bind _room2ds (Variables|Default|Getroom2ds))
  (bind _room3d (Variables|Default|Getroom3d))
  (bind _room4d_ (Variables|Default|Getroom4d%20))
  (bind _maxy_2 (Variables|Default|GetMaxY))
  (bind _tilesize (Variables|Default|GetTileSize))
  (bind _returnvalue_2 (* _maxx _maxy_2))
  ;[1 1 1] disable shadow casting by the floor(helps performance)
  (Rendering|SetCastShadow (Variables|Default|Getroom2ds) false)
  ;[1 1 1] Create board to build rooms on
  (Utilities|Array|Resize (Variables|Default|GetTileType) _returnvalue_2)
  (bind _output_get (Variables|Default|Setlength (- _returnvalue_2 1)))
  (for _index (range 0 _output_get)
    ;[1 1 1] Spawn rooms in checker board fashion
    (bind (_rowindex _colindex) (CallFunction|FlattenedtoNormalIndeces _index (Variables|Default|GetMaxY)))
    (Variables|Default|Setrow _rowindex)
    (Variables|Default|Setcol _colindex)
    (if (or (and (== (Math|Integer|%(Integer) _rowindex 2) 0) (== (Math|Integer|%(Integer) _colindex 2) 0)) (and (!= (Math|Integer|%(Integer) _rowindex 2) 0) (!= (Math|Integer|%(Integer) _colindex 2) 0)))
      ;[1 1 1] 20 percent chance a room spawns
      (if (<= (Math|Random|RandomIntegerinRange 0 (Variables|Default|GetMaxY)) (/ (Variables|Default|GetMaxY) 5))
        ;[1 1 1] Spawns a room and then gets the door positions for that room and the center position for that room also the array position of the room
        (if (== _returnvalue 0)
          (Components|InstancedStaticMesh|AddInstance _room_1d (Math|Conversions|ToTransform(Vector) (Math|Vector|MakeVector (Math|Conversions|ToFloat(Integer) (* (/ _index _maxy) _tilesize)) (Math|Conversions|ToFloat(Integer) (* (Math|Integer|%(Integer) _index _maxy) _tilesize)) 0.0)))
          (bind _output_get_2 (Variables|Default|Setroom%20 (Utilities|Struct|MakeRoomArrayItem (Variables|Default|Getcol) (Variables|Default|Getrow) (Transformation|GetSocketLocation _room_1d "Center"))))
          (Utilities|Array|Add (Variables|Default|GetRooms) _output_get_2)
          (Utilities|Array|Clear (Variables|Default|GetDoors))
          (Utilities|Array|Add (Variables|Default|GetDoors) (Transformation|GetSocketLocation _room_1d "Door 1"))
          (Utilities|Array|Add (Variables|Default|GetDoor%20positions) (Utilities|Struct|MakeRoomDoorpositions (Variables|Default|GetDoors)))
          (elif (== _returnvalue 1)
            (Components|InstancedStaticMesh|AddInstance _room2d (Math|Conversions|ToTransform(Vector) (Math|Vector|MakeVector (Math|Conversions|ToFloat(Integer) (* (/ _index _maxy) _tilesize)) (Math|Conversions|ToFloat(Integer) (* (Math|Integer|%(Integer) _index _maxy) _tilesize)) 0.0)))
            (bind _output_get_3 (Variables|Default|Setroom%20 (Utilities|Struct|MakeRoomArrayItem (Variables|Default|Getcol) (Variables|Default|Getrow) (Transformation|GetSocketLocation _room2d "Center"))))
            (Utilities|Array|Add (Variables|Default|GetRooms) _output_get_3)
            (Utilities|Array|Clear (Variables|Default|GetDoors))
            (Utilities|Array|Add (Variables|Default|GetDoors) (Transformation|GetSocketLocation _room2d "Door 1"))
            (Utilities|Array|Add (Variables|Default|GetDoors) (Transformation|GetSocketLocation _room2d "Door 2"))
            (Utilities|Array|Add (Variables|Default|GetDoor%20positions) (Utilities|Struct|MakeRoomDoorpositions (Variables|Default|GetDoors)))
            (elif (== _returnvalue 2)
              (Components|InstancedStaticMesh|AddInstance _room2ds (Math|Conversions|ToTransform(Vector) (Math|Vector|MakeVector (Math|Conversions|ToFloat(Integer) (* (/ _index _maxy) _tilesize)) (Math|Conversions|ToFloat(Integer) (* (Math|Integer|%(Integer) _index _maxy) _tilesize)) 0.0)))
              (bind _output_get_4 (Variables|Default|Setroom%20 (Utilities|Struct|MakeRoomArrayItem (Variables|Default|Getcol) (Variables|Default|Getrow) (Transformation|GetSocketLocation _room2ds "Center"))))
              (Utilities|Array|Add (Variables|Default|GetRooms) _output_get_4)
              (Utilities|Array|Clear (Variables|Default|GetDoors))
              (Utilities|Array|Add (Variables|Default|GetDoors) (Transformation|GetSocketLocation _room2ds "Door 1"))
              (Utilities|Array|Add (Variables|Default|GetDoors) (Transformation|GetSocketLocation _room2ds "Door 2"))
              (Utilities|Array|Add (Variables|Default|GetDoor%20positions) (Utilities|Struct|MakeRoomDoorpositions (Variables|Default|GetDoors)))
              (elif (== _returnvalue 3)
                (Components|InstancedStaticMesh|AddInstance _room3d (Math|Conversions|ToTransform(Vector) (Math|Vector|MakeVector (Math|Conversions|ToFloat(Integer) (* (/ _index _maxy) _tilesize)) (Math|Conversions|ToFloat(Integer) (* (Math|Integer|%(Integer) _index _maxy) _tilesize)) 0.0)))
                (bind _output_get_5 (Variables|Default|Setroom%20 (Utilities|Struct|MakeRoomArrayItem (Variables|Default|Getcol) (Variables|Default|Getrow) (Transformation|GetSocketLocation _room3d "Center"))))
                (Utilities|Array|Add (Variables|Default|GetRooms) _output_get_5)
                (Utilities|Array|Clear (Variables|Default|GetDoors))
                (Utilities|Array|Add (Variables|Default|GetDoors) (Transformation|GetSocketLocation _room3d "Door 1"))
                (Utilities|Array|Add (Variables|Default|GetDoors) (Transformation|GetSocketLocation _room3d "Door 2"))
                (Utilities|Array|Add (Variables|Default|GetDoors) (Transformation|GetSocketLocation _room3d "Door 3"))
                (Utilities|Array|Add (Variables|Default|GetDoor%20positions) (Utilities|Struct|MakeRoomDoorpositions (Variables|Default|GetDoors)))
                (else
                  (Components|InstancedStaticMesh|AddInstance _room4d_ (Math|Conversions|ToTransform(Vector) (Math|Vector|MakeVector (Math|Conversions|ToFloat(Integer) (* (/ _index _maxy) _tilesize)) (Math|Conversions|ToFloat(Integer) (* (Math|Integer|%(Integer) _index _maxy) _tilesize)) 0.0)))
                  (bind _output_get_6 (Variables|Default|Setroom%20 (Utilities|Struct|MakeRoomArrayItem (Variables|Default|Getcol) (Variables|Default|Getrow) (Transformation|GetSocketLocation _room4d_ "Center"))))
                  (Utilities|Array|Add (Variables|Default|GetRooms) _output_get_6)
                  (Utilities|Array|Clear (Variables|Default|GetDoors))
                  (Utilities|Array|Add (Variables|Default|GetDoors) (Transformation|GetSocketLocation _room4d_ "Door 1"))
                  (Utilities|Array|Add (Variables|Default|GetDoors) (Transformation|GetSocketLocation _room4d_ "Door 2"))
                  (Utilities|Array|Add (Variables|Default|GetDoors) (Transformation|GetSocketLocation _room4d_ "Door 3"))
                  (Utilities|Array|Add (Variables|Default|GetDoors) (Transformation|GetSocketLocation _room4d_ "Door 4"))
                  (Utilities|Array|Add (Variables|Default|GetDoor%20positions) (Utilities|Struct|MakeRoomDoorpositions (Variables|Default|GetDoors)))))))))))
  (CallFunction|CreateSpanningTree (Variables|Default|GetRooms)))

(fn NormalIndecestoFlattenedIndex
  (params (maxY :type Integer) (rowIndex :type Integer) (colIndex :type Integer))
  (return (+ (* maxY rowIndex) colIndex)))

(fn FlattenedtoNormalIndeces
  (params (FlattenedIndex :type Integer) (MaxY :type Integer))
  (return (/ FlattenedIndex MaxY) (Math|Integer|%(Integer) FlattenedIndex MaxY)))

(fn CreateSpanningTree
  (params (Pos_ind :type Array%20of%20Room%20Array%20Item%20Structures))
  (bind _output_get (LocalVariables|SetRest Pos_ind))
  (Utilities|Array|Add (LocalVariables|GetDone) (Utilities|Array|Get(acopy) _output_get))
  (Utilities|Array|RemoveIndex (LocalVariables|GetRest))
  (while (!= (Utilities|Array|Length (LocalVariables|GetRest)) 0)
    (bind (_index_done _index_search) (CallFunction|FindMinDistBetweenArrays (LocalVariables|GetDone) (LocalVariables|GetRest)))
    (Utilities|Array|Add (Variables|Default|GetEdges) (Utilities|Struct|MakeIntVector (Math|Float|Truncate (.Z (Math|Vector|BreakVector (.centerposition (Utilities|Array|Get(acopy) (LocalVariables|GetDone) _index_done))))) (Math|Float|Truncate (.Z (Math|Vector|BreakVector (.centerposition (Utilities|Array|Get(acopy) (LocalVariables|GetRest) _index_search)))))))
    (Utilities|Array|Add (LocalVariables|GetDone) (Utilities|Array|Get(acopy) (LocalVariables|GetRest) _index_search))
    (Utilities|Array|RemoveIndex (LocalVariables|GetRest) _index_search)))

(fn FindMinDistBetweenArrays
  (params (Done :type Array%20of%20Room%20Array%20Item%20Structures) (To%20search :type Array%20of%20Room%20Array%20Item%20Structures))
  (return 0 0))

(fn CreateCorridor)

(fn SpawnHallway)