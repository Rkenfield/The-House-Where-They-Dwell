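; Side table Blueprint for level generation that spawns decorations on its mesh sockets at BeginPlay.
; It loops over all socket names, giving Deco1 and Deco2 each a one-in-three chance of a VaseSpawn actor, while Deco3 always gets a HallwayTableDeco.
; Each actor spawns at its socket's world transform.
; A disconnected random check for the Deco3 spawn never runs.
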(event EventBeginPlay
  ;[1 1 1] Spawn a vase
  (for _array_element (Transformation|GetAllSocketNames (Variables|Default|GetSideTable))
    (Utilities|FlowControl|Sequence
      (:then_0
        (if (Utilities|Name|Equal(Name) _array_element "Deco1")
          (if (== (Math|Random|RandomInteger 3) 0)
            (Game|SpawnActorfromClass "/Game/Blueprints/LevelGeneration/VaseSpawn.VaseSpawn_C" (Transformation|GetSocketTransform (Variables|Default|GetSideTable) _array_element "RTS_World") "Undefined" 0 0 :!label _label))))
      (:then_1
        (if (Utilities|Name|Equal(Name) _array_element "Deco2")
          (if (== (Math|Random|RandomInteger 3) 0)
            (goto _label))))
      (:then_2
        (if (Utilities|Name|Equal(Name) _array_element "Deco3")
          (Game|SpawnActorfromClass "/Game/Blueprints/LevelGeneration/HallwayTableDeco.HallwayTableDeco_C" (Transformation|GetSocketTransform (Variables|Default|GetSideTable) _array_element "RTS_World") "Undefined" 0 0 0 0))))))

(fn ConstructionScript)