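; Two-door hallway piece for procedural house generation that randomly walls off its doorways or attaches rooms at mesh sockets.
; On BeginPlay it reseeds a random stream, plugs doors flagged as fake, then picks a layout respecting those flags.
; Spawned rooms register in THWDGameMode's room array and count.
; The roll's Max of 3 yields only 0–2, so the both-rooms layout (case 3) never occurs.
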(event EventBeginPlay
  (bind _stream (Variables|Default|GetStream))
  (Class|KismetMathLibrary|SeedRandomStream _stream)
  (bind _output_get (Variables|Default|SetRoomChoice (Class|KismetMathLibrary|RandomIntegerfromStream 3 _stream)))
  (CallFunction|PlugEmptyDoors)
  (CallFunction|SpawnRooms _output_get))

(fn ConstructionScript
  (|CallParentFunction))

(fn PlugEmptyDoors
  (bind _staticmesh (Variables|Default|GetStaticMesh))
  (bind _staticmesh_2 (Variables|Default|GetStaticMesh))
  (bind _staticmesh_3 (Variables|Default|GetStaticMesh))
  (bind _staticmesh_4 (Variables|Default|GetStaticMesh))
  (bind _returnvalue (Transformation|GetSocketTransform _staticmesh "Door1" "RTS_World"))
  (bind _returnvalue_2 (Transformation|GetSocketTransform _staticmesh_2 "Door2" "RTS_World"))
  (bind _returnvalue_3 (Transformation|GetSocketTransform _staticmesh_3 "Door2" "RTS_World"))
  (bind _returnvalue_4 (Transformation|GetSocketTransform _staticmesh_4 "Door1" "RTS_World"))
  (if (Variables|Default|GetSpawnFakeDoorAt1)
    (if (Variables|Default|GetSpawnFakeDoorAt2)
      (Game|SpawnActorfromClass "/Game/Blueprints/LevelGeneration/Door_or_FilledWall.Door_or_FilledWall_C" (Math|Transform|MakeTransform (.location _returnvalue) (.rotation _returnvalue) "1,1,1") "Undefined" 0 0)
      (Game|SpawnActorfromClass "/Game/Blueprints/LevelGeneration/Door_or_FilledWall.Door_or_FilledWall_C" (Math|Transform|MakeTransform (.location _returnvalue_2) (.rotation _returnvalue_2) "1,1,1") "Undefined" 0 0)
      (else
        (Game|SpawnActorfromClass "/Game/Blueprints/LevelGeneration/Door_or_FilledWall.Door_or_FilledWall_C" (Math|Transform|MakeTransform (.location _returnvalue_4) (.rotation _returnvalue_4) "1,1,1") "Undefined" 0 0)))
    (elif (Variables|Default|GetSpawnFakeDoorAt2)
      (Game|SpawnActorfromClass "/Game/Blueprints/LevelGeneration/Door_or_FilledWall.Door_or_FilledWall_C" (Math|Transform|MakeTransform (.location _returnvalue_3) (.rotation _returnvalue_3) "1,1,1") "Undefined" 0 0))))

(fn SpawnRooms
  (params (Choice :type Integer))
  (bind _staticmesh (Variables|Default|GetStaticMesh))
  (bind _staticmesh_2 (Variables|Default|GetStaticMesh))
  (bind _staticmesh_3 (Variables|Default|GetStaticMesh))
  (bind _staticmesh_4 (Variables|Default|GetStaticMesh))
  (bind _staticmesh_5 (Variables|Default|GetStaticMesh))
  (bind _staticmesh_6 (Variables|Default|GetStaticMesh))
  (bind _staticmesh_7 (Variables|Default|GetStaticMesh))
  (bind _staticmesh_8 (Variables|Default|GetStaticMesh))
  (bind _returnvalue (Transformation|GetSocketTransform _staticmesh_3 "Door1" "RTS_World"))
  (bind _returnvalue_2 (Transformation|GetSocketTransform _staticmesh_4 "Door2" "RTS_World"))
  (bind _returnvalue_3 (Transformation|GetSocketTransform _staticmesh_7 "Room1Center" "RTS_World"))
  (bind _returnvalue_4 (Transformation|GetSocketTransform _staticmesh_6 "Room1Center" "RTS_World"))
  (bind _returnvalue_5 (Transformation|GetSocketTransform _staticmesh_5 "Room2Center" "RTS_World"))
  (bind _returnvalue_6 (Transformation|GetSocketTransform _staticmesh_2 "Room2Center" "RTS_World"))
  (bind _returnvalue_7 (Transformation|GetSocketTransform _staticmesh "Door1" "RTS_World"))
  (bind _returnvalue_8 (Transformation|GetSocketTransform _staticmesh_8 "Door2" "RTS_World"))
  (if (not (and (Math|Boolean|Equal(Boolean) (Variables|Default|GetSpawnFakeDoorAt1) true) (Math|Boolean|Equal(Boolean) (Variables|Default|GetSpawnFakeDoorAt2) true)))
    (switch int Choice
      (:0
        (Game|SpawnActorfromClass "/Game/Blueprints/LevelGeneration/Door_or_FilledWall.Door_or_FilledWall_C" (Math|Transform|MakeTransform (.location _returnvalue_7) (.rotation _returnvalue_7) "1,1,1") "Undefined" 0 0)
        (Game|SpawnActorfromClass "/Game/Blueprints/LevelGeneration/Door_or_FilledWall.Door_or_FilledWall_C" (Math|Transform|MakeTransform (.location _returnvalue_8) (.rotation _returnvalue_8) "1,1,1") "Undefined" 0 0))
      (:1
        (if (Math|Boolean|Equal(Boolean) (Variables|Default|GetSpawnFakeDoorAt1) false)
          (bind _returnvalue_9 (Game|SpawnActorfromClass "/Game/Blueprints/LevelGeneration/Room.Room_C" (Math|Transform|MakeTransform (.location _returnvalue_4) (.rotation _returnvalue_4) "1,1,1") "Undefined" 0 0))
          (CallFunction|AddRoomtoArray _returnvalue_9)
          (Game|SpawnActorfromClass "/Game/Blueprints/LevelGeneration/Door_or_FilledWall.Door_or_FilledWall_C" (Math|Transform|MakeTransform (.location _returnvalue_2) (.rotation _returnvalue_2) "1,1,1") "Undefined" 0 0)))
      (:2
        (if (Math|Boolean|Equal(Boolean) (Variables|Default|GetSpawnFakeDoorAt2) false)
          (bind _returnvalue_10 (Game|SpawnActorfromClass "/Game/Blueprints/LevelGeneration/Room.Room_C" (Math|Transform|MakeTransform (.location _returnvalue_5) (.rotation _returnvalue_5) "1,1,1") "Undefined" 0 0))
          (CallFunction|AddRoomtoArray _returnvalue_10)
          (Game|SpawnActorfromClass "/Game/Blueprints/LevelGeneration/Door_or_FilledWall.Door_or_FilledWall_C" (Math|Transform|MakeTransform (.location _returnvalue) (.rotation _returnvalue) "1,1,1") "Undefined" 0 0)))
      (:3
        (if (and (Math|Boolean|Equal(Boolean) (Variables|Default|GetSpawnFakeDoorAt1) false) (Math|Boolean|Equal(Boolean) (Variables|Default|GetSpawnFakeDoorAt2) false))
          (bind _returnvalue_11 (Game|SpawnActorfromClass "/Game/Blueprints/LevelGeneration/Room.Room_C" (Math|Transform|MakeTransform (.location _returnvalue_3) (.rotation _returnvalue_3) "1,1,1") "Undefined" 0 0))
          (bind _returnvalue_12 (Game|SpawnActorfromClass "/Game/Blueprints/LevelGeneration/Room.Room_C" (Math|Transform|MakeTransform (.location _returnvalue_6) (.rotation _returnvalue_6) "1,1,1") "Undefined" 0 0))
          (CallFunction|AddRoomtoArray _returnvalue_11)
          (CallFunction|AddRoomtoArray _returnvalue_12))))))

(fn AddRoomtoArray
  (params (RoomToAdd :type Room%20Object%20Reference))
  (bind _asthwdgame_mode (Utilities|Casting|CastToTHWDGameMode (Game|GetGameMode)))
  (Utilities|Array|Add (Variables|/Game/Blueprints/THWDGameMode.THWDGameMode_C|GetRoomsinHouse _asthwdgame_mode) (Utilities|Struct|MakeRooms RoomToAdd))
  (Variables|/Game/Blueprints/THWDGameMode.THWDGameMode_C|SetNumOfRooms _asthwdgame_mode (+ (Variables|/Game/Blueprints/THWDGameMode.THWDGameMode_C|GetNumOfRooms _asthwdgame_mode) 1)))