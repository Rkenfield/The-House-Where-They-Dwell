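; Level generator actor that builds a three-floor layout (basement, ground, upper) at BeginPlay.
; It sorts each floor component's sockets by name prefix into door, always-fill and hall-fill transforms.
; Each door randomly spawns a room or an index-matched hall fill, while always-fills spawn walls except index 13.
; The upper floor also spawns a lair room and excludes HallFill13; the MaxRooms limit is passed but never used.
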(event EventBeginPlay
  (CallFunction|GenerateBasementArrays)
  (CallFunction|GenerateGroundArrays)
  (CallFunction|GenerateUpperArrays))

(event Collision|EventActorBeginOverlap
  (params (OtherActor :type Actor%20Object%20Reference)))

(event EventTick
  (params (DeltaSeconds :type Float%20%28single-precision%29)))

(fn ConstructionScript)

(fn GenerateBasementArrays
  (for _array_element (Transformation|GetAllSocketNames (Variables|Default|GetBasement))
    (if (Utilities|Enum|Equal(Enum) (Utilities|String|GetSubstring (Utilities|String|ToString(Name) _array_element) 0 4) "Door")
      (Utilities|Array|Add (Variables|Default|GetBasementDoorSocketNames) _array_element)
      (Utilities|Array|Add (Variables|Default|GetBasementRoomSocketTransforms) (Transformation|GetSocketTransform (Variables|Default|GetBasement) _array_element "RTS_World"))
      (elif (Utilities|Enum|Equal(Enum) (Utilities|String|GetSubstring (Utilities|String|ToString(Name) _array_element) 0 10) "AlwaysFill")
        (Utilities|Array|Add (Variables|Default|GetBasementFillSocketTransforms) (Transformation|GetSocketTransform (Variables|Default|GetBasement) _array_element "RTS_World"))
        (elif (Utilities|Enum|Equal(Enum) (Utilities|String|GetSubstring (Utilities|String|ToString(Name) _array_element) 0 8) "HallFill")
          (Utilities|Array|Add (Variables|Default|GetBasementPossibleFillSocketTransforms) (Transformation|GetSocketTransform (Variables|Default|GetBasement) _array_element "RTS_World"))))))
  (CallFunction|SpawnRooms (Variables|Default|GetBasementRoomSocketTransforms) (Variables|Default|GetMaxRooms) (Variables|Default|GetChanceToSpawnRoom) (Variables|Default|GetBasementPossibleFillSocketTransforms))
  (CallFunction|SpawnFills (Variables|Default|GetBasementFillSocketTransforms)))

(fn GenerateGroundArrays
  (for _array_element (Transformation|GetAllSocketNames (Variables|Default|GetGround))
    (if (Utilities|Enum|Equal(Enum) (Utilities|String|GetSubstring (Utilities|String|ToString(Name) _array_element) 0 4) "Door")
      (Utilities|Array|Add (Variables|Default|GetGroundDoorSocketNames) _array_element)
      (Utilities|Array|Add (Variables|Default|GetGroundRoomSocketTransforms) (Transformation|GetSocketTransform (Variables|Default|GetGround) _array_element "RTS_World"))
      (elif (Utilities|Enum|Equal(Enum) (Utilities|String|GetSubstring (Utilities|String|ToString(Name) _array_element) 0 10) "AlwaysFill")
        (Utilities|Array|Add (Variables|Default|GetGroundFillSocketTransforms) (Transformation|GetSocketTransform (Variables|Default|GetGround) _array_element "RTS_World"))
        (elif (Utilities|Enum|Equal(Enum) (Utilities|String|GetSubstring (Utilities|String|ToString(Name) _array_element) 0 8) "HallFill")
          (Utilities|Array|Add (Variables|Default|GetGroundPossibleFillSocketTransforms) (Transformation|GetSocketTransform (Variables|Default|GetGround) _array_element "RTS_World"))))))
  (CallFunction|SpawnRooms (Variables|Default|GetGroundRoomSocketTransforms) (Variables|Default|GetMaxRooms) (Variables|Default|GetChanceToSpawnRoom) (Variables|Default|GetGroundPossibleFillSocketTransforms))
  (CallFunction|SpawnFills (Variables|Default|GetGroundFillSocketTransforms)))

(fn GenerateUpperArrays
  (for _array_element (Transformation|GetAllSocketNames (Variables|Default|GetUpper))
    (if (Utilities|Enum|Equal(Enum) (Utilities|String|GetSubstring (Utilities|String|ToString(Name) _array_element) 0 4) "Door")
      (Utilities|Array|Add (Variables|Default|GetUpperDoorSocketNames) _array_element)
      (Utilities|Array|Add (Variables|Default|GetUpperRoomSocketTransforms) (Transformation|GetSocketTransform (Variables|Default|GetUpper) _array_element "RTS_World"))
      (else
        ;[1 1 1] Maybe?????
        (if (Utilities|Enum|Equal(Enum) (Utilities|String|GetSubstring (Utilities|String|ToString(Name) _array_element) 0 6) "SWLair")
          (Game|SpawnActorfromClass "/Game/Blueprints/LevelGeneration/Room_SWLair.Room_SWLair_C" (Transformation|GetSocketTransform (Variables|Default|GetUpper) _array_element "RTS_World") "Undefined" 0 0)
          (elif (Utilities|Enum|Equal(Enum) (Utilities|String|GetSubstring (Utilities|String|ToString(Name) _array_element) 0 10) "AlwaysFill")
            (Utilities|Array|Add (Variables|Default|GetUpperFillSocketTransforms) (Transformation|GetSocketTransform (Variables|Default|GetUpper) _array_element "RTS_World"))
            (elif (and (Utilities|Enum|Equal(Enum) (Utilities|String|GetSubstring (Utilities|String|ToString(Name) _array_element) 0 8) "HallFill") (Utilities|Enum|NotEqual(Enum) (Utilities|String|ToString(Name) _array_element) "HallFill13"))
              (Utilities|Array|Add (Variables|Default|GetUpperPossibleFillSocketTransforms) (Transformation|GetSocketTransform (Variables|Default|GetUpper) _array_element "RTS_World"))))))))
  (CallFunction|SpawnRooms (Variables|Default|GetUpperRoomSocketTransforms) (Variables|Default|GetMaxRooms) (Variables|Default|GetChanceToSpawnRoom) (Variables|Default|GetUpperPossibleFillSocketTransforms))
  (CallFunction|SpawnFills (Variables|Default|GetUpperFillSocketTransforms)))

(fn SpawnRooms
  (params (RoomTransformArray :type Array%20of%20Transforms) (MaxRooms :type Integer) (Chance :type Integer) (FloorPossibleFills :type Array%20of%20Transforms))
  (bind _stream (Variables|Default|GetStream))
  (for (_array_element _array_index) RoomTransformArray
    (Class|KismetMathLibrary|SeedRandomStream _stream)
    (if (== (Class|KismetMathLibrary|RandomIntegerfromStream (- Chance 1) _stream) 0)
      (Game|SpawnActorfromClass "/Game/Blueprints/LevelGeneration/Room.Room_C" _array_element "Undefined" 0 0)
      (else
        (Game|SpawnActorfromClass "/Game/Blueprints/LevelGeneration/Door_or_FilledWall_JacobTest.Door_or_FilledWall_JacobTest_C" (Utilities|Array|Get(acopy) FloorPossibleFills _array_index) "Undefined" 0 0)))))

(fn SpawnFills
  (params (FillLocations :type Array%20of%20Transforms))
  (for (_array_element _array_index) FillLocations
    (if (!= _array_index 13)
      (Game|SpawnActorfromClass "/Game/Blueprints/LevelGeneration/Door_or_FilledWall_JacobTest.Door_or_FilledWall_JacobTest_C" _array_element "Undefined" 0 0))))