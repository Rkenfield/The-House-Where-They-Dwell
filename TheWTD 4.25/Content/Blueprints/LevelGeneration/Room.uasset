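; Room is a level-generation Blueprint that populates its doorways when play begins.
; On BeginPlay it loops over every socket on its static mesh and spawns an actor at that socket's world transform.
; The socket named Door1 receives a BP_Door, while every other socket receives a Door_or_FilledWall, so door placement is driven by the mesh's sockets.
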(event EventBeginPlay
  (for _array_element (Transformation|GetAllSocketNames (Variables|Default|GetStaticMesh))
    (if (Utilities|Name|NotEqual(Name) _array_element "Door1")
      (Game|SpawnActorfromClass "/Game/Blueprints/LevelGeneration/Door_or_FilledWall.Door_or_FilledWall_C" (Math|Transform|MakeTransform (.location (Transformation|GetSocketTransform (Variables|Default|GetStaticMesh) _array_element "RTS_World")) (.rotation (Transformation|GetSocketTransform (Variables|Default|GetStaticMesh) _array_element "RTS_World")) "1,1,1") "Undefined" 0 0)
      (else
        (Game|SpawnActorfromClass "/Game/Blueprints/Blueprints/BP_Door.BP_Door_C" (Math|Transform|MakeTransform (.location (Transformation|GetSocketTransform (Variables|Default|GetStaticMesh) _array_element "RTS_World")) (.rotation (Transformation|GetSocketTransform (Variables|Default|GetStaticMesh) _array_element "RTS_World")) "1,1,1") "Undefined" 0 0)))))

(fn ConstructionScript)