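; Bedroom room piece for level generation that furnishes itself from static mesh sockets and sets its room acoustics.
; On BeginPlay it loops the socket names, spawning a door at Door1, scaled-up dressers at the two Dresser sockets, and Door_or_FilledWall at every other socket.
; Overlapping its Box activates a small-room reverb effect, with no deactivation in this graph.
; An unconnected drawer-material loop never runs.
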(event OnComponentBeginOverlap(Box)
  (params (OverlappedComponent :type Primitive%20Component%20Object%20Reference) (OtherActor :type Actor%20Object%20Reference) (OtherComp :type Primitive%20Component%20Object%20Reference) (OtherBodyIndex :type Integer) (bFromSweep :type Boolean) (SweepResult :type Hit%20Result%20Structure%20%28by%20ref%29))
  (Class|GameplayStatics|ActivateReverbEffect "/Game/Audio/Reverb/SmallRoom.SmallRoom" "Bedroom01Verb" 0.0 1.0 1.0))

(event EventBeginPlay
  (bind _staticmesh (Variables|Default|GetStaticMesh))
  (for _array_element (Transformation|GetAllSocketNames (Variables|Default|GetStaticMesh))
    (if (Utilities|Name|NotEqual(Name) _array_element "Door1")
      (if (Utilities|Name|Equal(Name) _array_element "Dresser1")
        (Game|SpawnActorfromClass "/Game/Blueprints/Blueprints/BP_Dresser.BP_Dresser_C" (Math|Transform|MakeTransform (.location (Transformation|GetSocketTransform _staticmesh _array_element "RTS_World")) (.rotation (Transformation|GetSocketTransform _staticmesh _array_element "RTS_World")) "1.750000,1.750000,1.750000") "Undefined" 0 0)
        (elif (Utilities|Name|Equal(Name) _array_element "Dresser2")
          (Game|SpawnActorfromClass "/Game/Blueprints/Blueprints/BP_Dresser.BP_Dresser_C" (Math|Transform|MakeTransform (.location (Transformation|GetSocketTransform _staticmesh _array_element "RTS_World")) (.rotation (Transformation|GetSocketTransform _staticmesh _array_element "RTS_World")) "1.750000,1.750000,1.750000") "Undefined" 0 0)
          (else
            (Game|SpawnActorfromClass "/Game/Blueprints/LevelGeneration/Door_or_FilledWall.Door_or_FilledWall_C" (Math|Transform|MakeTransform (.location (Transformation|GetSocketTransform (Variables|Default|GetStaticMesh) _array_element "RTS_World")) (.rotation (Transformation|GetSocketTransform (Variables|Default|GetStaticMesh) _array_element "RTS_World")) "1,1,1") "Undefined" 0 0))))
      (else
        (Game|SpawnActorfromClass "/Game/Blueprints/Blueprints/BP_Door.BP_Door_C" (Math|Transform|MakeTransform (.location (Transformation|GetSocketTransform (Variables|Default|GetStaticMesh) _array_element "RTS_World")) (.rotation (Transformation|GetSocketTransform (Variables|Default|GetStaticMesh) _array_element "RTS_World")) "1,1,1") "Undefined" 0 0)))))

(fn ConstructionScript)