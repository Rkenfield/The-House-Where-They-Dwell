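; Test level generator that, on BeginPlay, randomly populates an upper floor with rooms at the Upper component's sockets.
; Sockets are grouped by name prefix (outside, inside, always-fill, hall fill), with the first, second and last groups selection-sorted by embedded number.
; Big rooms claim outside slots, often reserving the preceding one, then regular rooms follow, favoring inside slots.
; Door-or-filled-wall actors cover leftover and always-fill sockets.
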(event EventBeginPlay
  (CallFunction|GenerateUpperArrays))

(event Collision|EventActorBeginOverlap
  (params (OtherActor :type Actor%20Object%20Reference)))

(event EventTick
  (params (DeltaSeconds :type Float%20%28single-precision%29)))

(fn ConstructionScript)

(fn GenerateUpperArrays
  (for _array_element (Transformation|GetAllSocketNames (Variables|Default|GetUpper))
    (if (Utilities|Enum|Equal(Enum) (Utilities|String|GetSubstring (Utilities|String|ToString(Name) _array_element) 0) "O")
      (Utilities|Array|Add (LocalVariables|GetUpperOutsideRooms) _array_element)
      (elif (Utilities|Enum|Equal(Enum) (Utilities|String|GetSubstring (Utilities|String|ToString(Name) _array_element) 0) "I")
        (Utilities|Array|Add (LocalVariables|GetUpperInsideRooms) _array_element)
        (elif (Utilities|Enum|Equal(Enum) (Utilities|String|GetSubstring (Utilities|String|ToString(Name) _array_element) 0) "A")
          (Utilities|Array|Add (LocalVariables|GetUpperAlwaysFill) _array_element)
          (elif (Utilities|Enum|Equal(Enum) (Utilities|String|GetSubstring (Utilities|String|ToString(Name) _array_element) 0) "H")
            (Utilities|Array|Add (LocalVariables|GetUpperPossibleFills) _array_element))))))
  (bind _sorteddoors (CallFunction|SortRoomNameArray (LocalVariables|GetUpperOutsideRooms)))
  (bind _sorteddoors_2 (CallFunction|SortRoomNameArray (LocalVariables|GetUpperInsideRooms)))
  (bind _sorteddoors_3 (CallFunction|SortRoomNameArray (LocalVariables|GetUpperPossibleFills)))
  (CallFunction|SpawnRooms _sorteddoors (Variables|Default|GetMaxRooms) (Variables|Default|GetChanceToSpawnRoom) _sorteddoors_3 _sorteddoors_2)
  (CallFunction|SpawnFills (LocalVariables|GetUpperAlwaysFill)))

(fn SpawnRooms
  (params (OutsideRooms :type Array%20of%20Names) (MaxRooms :type Integer) (Chance :type Integer) (FloorPossibleFills :type Array%20of%20Names) (InsideRooms :type Array%20of%20Names))
  (bind _outsidespawnedboolarray (LocalVariables|GetOutsideSpawnedBoolArray))
  (for _array_element OutsideRooms
    (Utilities|Array|Add (LocalVariables|GetOutsideSpawnedBoolArray) false))
  (for _array_element_2 InsideRooms
    (Utilities|Array|Add (LocalVariables|GetinsideSpawnedBoolArray) false))
  ;[1 1 1] Large Rooms
  (while (< (LocalVariables|GetspawnedLarge) (Utilities|Array|Length (Variables|Default|GetBigRoomsUpper)))
    (LocalVariables|Setrandint (Math|Random|RandomIntegerinRange 1 (- (Utilities|Array|Length OutsideRooms) 1)))
    (bind _number (CallFunction|GetNumberfromName (Utilities|Array|Get(acopy) OutsideRooms (LocalVariables|Getrandint))))
    (if (Math|Boolean|ANDBoolean (Math|Boolean|Equal(Boolean) (Utilities|Array|Get(acopy) _outsidespawnedboolarray (LocalVariables|Getrandint)) false) (Math|Boolean|Equal(Boolean) (Utilities|Array|Get(acopy) _outsidespawnedboolarray (- (LocalVariables|Getrandint) 1)) false) (Math|Boolean|ORBoolean (!= _number 3) (!= _number 10) (!= _number 17) (!= _number 24)))
      (Game|SpawnActorfromClass (Utilities|Array|Get(acopy) (Variables|Default|GetBigRoomsUpper) (LocalVariables|GetspawnedLarge)) (Transformation|GetSocketTransform (Variables|Default|GetUpper) (Utilities|Array|Get(acopy) OutsideRooms (LocalVariables|Getrandint)) "RTS_World") "Undefined" 0 0)
      (Utilities|Array|SetArrayElem (LocalVariables|GetOutsideSpawnedBoolArray) (- (LocalVariables|Getrandint) 1) true)
      (Utilities|Array|SetArrayElem (LocalVariables|GetOutsideSpawnedBoolArray) (LocalVariables|Getrandint) true)
      (LocalVariables|SetspawnedLarge (+ (LocalVariables|GetspawnedLarge) 1))
      (Utilities|Array|SetArrayElem OutsideRooms (LocalVariables|Getrandint) "roomfilled")
      (elif (and (Math|Boolean|Equal(Boolean) (Utilities|Array|Get(acopy) _outsidespawnedboolarray (LocalVariables|Getrandint)) false) (Math|Boolean|ORBoolean (== _number 3) (== _number 10) (== _number 17) (== _number 24)))
        (Game|SpawnActorfromClass (Utilities|Array|Get(acopy) (Variables|Default|GetBigRoomsUpper) (LocalVariables|GetspawnedLarge)) (Transformation|GetSocketTransform (Variables|Default|GetUpper) (Utilities|Array|Get(acopy) OutsideRooms (LocalVariables|Getrandint)) "RTS_World") "Undefined" 0 0)
        (Utilities|Array|SetArrayElem (LocalVariables|GetOutsideSpawnedBoolArray) (LocalVariables|Getrandint) true)
        (LocalVariables|SetspawnedLarge (+ (LocalVariables|GetspawnedLarge) 1))
        (Utilities|Array|SetArrayElem OutsideRooms (LocalVariables|Getrandint) "roomfilled"))))
  ;[1 1 1] Regular rooms
  (while (< (LocalVariables|GetspawnedSmall) (Utilities|Array|Length (Variables|Default|GetRoomsUpper)))
    ;[1 1 1] choose inside or outside spawn area
    (if (== (Math|Random|RandomInteger 4) 0)
      (LocalVariables|Setrandint (Math|Random|RandomIntegerinRange 1 (- (Utilities|Array|Length OutsideRooms) 1)))
      (if (Math|Boolean|Equal(Boolean) (Utilities|Array|Get(acopy) (LocalVariables|GetOutsideSpawnedBoolArray) (LocalVariables|Getrandint)) false)
        (Game|SpawnActorfromClass (Utilities|Array|Get(acopy) (Variables|Default|GetRoomsUpper) (LocalVariables|GetspawnedSmall)) (Transformation|GetSocketTransform (Variables|Default|GetUpper) (Utilities|Array|Get(acopy) OutsideRooms (LocalVariables|Getrandint)) "RTS_World") "Undefined" 0 0)
        (Utilities|Array|SetArrayElem (LocalVariables|GetOutsideSpawnedBoolArray) (LocalVariables|Getrandint) true)
        (LocalVariables|SetspawnedSmall (+ (LocalVariables|GetspawnedSmall) 1))
        (Utilities|Array|SetArrayElem OutsideRooms (LocalVariables|Getrandint) "roomfilled"))
      (else
        (LocalVariables|Setrandint (Math|Random|RandomIntegerinRange 1 (- (Utilities|Array|Length InsideRooms) 1)))
        (if (Math|Boolean|Equal(Boolean) (Utilities|Array|Get(acopy) (LocalVariables|GetinsideSpawnedBoolArray) (LocalVariables|Getrandint)) false)
          (Game|SpawnActorfromClass (Utilities|Array|Get(acopy) (Variables|Default|GetRoomsUpper) (LocalVariables|GetspawnedSmall)) (Transformation|GetSocketTransform (Variables|Default|GetUpper) (Utilities|Array|Get(acopy) InsideRooms (LocalVariables|Getrandint)) "RTS_World") "Undefined" 0 0)
          (Utilities|Array|SetArrayElem (LocalVariables|GetinsideSpawnedBoolArray) (LocalVariables|Getrandint) true)
          (LocalVariables|SetspawnedSmall (+ (LocalVariables|GetspawnedSmall) 1))
          (Utilities|Array|SetArrayElem InsideRooms (LocalVariables|Getrandint) "roomfilled")))))
  (for _array_element_3 OutsideRooms
    (if (not (Utilities|Name|Equal(Name) _array_element_3 "roomfilled"))
      (bind _number_2 (CallFunction|GetNumberfromName _array_element_3))
      (Game|SpawnActorfromClass "/Game/Blueprints/LevelGeneration/Door_or_FilledWall_JacobTest.Door_or_FilledWall_JacobTest_C" (Transformation|GetSocketTransform (Variables|Default|GetUpper) (Utilities|Array|Get(acopy) FloorPossibleFills (- _number_2 1)) "RTS_World") "Undefined" 0 0)))
  (for _array_element_4 InsideRooms
    (if (not (Utilities|Name|Equal(Name) _array_element_4 "roomfilled"))
      (bind _number_3 (CallFunction|GetNumberfromName _array_element_4))
      (Game|SpawnActorfromClass "/Game/Blueprints/LevelGeneration/Door_or_FilledWall_JacobTest.Door_or_FilledWall_JacobTest_C" (Transformation|GetSocketTransform (Variables|Default|GetUpper) (Utilities|Array|Get(acopy) FloorPossibleFills (- _number_3 1)) "RTS_World") "Undefined" 0 0))))

(fn SpawnFills
  (params (AlwaysFillLocations :type Array%20of%20Names))
  (for _array_element AlwaysFillLocations
    (Game|SpawnActorfromClass "/Game/Blueprints/LevelGeneration/Door_or_FilledWall_JacobTest.Door_or_FilledWall_JacobTest_C" (Transformation|GetSocketTransform (Variables|Default|GetUpper) _array_element "RTS_World") "Undefined" 0 0)))

(fn SortRoomNameArray
  (params (DoorSocketNames :type Array%20of%20Names))
  (bind _unsorteddoornumbers (LocalVariables|GetunsortedDoorNumbers))
  (bind _unsorteddoornumbers_2 (LocalVariables|GetunsortedDoorNumbers))
  (bind _unsorteddoornumbers_3 (LocalVariables|GetunsortedDoorNumbers))
  (LocalVariables|SetUnsortedIndex 0)
  (bind _output_get (LocalVariables|SetSortedDoorNames DoorSocketNames))
  (for _array_element _output_get
    (bind _number (CallFunction|GetNumberfromName _array_element))
    (Utilities|Array|Add (LocalVariables|GetunsortedDoorNumbers) _number))
  (while (< (LocalVariables|GetUnsortedIndex) (- (Utilities|Array|Length DoorSocketNames) 1))
    (for (_array_element_2 _array_index) _unsorteddoornumbers
      (if (and (== (LocalVariables|GetUnsortedIndex) 0) (== _array_index 0))
        (LocalVariables|Setmin _array_element_2)
        (elif (>= _array_index (LocalVariables|GetUnsortedIndex))
          (if (< _array_element_2 (LocalVariables|Getmin))
            (LocalVariables|Setmin _array_element_2)
            (LocalVariables|SetTargetIndex _array_index)
            (LocalVariables|SetneedSwap true)))))
    (if (LocalVariables|GetneedSwap)
      (bind _output_get_2 (LocalVariables|SetSwapValue (Utilities|Array|Get(acopy) _unsorteddoornumbers_3 (LocalVariables|GetUnsortedIndex))))
      (bind _output_get_3 (LocalVariables|SetSwapValueName (Utilities|Array|Get(acopy) (LocalVariables|GetSortedDoorNames) (LocalVariables|GetUnsortedIndex))))
      (Utilities|Array|SetArrayElem (LocalVariables|GetSortedDoorNames) (LocalVariables|GetUnsortedIndex) (Utilities|Array|Get(acopy) (LocalVariables|GetSortedDoorNames) (LocalVariables|GetTargetIndex)))
      (Utilities|Array|SetArrayElem (LocalVariables|GetSortedDoorNames) (LocalVariables|GetTargetIndex) _output_get_3)
      (Utilities|Array|SetArrayElem _unsorteddoornumbers_2 (LocalVariables|GetUnsortedIndex) (Utilities|Array|Get(acopy) (LocalVariables|GetunsortedDoorNumbers) (LocalVariables|GetTargetIndex)))
      (Utilities|Array|SetArrayElem _unsorteddoornumbers_2 (LocalVariables|GetTargetIndex) _output_get_2)
      (LocalVariables|SetUnsortedIndex (+ (LocalVariables|GetUnsortedIndex) 1))
      (bind _output_get_4 (LocalVariables|Setmin (Utilities|Array|Get(acopy) _unsorteddoornumbers (LocalVariables|GetUnsortedIndex))))
      (LocalVariables|SetneedSwap false)
      (else
        (LocalVariables|SetUnsortedIndex (+ (LocalVariables|GetUnsortedIndex) 1))
        (LocalVariables|Setmin (Utilities|Array|Get(acopy) _unsorteddoornumbers_3 (LocalVariables|GetUnsortedIndex)))
        (LocalVariables|SetneedSwap false))))
  (return (LocalVariables|GetSortedDoorNames)))

(fn GetNumberfromName
  (params (InName :type Name))
  (Utilities|Array|Clear (LocalVariables|GetArrayofNumericValues))
  (for _array_element (Utilities|String|GetCharacterArrayfromString (Utilities|String|ToString(Name) InName))
    (if (Class|KismetStringLibrary|IsNumeric _array_element)
      (Utilities|Array|Add (LocalVariables|GetArrayofNumericValues) _array_element)))
  (return (Math|Conversions|ToInteger(Byte) (Utilities|String|JoinStringArray (LocalVariables|GetArrayofNumericValues) ""))))