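; Test level-generation wall actor that randomly dresses its WallFill mesh with a side table.
; On BeginPlay it scans the mesh's socket names and, for each starting with "Table", has a random chance to spawn a SideTable.
; The spawn transform always comes from the socket named exactly "Table", not the matched one.
; SpawnTable is empty, and socket-based random vase spawning is left disconnected.
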(event Custom|SpawnTable)

(event EventBeginPlay
  (bind _wallfill (Variables|Default|GetWallFill))
  (for _array_element (Transformation|GetAllSocketNames _wallfill)
    (if (Utilities|Enum|Equal(Enum) (Utilities|String|GetSubstring (Utilities|String|ToString(Name) _array_element) 0 5) "Table")
      (if (== (Math|Random|RandomInteger (Variables|Default|GetChanceToSpawn)) 0)
        (Game|SpawnActorfromClass "/Game/Blueprints/LevelGeneration/SideTable.SideTable_C" (Transformation|GetSocketTransform _wallfill "Table" "RTS_World") "Undefined" 0 0)))))

(fn ConstructionScript)