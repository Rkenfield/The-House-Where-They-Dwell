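; Multiplayer game mode that sets up up to four local split-screen players and assigns each a playable character.
; BeginPlay enables splitscreen, creates the players, then reads saved character choices from the game instance.
; Each choice selects one of the Player1–4 classes, and the matching controller possesses the existing actor of that class.
; SpawnPlayer repeats that lookup and possession for a calling controller that already has a pawn.
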(event Custom|SpawnPlayer
  (params (Controller :type Player%20Controller%20Object%20Reference))
  (bind _returnvalue (Class|GameplayStatics|GetPlayerControllerID Controller))
  (bind _returnvalue_2 (Game|GetPlayerController _returnvalue))
  ;[1 1 1] SpawnPlayer- Allows each player to take control of one of the playable characters when either '1' (keyboard) or 'Special Left Button' (Gamepad) is pressed
  (Utilities|IsValid (Pawn|GetControlledPawn Controller)
    (:Is%20Valid
      (bind _charindex (Class|BPIGameInstance|LoadCharData(Message) (Game|GetGameInstance)))
      (bind _returnvalue_3 (Actor|GetActorOfClass (Utilities|Select :Index (Utilities|Array|Get(acopy) _charindex _returnvalue) :Option%200 (Variables|Default|GetPlayer1) :Option%201 (Variables|Default|GetPlayer2) :Option%202 (Variables|Default|GetPlayer3) :Option%203 (Variables|Default|GetPlayer4))))
      (Utilities|IsValid _returnvalue_2
        (:Is%20Valid
          (Pawn|Possess _returnvalue_2 _returnvalue_3))))))

(event EventBeginPlay
  ;[1 1 1] Begin Play- Creates 4 players
  (Class|GameplayStatics|SetForceDisableSplitscreen false)
  (while (<= (Variables|Default|GetNoOfPlayers) 3)
    (bind _returnvalue (Class|GameplayStatics|CreatePlayer (Variables|Default|GetNoOfPlayers)))
    (Variables|Default|SetNoOfPlayers (+ (Variables|Default|GetNoOfPlayers) 1)))
  (bind _charindex (Class|BPIGameInstance|LoadCharData(Message) (Game|GetGameInstance)))
  (for (_array_element _array_index) _charindex
    (bind _returnvalue_2 (Actor|GetActorOfClass (Utilities|Select :Index _array_element :Option%200 (Variables|Default|GetPlayer1) :Option%201 (Variables|Default|GetPlayer2) :Option%202 (Variables|Default|GetPlayer3) :Option%203 (Variables|Default|GetPlayer4))))
    (Utilities|IsValid (Game|GetPlayerController _array_index)
      (:Is%20Valid
        (Pawn|Possess (Game|GetPlayerController _array_index) _returnvalue_2)))))

(fn ConstructionScript)