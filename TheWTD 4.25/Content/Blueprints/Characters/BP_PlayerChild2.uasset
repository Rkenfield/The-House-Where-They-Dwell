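; Second-player character Blueprint, a child of BP_PlayerParent, handling hover prompts and HUD for local multiplayer.
; Tick line-traces from the follow camera, using actor tags and DoOnce gates to show or clear widgets for small spiders, items and computer stations.
; BeginPlay sets camera aspect ratio by player count and creates the Player 2 HUD; HUDRefresh rebuilds it by controller ID.
; Nest detection and inventory swap, use and drop logic are disconnected.
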(event EventTick
  (params (DeltaSeconds :type Float%20%28single-precision%29))
  (bind _self self)
  (bind _followcamera (Variables|Default|GetFollowCamera))
  (bind _returnvalue (Pawn|GetController _self))
  (bind _returnvalue_2 (Transformation|GetWorldLocation _followcamera))
  (bind _aspc_multiplayer (Utilities|Casting|CastToPC_Multiplayer _returnvalue))
  ;[1 1 1] View Item Details on Hover (modified by Alex on 1-26-21)
  (Utilities|FlowControl|Sequence
    (:then_0
      (bind (_outhit _returnvalue_3) (Collision|LineTraceByChannel _returnvalue_2 (+ _returnvalue_2 (* (Math|Vector|GetForwardVector _followcamera) 2e+02)) "TraceTypeQuery2" false 0 "None"))
      (if _returnvalue_3 ; Did you hit an object?
        ;;[1 1 1] If you hit an actor.
        (bind _output_get (Variables|Default|SetHitActorHover (.hitactor _outhit)))
        (if (Actor|ActorHasTag _output_get "Spider") ; Does HitActorHover have the Spider tag?
          ;;;[1 1 1] If it's a spider minion
          (bind _asspider_minion (Utilities|Casting|CastToSpiderMinion (Variables|Default|GetHitActorHover)))
          (if (Variables|/Game/Blueprints/AI/SpiderWitch/Spider/SpiderMinion.SpiderMinion_C|GetSpiderSmall _asspider_minion)
            (Variables|Default|SetSpiderHover true)
            (Utilities|FlowControl|DoOnce false :!label _label
              (:Completed
                (bind _returnvalue_4 (UserInterface|CreateWidget "/Game/Blueprints/HUD/SpiderDestructionWidget.SpiderDestructionWidget_C" _aspc_multiplayer))
                (bind _output_get_2 (Variables|Default|SetSpiderDestructionWidget _returnvalue_4))
                (UserInterface|Viewport|AddtoPlayerScreen _output_get_2)))
            (else
              ;;[1 1 1] If you don't hit an actor.
              (bind _spiderdestructionwidget (Variables|Default|GetSpiderDestructionWidget :!label _label_2)
                (:then
                  (Widget|RemovefromParent _spiderdestructionwidget))
                (:else
                  _))
              (Variables|Default|SetSpiderHover false)
              (Utilities|FlowControl|Sequence
                (:then_0
                  (goto _label Reset))
                (:then_1
                  (if (Variables|Default|GetItemHover) :!label _label_3
                    (Widget|RemovefromParent (Variables|Default|GetItemHUD))
                    (Variables|Default|SetItemHover false)
                    (goto _label_4 Reset)
                    (elif (Variables|Default|GetNestHover)
                      (Widget|RemovefromParent (Variables|Default|GetNestWidget))
                      (Variables|Default|SetNestHover false)
                      (Utilities|FlowControl|DoOnce false) ; enters at Reset
                      (elif (Variables|Default|GetComputerStationHover)
                        (Widget|RemovefromParent (Variables|Default|GetComputerStationTextWidget))
                        (Variables|Default|SetComputerStationHover false)
                        (Utilities|FlowControl|Sequence
                          (:then_0
                            (goto _label_6 Reset))
                          (:then_1
                            (goto _label_5 Reset))))))))))
          (elif (Actor|ActorHasTag (Variables|Default|GetHitActorHover) "Item") ; Does HitActorHover have the Item tag?
            ;;;[1 1 1] If it's an item
            (bind _asbp_item (Utilities|Casting|CastToBP_Item (Variables|Default|GetHitActorHover)))
            (Variables|Default|SetItemHover true)
            (Utilities|FlowControl|DoOnce false :!label _label_4
              (:Completed
                (bind _returnvalue_5 (UserInterface|CreateWidget "/Game/Blueprints/HUD/ItemHUD.ItemHUD_C" _aspc_multiplayer (.name (Variables|/Game/Blueprints/Blueprints/Item/BP_Item.BP_Item_C|GetItemStructure _asbp_item)) (.description (Variables|/Game/Blueprints/Blueprints/Item/BP_Item.BP_Item_C|GetItemStructure _asbp_item)) (Variables|/Game/Blueprints/Blueprints/Item/BP_Item.BP_Item_C|GetQuantity _asbp_item)))
                (bind _output_get_3 (Variables|Default|SetItemHUD _returnvalue_5))
                (UserInterface|Viewport|AddtoPlayerScreen _output_get_3)))
            (elif (Actor|ActorHasTag (Variables|Default|GetHitActorHover) "ComputerStation") ; Is it a computer station?
              (bind _asbp_computer_station (Utilities|Casting|CastToBP_ComputerStation (Variables|Default|GetHitActorHover)))
              (if (Variables|/Game/Blueprints/Blueprints/BP_ComputerStation.BP_ComputerStation_C|GetCameraPlaced _asbp_computer_station) ; Has the camera already been placed?
                (Utilities|FlowControl|DoOnce false
                  (:Completed
                    (Widget|RemovefromParent (Variables|Default|GetComputerStationTextWidget)) ; Fixes an issue where the Upload footage widget won't go away after you place the camera.
                  ))
                (else
                  (Variables|Default|SetComputerStationHover true)
                  (if (Variables|Default|GetCameraEquipped)
                    (Utilities|FlowControl|DoOnce false :!label _label_5
                      (:Completed
                        (bind _returnvalue_6 (UserInterface|CreateWidget "/Game/Blueprints/HUD/ComputerStationTextWidgetB.ComputerStationTextWidgetB_C" _aspc_multiplayer))
                        (bind _output_get_4 (Variables|Default|SetComputerStationTextWidget _returnvalue_6))
                        (UserInterface|Viewport|AddtoPlayerScreen _output_get_4)))
                    (else
                      (Utilities|FlowControl|DoOnce false :!label _label_6
                        (:Completed
                          (bind _returnvalue_7 (UserInterface|CreateWidget "/Game/Blueprints/HUD/ComputerStationTextWidgetA.ComputerStationTextWidgetA_C" _aspc_multiplayer))
                          (bind _output_get_5 (Variables|Default|SetComputerStationTextWidget _returnvalue_7))
                          (UserInterface|Viewport|AddtoPlayerScreen _output_get_5))))))))))
        (elif (Variables|Default|GetSpiderHover)
          (goto _label_2)
          (else
            (goto _label_3)))))))

(event EventBeginPlay
  (bind _followcamera (Variables|Default|GetFollowCamera))
  ;[1 1 1] Creates Player Inventory
  ;;[1 1 1] Check to make sure there are at least 2 players so that the second HUD doesn't come up when testing with one player.
  ;;;[1 1 1] Sets player 2's aspect ratio based on if there are 1 or 2 players
  (bind _asbp_wtdgame_mode (Utilities|Casting|CastToBP_WTDGameMode (Game|GetGameMode)))
  (bind _returnvalue (Class|GameModeBase|GetNumPlayers _asbp_wtdgame_mode))
  (if (> _returnvalue 1)
    (Variables|/Script/Engine.CameraComponent|SetAspectRatio _followcamera (Variables|Default|GetTwoPlayerAspectRatio))
    (bind _returnvalue_2 (UserInterface|CreateWidget "/Game/Blueprints/HUD/Player2HUD.Player2HUD_C" (Game|GetPlayerController 1) (Variables|Default|GetInventoryComponent) (Math|Float|Truncate (Variables|Default|GetHealth))))
    (bind _output_get (Variables|Default|SetHUD_0 _returnvalue_2))
    (UserInterface|Viewport|AddtoPlayerScreen _output_get)
    (else
      (Variables|/Script/Engine.CameraComponent|SetAspectRatio _followcamera (Variables|Default|GetOnePlayerAspectRatio)))))

(event EventUpdateInventory
  ;[1 1 1] Updates player inventory
)

(event Input|ActionEvents|InputActionInventory1
  (params (Key :type Key%20Structure))
  ;[1 1 1] Inventory Access
)

(event Input|ActionEvents|InputActionInventory2
  (params (Key :type Key%20Structure))
  ;[1 1 1] Inventory Access
)

(event Input|ActionEvents|InputActionDropItem
  (params (Key :type Key%20Structure))
  ;[1 1 1] Drop Item
)

(event Input|ActionEvents|InputActionUseItem
  (params (Key :type Key%20Structure))
  ;[1 1 1] Using the player's handheld item
)

(event Input|ActionEvents|InputActionInventory3
  (params (Key :type Key%20Structure))
  ;[1 1 1] Inventory Access
)

(event Input|ActionEvents|InputActionInventory4
  (params (Key :type Key%20Structure))
  ;[1 1 1] Inventory Access
)

(fn ConstructionScript
  (|CallParentFunction))

(fn HudRefresh0
  ;[1 1 1] Updates the player's HUD with the new inventory items.
)

(fn HUDRefresh
  (bind _returnvalue (Pawn|GetController))
  (bind _aspc_multiplayer (Utilities|Casting|CastToPC_Multiplayer _returnvalue))
  ;[1 1 1] Overrides the HUDRefresh function from BP_PlayerParent
  (Widget|RemovefromParent (Variables|Default|GetHUD_0))
  (bind _returnvalue_2 (UserInterface|CreateWidget (Utilities|Select :Index (Class|GameplayStatics|GetPlayerControllerID _aspc_multiplayer) :Option%200 "/Game/Blueprints/HUD/Player1HUD.Player1HUD_C" :Option%201 "/Game/Blueprints/HUD/Player2HUD.Player2HUD_C" :Option%202 "/Game/Blueprints/HUD/Player3HUD.Player3HUD_C" :Option%203 0) _aspc_multiplayer))
  (bind _output_get (Variables|Default|SetHUD_0 _returnvalue_2))
  (UserInterface|Viewport|AddtoPlayerScreen _output_get)
  (Development|PrintString "HUDRefresh Child 2")
  (|CallParentFunction))