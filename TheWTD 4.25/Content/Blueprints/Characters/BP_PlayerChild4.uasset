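; Player character Blueprint for local multiplayer that handles the on-screen inventory HUD and item inspection.
; BeginPlay creates one of four HUD widgets by controller ID; HUDRefresh rebuilds it, though its fourth option is unset, then calls the parent.
; Tick line-traces from the follow camera, showing a BP_Item details widget once per hover and removing it when the trace misses.
; Slot swap, use and drop logic is disconnected, and HUDRefresh0 is empty.
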(event EventTick
  (params (DeltaSeconds :type Float%20%28single-precision%29))
  (bind _followcamera (Variables|Default|GetFollowCamera))
  (bind _returnvalue (Transformation|GetWorldLocation _followcamera))
  (Utilities|FlowControl|Sequence
    (:then_0
      ;[1 1 1] View Item Details on Hover
      (bind (_outhit _returnvalue_2) (Collision|LineTraceForObjects _returnvalue (+ _returnvalue (* (Math|Vector|GetForwardVector _followcamera) 2e+02)) (Utilities|Array|MakeArray "ObjectTypeQuery2") false 0 "None"))
      (if _returnvalue_2
        (bind _asbp_item (Utilities|Casting|CastToBP_Item (.HitActor (Collision|BreakHitResult _outhit))))
        (Variables|Default|SetItemHover true)
        (Utilities|FlowControl|DoOnce false :!label _label
          (:Completed
            (bind _returnvalue_3 (UserInterface|CreateWidget "/Game/Blueprints/HUD/ItemHUD.ItemHUD_C" (.AsPC%20Multiplayer (Utilities|Casting|CastToPC_Multiplayer (Pawn|GetController self))) (.name (Variables|/Game/Blueprints/Blueprints/Item/BP_Item.BP_Item_C|GetItemStructure _asbp_item)) (.description (Variables|/Game/Blueprints/Blueprints/Item/BP_Item.BP_Item_C|GetItemStructure _asbp_item)) (Variables|/Game/Blueprints/Blueprints/Item/BP_Item.BP_Item_C|GetQuantity _asbp_item)))
            (UserInterface|Viewport|AddtoPlayerScreen _returnvalue_3)))
        (elif (Variables|Default|GetItemHover)
          (Widget|RemovefromParent _returnvalue_3)
          (Variables|Default|SetItemHover false)
          (goto _label Reset))))))

(event EventBeginPlay
  (bind _returnvalue (Pawn|GetController))
  (bind _aspc_multiplayer (Utilities|Casting|CastToPC_Multiplayer _returnvalue))
  ;[1 1 1] Creates Player Inventory
  (bind _returnvalue_2 (UserInterface|CreateWidget (Utilities|Select :Index (Class|GameplayStatics|GetPlayerControllerID _aspc_multiplayer) :Option%200 "/Game/Blueprints/HUD/Player1HUD.Player1HUD_C" :Option%201 "/Game/Blueprints/HUD/Player2HUD.Player2HUD_C" :Option%202 "/Game/Blueprints/HUD/Player3HUD.Player3HUD_C" :Option%203 "/Game/Blueprints/HUD/Player4HUD.Player4HUD_C") _aspc_multiplayer))
  (bind _output_get (Variables|Default|SetHUD_0 _returnvalue_2))
  (UserInterface|Viewport|AddtoPlayerScreen _output_get))

(event EventUpdateInventory
  ;[1 1 1] Updates player inventory
)

(event Input|ActionEvents|InputActionInventory1
  (params (Key :type Key%20Structure))
  ;[1 1 1] Inventory Access
)

(event Input|ActionEvents|InputActionInventory2
  (params (Key :type Key%20Structure))
  ;[1 1 1] Inventory Access
)

(event Input|ActionEvents|InputActionDropItem
  (params (Key :type Key%20Structure))
  ;[1 1 1] Drop Item
)

(event Input|ActionEvents|InputActionUseItem
  (params (Key :type Key%20Structure))
  ;[1 1 1] Using the player's handheld item
)

(event Input|ActionEvents|InputActionInventory3
  (params (Key :type Key%20Structure))
  ;[1 1 1] Inventory Access
)

(event Input|ActionEvents|InputActionInventory4
  (params (Key :type Key%20Structure))
  ;[1 1 1] Inventory Access
)

(fn ConstructionScript
  (|CallParentFunction))

(fn HUDRefresh0
  ;[1 1 1] Updates the player's HUD with the new inventory items.
)

(fn HUDRefresh
  (bind _returnvalue (Pawn|GetController))
  (bind _aspc_multiplayer (Utilities|Casting|CastToPC_Multiplayer _returnvalue))
  ;[1 1 1] Updates the player's HUD with the new inventory items.
  (Widget|RemovefromParent (Variables|Default|GetHUD_0))
  (bind _returnvalue_2 (UserInterface|CreateWidget (Utilities|Select :Index (Class|GameplayStatics|GetPlayerControllerID _aspc_multiplayer) :Option%200 "/Game/Blueprints/HUD/Player1HUD.Player1HUD_C" :Option%201 "/Game/Blueprints/HUD/Player2HUD.Player2HUD_C" :Option%202 "/Game/Blueprints/HUD/Player3HUD.Player3HUD_C" :Option%203 0) _aspc_multiplayer))
  (bind _output_get (Variables|Default|SetHUD_0 _returnvalue_2))
  (UserInterface|Viewport|AddtoPlayerScreen _output_get)
  (|CallParentFunction))