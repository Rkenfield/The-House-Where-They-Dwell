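; Level-design spline tool that tiles a chosen static mesh along a spline, such as for cords, built in the Construction Script.
; The mesh's bounding-box length on the selected alignment axis sets the segment count, with partial lengths rounded down but at least one segment.
; Each segment is a spline mesh component bent between sampled spline positions and length-scaled tangents.
; Segments share a configurable scale and add a roll offset to the spline's roll.
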(fn ConstructionScript
  (bind _mesh (Variables|Default|GetMesh))
  (bind _spline (Variables|Default|GetSpline))
  (bind _spline_2 (Variables|Default|GetSpline))
  (bind _meshscale (Variables|Default|GetMeshScale))
  (bind _meshroll (Variables|Default|GetMeshRoll))
  (bind _meshalignmentaxis (Variables|Default|GetMeshAlignmentAxis))
  (bind _returnvalue (StaticMesh|GetBoundingBox _mesh))
  (bind _returnvalue_2 (Math|Trig|DegreesToRadians _meshroll))
  (bind _returnvalue_3 (- (.max _returnvalue) (.min _returnvalue)))
  (bind _returnvalue_4 (Utilities|Select :Index _meshalignmentaxis :X (.x _returnvalue_3) :Y (.y _returnvalue_3) :Z (.z _returnvalue_3)))
  (bind _returnvalue_5 (Math|Float|Absolute(Float) _returnvalue_4))
  (Variables|Default|GetMesh
    (:then
      (for _index (range 0 (Math|Integer|Max(Integer) (- (Math|Float|Floor (/ (Spline|GetSplineLength (Variables|Default|GetSpline)) _returnvalue_5)) 1)))
        (bind _returnvalue_6 (AddComponent|AddSplineMeshComponent false))
        (Components|StaticMesh|SetStaticMesh _returnvalue_6 (Variables|Default|GetMesh))
        (SplineMesh|SetStartandEnd _returnvalue_6 (Spline|GetLocationatDistanceAlongSpline _spline (* _index _returnvalue_5) "Local") (* (Spline|GetDirectionatDistanceAlongSpline _spline (* _index _returnvalue_5) "Local") _returnvalue_5) (Spline|GetLocationatDistanceAlongSpline _spline_2 (* (+ _index 1) _returnvalue_5) "Local") (* (Spline|GetDirectionatDistanceAlongSpline _spline_2 (* (+ _index 1) _returnvalue_5) "Local") _returnvalue_5) true :!class /Script/Engine.SplineMeshComponent)
        (SplineMesh|SetEndScale _returnvalue_6 _meshscale true :!class /Script/Engine.SplineMeshComponent)
        (SplineMesh|SetStartScale _returnvalue_6 _meshscale true :!class /Script/Engine.SplineMeshComponent)
        (SplineMesh|SetForwardAxis _returnvalue_6 (Variables|Default|GetMeshAlignmentAxis) true)
        ;[1 1 1] Roll
        (Class|SplineMeshComponent|SetStartRoll _returnvalue_6 (+ (Math|Trig|DegreesToRadians (Class|SplineComponent|GetRollatDistanceAlongSpline _spline_2 (* _index _returnvalue_5) "Local")) _returnvalue_2) true)
        (Class|SplineMeshComponent|SetEndRoll _returnvalue_6 (+ (Math|Trig|DegreesToRadians (Class|SplineComponent|GetRollatDistanceAlongSpline _spline_2 (* (+ _index 1) _returnvalue_5) "Local")) _returnvalue_2) true)))
    (:else)))