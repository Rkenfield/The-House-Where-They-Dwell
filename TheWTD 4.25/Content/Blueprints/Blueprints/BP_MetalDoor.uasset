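; A metal door that the player toggles open and closed through BPI_Interaction.
; The DoorDriver timeline plays or reverses to swing the Pivot between start and end rotations along a curve.
; Open and Close audio components fade in and out to crossfade when the door is toggled mid-sound.
; BeginPlay randomizes their handle and creak sample parameters, so each door keeps one set of sounds per session.
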(event Custom|OpenDoor
  ;[1 1 1] Alex: Event that defines the function that opens the door.
  (Utilities|Casting|CastToBP_PlayerParent (Game|GetPlayerCharacter 0))
  (if (Variables|Default|GetIsOpen)
    (Variables|Default|SetIsOpen false) ; If IsOpen is true, set it to false.
    ;;[1 1 1] Audio Cues
    (if (Audio|Components|Audio|IsPlaying (Variables|Default|GetOpen)) ; If still playing open...
      (Audio|Components|Audio|FadeOut (Variables|Default|GetOpen) 0.3 0.0 "SCurve" :!class /Script/Engine.AudioComponent) ; fade open out...
    )
    (Audio|Components|Audio|FadeIn (Variables|Default|GetClose) 0.5 1.0 0.0 "Sin" :!class /Script/Engine.AudioComponent) ; in both cases fade in close
    (bind _doorcurve (Timeline|DoorDriver Reverse)
      (:Update
        (Transformation|SetRelativeRotation (Variables|Default|GetPivot) (Math|Rotator|Lerp(Rotator) (Variables|Default|GetStartRotation) (Variables|Default|GetEndRotation) _doorcurve) false false)))
    (else
      (Variables|Default|SetIsOpen true) ; If IsOpen is false, set it to true.
      (if (Audio|Components|Audio|IsPlaying (Variables|Default|GetClose)) ; If still playing close...
        (Audio|Components|Audio|FadeOut (Variables|Default|GetClose) 0.3 0.0 "SCurve" :!class /Script/Engine.AudioComponent) ; fade close out...
      )
      (Audio|Components|Audio|FadeIn (Variables|Default|GetOpen) 0.05 1.0 0.0 "Sin" :!class /Script/Engine.AudioComponent) ; in both cases fade in open
      (Timeline|DoorDriver Play))))

(event EventInteract
  (params (Interactor :type Actor%20Object%20Reference) (HitComponent :type Primitive%20Component%20Object%20Reference))
  ;[1 1 1] Alex: Have BPI_Interaction implemented. Declares the function that opens the door.
  (Utilities|Casting|CastToBP_PlayerParent Interactor)
  (CallFunction|OpenDoor))

(event EventBeginPlay
  (bind _close (Variables|Default|GetClose))
  (bind _open (Variables|Default|GetOpen))
  ;[1 1 1] Logan: Set Door Samples
  (Effects|Components|ParticleSystem|SetIntParameter _open "OpenHandle" (Math|Random|RandomIntegerinRange 0 7))
  (Effects|Components|ParticleSystem|SetIntParameter _open "OpenCreak" (Math|Random|RandomIntegerinRange 0 4))
  (Effects|Components|ParticleSystem|SetIntParameter _close "CloseHandle" (Math|Random|RandomIntegerinRange 0 4))
  (Effects|Components|ParticleSystem|SetIntParameter _close "CloseCreak" (Math|Random|RandomIntegerinRange 0 4)))

(fn ConstructionScript)