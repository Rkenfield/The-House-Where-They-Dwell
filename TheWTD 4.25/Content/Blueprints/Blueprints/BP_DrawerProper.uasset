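; BP_DrawerProper is an interactable drawer that slides open and closed when the ThirdPersonCharacter interacts with it.
; Interact checks the interactor's class and calls OpenDrawer, which flips IsOpen and plays or reverses the DrawerDriver timeline.
; The timeline's DrawerCurve lerps the Pivot's relative location between StartPosition and EndPosition.
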(event Custom|OpenDrawer
  (Utilities|Casting|CastToThirdPersonCharacter (Game|GetPlayerCharacter 0))
  (if (Variables|Default|GetisOpen)
    (Variables|Default|SetisOpen false)
    (bind _drawercurve (Timeline|DrawerDriver Reverse)
      (:Update
        (Transformation|SetRelativeLocation (Variables|Default|GetPivot) (Math|Vector|Lerp(Vector) (Variables|Default|GetstartPosition) (Variables|Default|GetendPosition) _drawercurve) false false)))
    (else
      (Variables|Default|SetisOpen true)
      (Timeline|DrawerDriver Play))))

(event EventBeginPlay)

(event Collision|EventActorBeginOverlap
  (params (OtherActor :type Actor%20Object%20Reference)))

(event EventTick
  (params (DeltaSeconds :type Float%20%28single-precision%29)))

(event EventInteract
  (params (Interactor :type Actor%20Object%20Reference))
  (Utilities|Casting|CastToThirdPersonCharacter Interactor)
  (CallFunction|OpenDrawer))

(fn ConstructionScript)