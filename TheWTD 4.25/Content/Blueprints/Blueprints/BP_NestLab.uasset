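; Destructible spider nest that spawns spider minions on a looping timer up to a set maximum.
; A DousedLab timeline changes the material's color and roughness, and a match overlapping a nest tagged Doused stops spawning and triggers destruction.
; Destruction plays fire particles and a dynamic-material dissolve before destroying the actor.
; Attic-tagged nests increment a game mode counter, which advances the objective and starts phase 4 when all are destroyed.
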(event Custom|SpawnSpiderMinion
  (bind _spiderspawnpoint (Variables|Default|GetSpiderSpawnPoint))
  (if (< (Variables|Default|GetNoOfSpawnedSpiders) (Variables|Default|GetMaxNofOfSpawnedSpiders)) ; Is the number of spawned spiders < than the max?
    (Game|SpawnActorfromClass "/Game/Blueprints/AI/SpiderWitch/Spider/NormalSpider/SpiderMinion.SpiderMinion_C" (Math|Transform|MakeTransform (Transformation|GetWorldLocation _spiderspawnpoint) (Transformation|GetWorldRotation _spiderspawnpoint) "1,1,1") "AlwaysSpawn" 0 0)
    (Variables|Default|SetNoOfSpawnedSpiders (+ (Variables|Default|GetNoOfSpawnedSpiders) 1)) ; Increase NoOfSpawnedSpiders by 1.
    (Audio|Components|Audio|Play (Variables|Default|GetSpiderSpawn) 0.0)
    (else
      (CallFunction|StopSpiderMinionSpawn))))

(event Custom|StopSpiderMinionSpawn
  (Utilities|Time|SetTimerbyEvent (delegate Custom|SpawnSpiderMinion) 0.0))

(event Custom|StartSpiderMinionSpawn
  ;[1 1 1] Spawns the first spider minion (if this isn't here, the first spider spawn is delayed by the MinionSpawnInterval).
  (CallFunction|SpawnSpiderMinion)
  (Variables|Default|SetNoOfSpawnedSpiders 1)
  (Utilities|Time|SetTimerbyEvent (delegate Custom|SpawnSpiderMinion) (Variables|Default|GetMinionSpawnInterval) true))

(event Custom|Destruction
  (bind _gamemode (Variables|Default|GetGameMode))
  (bind _gamemode_2 (Variables|Default|GetGameMode))
  ;[1 1 1] Destruction
  (if (Actor|ActorHasTag "AtticNest") ; Is it an AtticNest?
    (Variables|/Game/Blueprints/BP_WTDGameMode.BP_WTDGameMode_C|SetDestroyedAtticNests _gamemode (+ (Variables|/Game/Blueprints/BP_WTDGameMode.BP_WTDGameMode_C|GetDestroyedAtticNests _gamemode) 1)))
  ;;[1 1 1] Play Fire particle and dissolve transition before actor is destroyed
  (Components|Activation|Activate (Variables|Default|GetP_Fire) false)
  (Utilities|FlowControl|Delay 0.5)
  (bind (_direction _baselength _webslength) (Timeline|Dissolve Play)
    (:Update
      (Rendering|Material|SetScalarParameterValue (Variables|Default|GetBaseLength) "Length" _baselength :!class /Script/Engine.MaterialInstanceDynamic)
      (Rendering|Material|SetScalarParameterValue (Variables|Default|GetWebsLength) "Length" _webslength :!class /Script/Engine.MaterialInstanceDynamic)
      (Components|Activation|Deactivate (Variables|Default|GetP_Fire))
      (if (Actor|ActorHasTag "AtticNest") ; Is it an AtticNest?
        _))
    (:Finished
      (Actor|DestroyActor)
      (if (== (Variables|/Game/Blueprints/BP_WTDGameMode.BP_WTDGameMode_C|GetDestroyedAtticNests _gamemode_2) (Variables|/Game/Blueprints/BP_WTDGameMode.BP_WTDGameMode_C|GetMaxNoOfAtticNests _gamemode_2)) ; Are all the attic nests destroyed?
        (Variables|/Game/Blueprints/BP_WTDGameMode.BP_WTDGameMode_C|SetCurrentObjectiveNum _gamemode_2 7)
        (Default|SetPhase4 _gamemode_2)))))

(event Custom|DousedLab
  (bind (_direction _roughness _color) (Timeline|DousedTime Play)
    (:Update
      (Rendering|Material|SetScalarParameterValueonMaterials (Variables|Default|GetMesh) "DousedRoughness" _roughness)
      (Rendering|Material|SetVectorParameterValueonMaterials (Variables|Default|GetMesh) "DousedColor" _color))))

(event EventBeginPlay
  (bind _asbp_wtdgame_mode (Utilities|Casting|CastToBP_WTDGameMode (Game|GetGameMode)))
  (Variables|Default|SetGameMode _asbp_wtdgame_mode))

(event Collision|EventActorBeginOverlap
  (params (OtherActor :type Actor%20Object%20Reference))
  (bind _asbp_match (Utilities|Casting|CastToBP_Match OtherActor))
  (if (Actor|ActorHasTag self "Doused") ; Does the nest have the Doused tag?
    (if (not (Actor|ActorHasTag self "Fire")) ; Does the nest already have the Fire tag?
      (CallFunction|StopSpiderMinionSpawn)
      (Utilities|FlowControl|Delay 1.0)
      (CallFunction|Destruction)
      (Utilities|Array|Add (Variables|Actor|GetTags) "Fire")
      (Actor|DestroyActor _asbp_match))))

(fn ConstructionScript
  (bind _mesh (Variables|Default|GetMesh))
  (bind _returnvalue (Rendering|Material|CreateDynamicMaterialInstance _mesh 0 "/Game/Art/Materials/Nests/New/BurningMaterial/MI_DissolveBase.MI_DissolveBase" "None" :!class /Script/Engine.PrimitiveComponent))
  (Variables|Default|SetBaseLength _returnvalue)
  (bind _returnvalue_2 (Rendering|Material|CreateDynamicMaterialInstance _mesh 1 "/Game/Art/Materials/Nests/New/BurningMaterial/MI_DissolveWebs.MI_DissolveWebs" "None" :!class /Script/Engine.PrimitiveComponent))
  (Variables|Default|SetWebsLength _returnvalue_2))