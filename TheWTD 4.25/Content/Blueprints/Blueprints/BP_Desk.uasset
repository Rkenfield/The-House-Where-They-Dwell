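; BP_Desk is an interactable desk whose drawers slide open and closed when a BP_PlayerParent interacts with a component tagged "Drawer".
; An "Open" component tag tracks each drawer's state and decides whether the single shared timeline plays forward or in reverse.
; The timeline curve lerps the drawer's relative location between StartPosition and EndPosition, while a DoOnce gate blocks further drawer interaction until the animation finishes.
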(event Custom|OpenDrawer
  (params (Drawer :type Primitive%20Component%20Object%20Reference))
  (bind _componenttags (Variables|/Script/Engine.ActorComponent|GetComponentTags Drawer))
  (if (Components|ComponentHasTag Drawer "Open") ; Is the drawer already open?
    (Utilities|Array|RemoveItem _componenttags "Open") ; If the door is open, remove the Open tag from it.
    (bind _drawercurve (Timeline|Timeline_0 ReverseFromEnd)
      (:Update
        (Transformation|SetRelativeLocation Drawer (Math|Vector|Lerp(Vector) (Variables|Default|GetStartPosition) (Variables|Default|GetEndPosition) _drawercurve) false false))
      (:Finished
        (Utilities|FlowControl|DoOnce false) ; enters at Reset
      ))
    (else
      (Utilities|Array|Add _componenttags "Open") ; If the door is closed, give it the Open tag.
      (Timeline|Timeline_0 PlayFromStart))))

(event EventBeginPlay)

(event Collision|EventActorBeginOverlap
  (params (OtherActor :type Actor%20Object%20Reference)))

(event EventTick
  (params (DeltaSeconds :type Float%20%28single-precision%29)))

(event EventInteract
  (params (Interactor :type Actor%20Object%20Reference) (HitComponent :type Primitive%20Component%20Object%20Reference))
  (Utilities|Casting|CastToBP_PlayerParent Interactor)
  (if (Components|ComponentHasTag HitComponent "Drawer")
    (Utilities|FlowControl|DoOnce false
      (:Completed
        (CallFunction|OpenDrawer HitComponent)))))

(fn ConstructionScript)