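; Scene component that spawns equipment items, a camera on tripod or a throwable audio recorder, at its own world position and rotation.
; Each item has its own spawn function, which adjusts for collisions but always spawns.
; The camera class comes from the first SpawnableEquipment entry, while the audio recorder class is set directly.
; BeginPlay caches the BP_WTDGameMode reference, though neither spawn function uses it.
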(event EventBeginPlay
  (bind _asbp_wtdgame_mode (Utilities|Casting|CastToBP_WTDGameMode (Game|GetGameMode)))
  (Variables|Default|SetGameMode _asbp_wtdgame_mode))

(event EventTick
  (params (DeltaSeconds :type Float%20%28single-precision%29)))

(fn SpawnCameraonTripod
  (Game|SpawnActorfromClass (Utilities|Array|Get(acopy) (Variables|Default|GetSpawnableEquipment)) (Math|Transform|MakeTransform (Transformation|GetWorldLocation) (Transformation|GetWorldRotation)) "AdjustIfPossibleButAlwaysSpawn" 0 0))

(fn SpawnAudioRecorder
  (Game|SpawnActorfromClass "/Game/Blueprints/Blueprints/Item/BP_Item_Throwable_AudioRecorder.BP_Item_Throwable_AudioRecorder_C" (Math|Transform|MakeTransform (Transformation|GetWorldLocation) (Transformation|GetWorldRotation)) "AdjustIfPossibleButAlwaysSpawn" 0 0))