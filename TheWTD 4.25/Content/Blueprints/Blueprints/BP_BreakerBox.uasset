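; Breaker box minigame actor: interacting opens the player's minigame menu and blends the camera to the box.
; Six switch events each toggle an on/off flag and play a timeline that lerps the switch's relative rotation to either side.
; Only Switch 1 drives a meter so far, stepping the left dial by one sixth of its travel range, computed at BeginPlay, when its animation finishes.
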(event Custom|S5Rotation
  (bind _switch5 (Variables|Default|GetSwitch5))
  (bind _relativerotation (Variables|/Script/Engine.SceneComponent|GetRelativeRotation _switch5))
  ;[1 1 1] S5Rotation
  (if (Variables|Default|GetS5On)
    (Variables|Default|SetS5On false)
    (bind _dialrotation (Timeline|Timeline_4 PlayFromStart)
      (:Update
        (Transformation|SetRelativeRotation _switch5 (Math|Rotator|Lerp(Rotator) _relativerotation "0,-40.000000, 0" _dialrotation) false false)))
    (else
      (Variables|Default|SetS5On true)
      (bind _dialrotation_2 (Timeline|Timeline_5 PlayFromStart)
        (:Update
          (Transformation|SetRelativeRotation _switch5 (Math|Rotator|Lerp(Rotator) _relativerotation "0,40.000000, 0" _dialrotation_2) false false))))))

(event Custom|S6Rotation
  (bind _switch6 (Variables|Default|GetSwitch6))
  (bind _relativerotation (Variables|/Script/Engine.SceneComponent|GetRelativeRotation _switch6))
  ;[1 1 1] S6Rotation
  (if (Variables|Default|GetS6On)
    (Variables|Default|SetS6On false)
    (bind _dialrotation (Timeline|Timeline_10 PlayFromStart)
      (:Update
        (Transformation|SetRelativeRotation _switch6 (Math|Rotator|Lerp(Rotator) _relativerotation "0,40.000000, 0" _dialrotation) false false)))
    (else
      (Variables|Default|SetS6On true)
      (bind _dialrotation_2 (Timeline|Timeline_11 PlayFromStart)
        (:Update
          (Transformation|SetRelativeRotation _switch6 (Math|Rotator|Lerp(Rotator) _relativerotation "0,-40.000000, 0" _dialrotation_2) false false))))))

(event Custom|S3Rotation
  (bind _switch3 (Variables|Default|GetSwitch3))
  (bind _relativerotation (Variables|/Script/Engine.SceneComponent|GetRelativeRotation _switch3))
  ;[1 1 1] S3Rotation
  (if (Variables|Default|GetS3On)
    (Variables|Default|SetS3On false)
    (bind _dialrotation (Timeline|Timeline_2 PlayFromStart)
      (:Update
        (Transformation|SetRelativeRotation _switch3 (Math|Rotator|Lerp(Rotator) _relativerotation "0,-40.000000, 0" _dialrotation) false false)))
    (else
      (Variables|Default|SetS3On true)
      (bind _dialrotation_2 (Timeline|Timeline_3 PlayFromStart)
        (:Update
          (Transformation|SetRelativeRotation _switch3 (Math|Rotator|Lerp(Rotator) _relativerotation "0,40.000000, 0" _dialrotation_2) false false))))))

(event Custom|S1Rotation
  (bind _switch1 (Variables|Default|GetSwitch1))
  (bind _leftdial (Variables|Default|GetLeftDial))
  (bind _leftdial_2 (Variables|Default|GetLeftDial))
  (bind _relativerotation (Variables|/Script/Engine.SceneComponent|GetRelativeRotation _switch1))
  (bind _relativelocation (Variables|/Script/Engine.SceneComponent|GetRelativeLocation _leftdial))
  (bind _relativelocation_2 (Variables|/Script/Engine.SceneComponent|GetRelativeLocation _leftdial_2))
  ;[1 1 1] S1Rotation
  (if (Variables|Default|GetS1On)
    (Variables|Default|SetS1On false)
    (bind _dialrotation (Timeline|Timeline_0 PlayFromStart)
      (:Update
        (Transformation|SetRelativeRotation _switch1 (Math|Rotator|Lerp(Rotator) _relativerotation "0,-40.000000, 0" _dialrotation) false false))
      (:Finished
        (bind _output_get (Variables|Default|SetLeftDialCurrentLocation (- (Variables|Default|GetLeftDialCurrentLocation) (Variables|Default|GetLeftDialValueTemp))))
        (Transformation|SetRelativeLocation _leftdial (Math|Vector|MakeVector _output_get (.y _relativelocation) (.z _relativelocation)) false false)))
    (else
      (Variables|Default|SetS1On true)
      (bind _dialrotation_2 (Timeline|Timeline_1 PlayFromStart)
        (:Update
          (Transformation|SetRelativeRotation _switch1 (Math|Rotator|Lerp(Rotator) _relativerotation "0,40.000000, 0" _dialrotation_2) false false))
        (:Finished
          (bind _output_get_2 (Variables|Default|SetLeftDialCurrentLocation (+ (Variables|Default|GetLeftDialCurrentLocation) (Variables|Default|GetLeftDialValueTemp))))
          (Transformation|SetRelativeLocation _leftdial_2 (Math|Vector|MakeVector _output_get_2 (.y _relativelocation_2) (.z _relativelocation_2)) false false))))))

(event Custom|S2Rotation
  (bind _switch2 (Variables|Default|GetSwitch2))
  (bind _relativerotation (Variables|/Script/Engine.SceneComponent|GetRelativeRotation _switch2))
  ;[1 1 1] S2Rotation
  (if (Variables|Default|GetS2On)
    (Variables|Default|SetS2On false)
    (bind _dialrotation (Timeline|Timeline_6 PlayFromStart)
      (:Update
        (Transformation|SetRelativeRotation _switch2 (Math|Rotator|Lerp(Rotator) _relativerotation "0,40.000000, 0" _dialrotation) false false)))
    (else
      (Variables|Default|SetS2On true)
      (bind _dialrotation_2 (Timeline|Timeline_7 PlayFromStart)
        (:Update
          (Transformation|SetRelativeRotation _switch2 (Math|Rotator|Lerp(Rotator) _relativerotation "0,-40.000000, 0" _dialrotation_2) false false))))))

(event Custom|S4Rotation
  (bind _switch4 (Variables|Default|GetSwitch4))
  (bind _relativerotation (Variables|/Script/Engine.SceneComponent|GetRelativeRotation _switch4))
  ;[1 1 1] S4Rotation
  (if (Variables|Default|GetS4On)
    (Variables|Default|SetS4On false)
    (bind _dialrotation (Timeline|Timeline_8 PlayFromStart)
      (:Update
        (Transformation|SetRelativeRotation _switch4 (Math|Rotator|Lerp(Rotator) _relativerotation "0,40.000000, 0" _dialrotation) false false)))
    (else
      (Variables|Default|SetS4On true)
      (bind _dialrotation_2 (Timeline|Timeline_9 PlayFromStart)
        (:Update
          (Transformation|SetRelativeRotation _switch4 (Math|Rotator|Lerp(Rotator) _relativerotation "0,-40.000000, 0" _dialrotation_2) false false))))))

(event EventBeginPlay
  (Variables|Default|SetLeftDialCurrentLocation (Variables|Default|GetLeftDialStartLocation))
  (bind _output_get (Variables|Default|SetLeftMeterDomain (- (Variables|Default|GetLeftDialStartLocation) (Variables|Default|GetLeftDialEndLocation))))
  (bind _output_get_2 (Variables|Default|SetLeftDialValueTemp (Math|Float|Absolute(Float) (/ _output_get 6.0))))
  (Development|PrintString (Utilities|String|ToString(Float) _output_get_2)))

(event Collision|EventActorBeginOverlap
  (params (OtherActor :type Actor%20Object%20Reference)))

(event EventTick
  (params (DeltaSeconds :type Float%20%28single-precision%29)))

(event EventInteract
  (params (Interactor :type Actor%20Object%20Reference) (HitComponent :type Primitive%20Component%20Object%20Reference))
  ;[1 1 1] Interaction
  (bind _asbp_player_parent (Utilities|Casting|CastToBP_PlayerParent Interactor))
  (bind _output_get (Variables|Default|SetCharacter _asbp_player_parent))
  (Default|CreateMinigameMenu _output_get)
  (Game|Player|SetViewTargetwithBlend (.AsPC%20Multiplayer (Utilities|Casting|CastToPC_Multiplayer (Pawn|GetController _output_get))) self 2.0 "VTBlend_Linear" 0.0 false))

(fn ConstructionScript)