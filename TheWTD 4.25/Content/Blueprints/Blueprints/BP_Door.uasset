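; BP_Door is an interactable door that toggles between open and closed when the player uses it.
; The BPI_Interaction Interact event checks that the interactor is a BP_PlayerParent, then calls OpenDoor.
; OpenDoor flips IsOpen and plays or reverses the DoorDriver timeline, whose curve lerps the Pivot's relative rotation between StartRotation and EndRotation.
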(event Custom|OpenDoor
  ;[1 1 1] Alex: Event that defines the function that opens the door.
  (Utilities|Casting|CastToBP_PlayerParent (Game|GetPlayerCharacter 0))
  (if (Variables|Default|GetIsOpen)
    (Variables|Default|SetIsOpen false) ; If IsOpen is true, set it to false.
    (bind _doorcurve (Timeline|DoorDriver Reverse)
      (:Update
        (Transformation|SetRelativeRotation (Variables|Default|GetPivot) (Math|Rotator|Lerp(Rotator) (Variables|Default|GetStartRotation) (Variables|Default|GetEndRotation) _doorcurve) false false)))
    (else
      (Variables|Default|SetIsOpen true) ; If IsOpen is false, set it to true.
      (Timeline|DoorDriver Play))))

(event EventBeginPlay)

(event Collision|EventActorBeginOverlap
  (params (OtherActor :type Actor%20Object%20Reference)))

(event EventTick
  (params (DeltaSeconds :type Float%20%28single-precision%29)))

(event EventInteract
  (params (Interactor :type Actor%20Object%20Reference))
  ;[1 1 1] Alex: Have BPI_Interaction implemented. Declares the function that opens the door.
  (Utilities|Casting|CastToBP_PlayerParent Interactor)
  (CallFunction|OpenDoor))

(fn ConstructionScript)