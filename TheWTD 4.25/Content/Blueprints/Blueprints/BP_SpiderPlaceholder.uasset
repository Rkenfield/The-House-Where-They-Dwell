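; BP_SpiderPlaceholder is a stand-in spider actor that shrinks when its Shrink event fires and is eventually destroyed.
; Shrink flags the player's ThirdPersonCharacter as UsingSpray, then a timeline lerps the Pivot's world scale from its current value toward that value times ShrinkSize.
; On finish it clears the flag and destroys the spider if the scale has reached a hardcoded quarter size, which assumes a default Pivot scale of one.
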(event Custom|Shrink
  (bind _asthird_person_character (Utilities|Casting|CastToThirdPersonCharacter (Game|GetPlayerCharacter 0)))
  (bind _output_get (Variables|Default|SetCharacter _asthird_person_character))
  (Variables|/Game/Blueprints/Characters/ThirdPersonCharacter.ThirdPersonCharacter_C|SetUsingSpray _output_get true)
  (Variables|Default|SetStartScale (Transformation|GetWorldScale (Variables|Default|GetPivot)))
  (bind _actorsize (Timeline|Shrink1 PlayFromStart)
    (:Update
      (Transformation|SetWorldScale3D (Variables|Default|GetPivot) (Math|Vector|Lerp(Vector) (Variables|Default|GetStartScale) (* (Variables|Default|GetStartScale) (Variables|Default|GetShrinkSize)) _actorsize)))
    (:Finished
      (if (Math|Vector|Equal(Vector) (Transformation|GetWorldScale (Variables|Default|GetPivot)) "0.250000,0.250000,0.250000" 0.0001) ; Is the spider at the destroying size?
        (Actor|DestroyActor))
      (Variables|/Game/Blueprints/Characters/ThirdPersonCharacter.ThirdPersonCharacter_C|SetUsingSpray (Variables|Default|GetCharacter) false))))

(fn ConstructionScript)