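; BP_EquipmentSpawner is a placed actor that spawns equipment, a camera on a tripod or an audio recorder, at its own location and rotation.
; Separate functions spawn each item from fixed slots in a SpawnableEquipment class array.
; BeginPlay caches the BP_WTDGameMode, though nothing here uses it yet.
; AttemptToSpawnRecorder is an empty stub, and the spawn functions are not called within this Blueprint.
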(event EventBeginPlay
  (bind _asbp_wtdgame_mode (Utilities|Casting|CastToBP_WTDGameMode (Game|GetGameMode)))
  (Variables|Default|SetGameMode _asbp_wtdgame_mode))

(event Collision|EventActorBeginOverlap
  (params (OtherActor :type Actor%20Object%20Reference)))

(event EventTick
  (params (DeltaSeconds :type Float%20%28single-precision%29)))

(fn ConstructionScript)

(fn AttempttoSpawnRecorder)

(fn SpawnCameraonTripod
  (Game|SpawnActorfromClass (Utilities|Array|Get(acopy) (Variables|Default|GetSpawnableEquipment)) (Math|Transform|MakeTransform (Transformation|GetActorLocation) (Transformation|GetActorRotation)) "Undefined" 0 0))

(fn SpawnAudioRecorder
  (Game|SpawnActorfromClass (Utilities|Array|Get(acopy) (Variables|Default|GetSpawnableEquipment) 1) (Math|Transform|MakeTransform (Transformation|GetActorLocation) (Transformation|GetActorRotation)) "Undefined" 0 0))