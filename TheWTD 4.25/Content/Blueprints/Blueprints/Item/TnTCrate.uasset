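; TnT crate actor that supplies throwable dynamite items at a spawn point.
; On BeginPlay it spawns a dynamite, sets itself as that item's Spawner and marks itself Available.
; A looping timer at SpawnRate runs CheckTNT, which spawns a replacement whenever Available is false.
; Nothing here clears Available.
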(event EventBeginPlay
  (bind _spawnpoint1 (Variables|Default|GetSpawnPoint1))
  (bind _returnvalue (Transformation|GetWorldTransform _spawnpoint1))
  (bind _returnvalue_2 (Game|SpawnActorfromClass "/Game/Blueprints/Blueprints/Item/BP_Item_Throwable_Dynamite.BP_Item_Throwable_Dynamite_C" (Math|Transform|MakeTransform (.location _returnvalue) (.rotation _returnvalue) "1,1,1") "Undefined" 0 0))
  (Variables|/Game/Blueprints/Blueprints/Item/BP_Item_Throwable_Dynamite.BP_Item_Throwable_Dynamite_C|SetSpawner _returnvalue_2 self)
  (Variables|Default|SetAvailable true)
  (Utilities|Time|SetTimerbyFunctionName self "CheckTNT" (Variables|Default|GetSpawnRate) true))

(event EventTick
  (params (DeltaSeconds :type Float%20%28single-precision%29)))

(fn ConstructionScript)

(fn CheckTNT
  (bind _spawnpoint1 (Variables|Default|GetSpawnPoint1))
  (bind _returnvalue (Transformation|GetWorldTransform _spawnpoint1))
  (if (not (Variables|Default|GetAvailable))
    (bind _returnvalue_2 (Game|SpawnActorfromClass "/Game/Blueprints/Blueprints/Item/BP_Item_Throwable_Dynamite.BP_Item_Throwable_Dynamite_C" (Math|Transform|MakeTransform (.location _returnvalue) (.rotation _returnvalue) "1,1,1") "Undefined" 0 0))
    (Variables|/Game/Blueprints/Blueprints/Item/BP_Item_Throwable_Dynamite.BP_Item_Throwable_Dynamite_C|SetSpawner _returnvalue_2 self)
    (Variables|Default|SetAvailable true)))