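; Throwable item Blueprint that launches itself in the user's camera direction when used.
; UseItem calls the parent logic, sets the static mesh's physics velocity to the follow camera's forward vector scaled by the user's Throw value, then flags IsThrown.
; The mesh hit event is empty, with debug printing and the flag reset left disconnected, and PassiveEffect only defers to the parent.
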(event OnComponentHit(StaticMesh)
  (params (HitComponent :type Primitive%20Component%20Object%20Reference) (OtherActor :type Actor%20Object%20Reference) (OtherComp :type Primitive%20Component%20Object%20Reference) (NormalImpulse :type Vector :default "0, 0, 0") (Hit :type Hit%20Result%20Structure%20%28by%20ref%29)))

(event EventBeginPlay)

(event Collision|EventActorBeginOverlap
  (params (OtherActor :type Actor%20Object%20Reference)))

(event EventTick
  (params (DeltaSeconds :type Float%20%28single-precision%29)))

(fn ConstructionScript
  (|CallParentFunction))

(fn UseItem
  (params (User :type BP%20Player%20Parent%20Object%20Reference))
  ;[1 1 1] Throws item in a direction when used
  (bind _success (|CallParentFunction 0))
  (Physics|SetPhysicsLinearVelocity (Variables|Default|GetStaticMesh) (* (Math|Vector|GetForwardVector (Variables|/Game/Blueprints/Characters/BP_PlayerParent.BP_PlayerParent_C|GetFollowCamera User)) (Variables|/Game/Blueprints/Characters/BP_PlayerParent.BP_PlayerParent_C|GetThrow User)) false "None")
  (Variables|Default|SetIsThrown true)
  (return _success))

(fn PassiveEffect
  (params (User :type BP%20Player%20Parent%20Object%20Reference))
  (bind _success (|CallParentFunction 0))
  (return _success))