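; Fanny pack consumable item that expands the user's inventory by one slot.
; Its UseItem override acts only when the user's InventoryComponent has exactly four slots, raising the count to five and calling PrepareInventory.
; The parent UseItem runs only after that upgrade, so users with any other slot count skip it entirely.
; The event graph holds only disabled default events.
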(event EventBeginPlay
  (|CallParentFunction) ; This node is disabled and will not be called.\nDrag off pins to build functionality.
)

(event Collision|EventActorBeginOverlap
  (params (OtherActor :type Actor%20Object%20Reference))
  (|CallParentFunction OtherActor) ; This node is disabled and will not be called.\nDrag off pins to build functionality.
)

(event EventTick
  (params (DeltaSeconds :type Float%20%28single-precision%29))
  (|CallParentFunction DeltaSeconds) ; This node is disabled and will not be called.\nDrag off pins to build functionality.
)

(fn ConstructionScript
  (|CallParentFunction))

(fn UseItem
  (params (User :type BP%20Player%20Parent%20Object%20Reference))
  (bind _inventorycomponent (Variables|/Game/Blueprints/Characters/BP_PlayerParent.BP_PlayerParent_C|GetInventoryComponent User))
  (if (== (Variables|/Game/Blueprints/Blueprints/InventoryComponent.InventoryComponent_C|GetNoOfSlots (Variables|/Game/Blueprints/Characters/BP_PlayerParent.BP_PlayerParent_C|GetInventoryComponent User)) 4)
    (Variables|/Game/Blueprints/Blueprints/InventoryComponent.InventoryComponent_C|SetNoOfSlots _inventorycomponent 5)
    (Default|PrepareInventory _inventorycomponent)
    (bind _success (|CallParentFunction 0))
    (return _success)))