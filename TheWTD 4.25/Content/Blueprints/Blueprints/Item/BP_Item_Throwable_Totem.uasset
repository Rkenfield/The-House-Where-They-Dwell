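; BP_Item_Throwable_Totem is an item Blueprint, named as a throwable totem, that grants its user health regeneration as a passive effect.
; PassiveEffect runs the parent logic, then passes a fixed regen amount to the user's HealthRegen and returns the parent's result.
; RemovePassive runs the parent logic, then calls HealthRegen with zero.
; It adds no event graph logic of its own.
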(event EventBeginPlay
  (|CallParentFunction) ; This node is disabled and will not be called.\nDrag off pins to build functionality.
)

(event Collision|EventActorBeginOverlap
  (params (OtherActor :type Actor%20Object%20Reference))
  (|CallParentFunction OtherActor) ; This node is disabled and will not be called.\nDrag off pins to build functionality.
)

(event EventTick
  (params (DeltaSeconds :type Float%20%28single-precision%29))
  (|CallParentFunction DeltaSeconds) ; This node is disabled and will not be called.\nDrag off pins to build functionality.
)

(fn ConstructionScript
  (|CallParentFunction))

(fn PassiveEffect
  (params (User :type BP%20Player%20Parent%20Object%20Reference))
  (bind _success (|CallParentFunction 0))
  (Default|HealthRegen User 5.0)
  (return _success))

(fn RemovePassive
  (params (User :type BP%20Player%20Parent%20Object%20Reference))
  (|CallParentFunction 0)
  (Default|HealthRegen User 0.0))