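; Throwable matches item Blueprint that sets doused nests alight on contact.
; On actor overlap it casts the other actor to BP_Nest and checks its actor tags for Doused without an existing Fire tag.
; A qualifying nest gets the Fire tag added, which is then printed as debug output.
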(event EventBeginPlay
  (|CallParentFunction) ; This node is disabled and will not be called.\nDrag off pins to build functionality.
)

(event EventTick
  (params (DeltaSeconds :type Float%20%28single-precision%29))
  (|CallParentFunction DeltaSeconds) ; This node is disabled and will not be called.\nDrag off pins to build functionality.
)

(event Collision|EventActorBeginOverlap
  (params (OtherActor :type Actor%20Object%20Reference))
  (bind _asbp_nest (Utilities|Casting|CastToBP_Nest OtherActor))
  (if (Actor|ActorHasTag _asbp_nest "Doused") ; Does the nest have the Doused tag?
    (if (not (Actor|ActorHasTag _asbp_nest "Fire")) ; Does the nest already have the Fire tag?
      (bind _returnvalue (Utilities|Array|Add (Variables|/Script/Engine.Actor|GetTags _asbp_nest) "Fire")) ; Gives the nest the Fire tag.
      (Development|PrintString (Utilities|String|ToString(Name) (Utilities|Array|Get(acopy) (Variables|/Script/Engine.Actor|GetTags _asbp_nest) _returnvalue))))))

(fn ConstructionScript
  (|CallParentFunction))