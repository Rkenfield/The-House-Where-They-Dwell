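; Dynamite actor that explodes on a timer or early when its capsule touches a player other than its owner, a SpiderWitch or a Spider.
; Direct player or witch contact overrides the explosion radius before detonation.
; Explode resizes a sphere, damages overlapping players and SpiderWitches but not Spiders, then plays effects and destroys itself.
; ResetSpawner marks the spawning TnTCrate unavailable, though nothing here calls it.
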(event OnComponentBeginOverlap(Capsule)
  (params (OverlappedComponent :type Primitive%20Component%20Object%20Reference) (OtherActor :type Actor%20Object%20Reference) (OtherComp :type Primitive%20Component%20Object%20Reference) (OtherBodyIndex :type Integer) (bFromSweep :type Boolean) (SweepResult :type Hit%20Result%20Structure%20%28by%20ref%29))
  (if (!= OtherActor self)
    (if (!= OtherActor (Variables|Default|GetOwningPlayer))
      (if (Actor|ActorHasTag OtherActor "Player")
        (Variables|Default|SetExplosionRadiusSize 1e+01)
        (CallFunction|Explode :!label _label)
        (elif (Actor|ActorHasTag OtherActor "SpiderWitch")
          (Variables|Default|SetExplosionRadiusSize 1e+01)
          (goto _label)
          (elif (Actor|ActorHasTag OtherActor "Spider")
            (goto _label)))))))

(event EventBeginPlay
  (Utilities|Time|SetTimerbyFunctionName self "Explode" (Variables|Default|GetTimeBeforeExplosion)))

(event Collision|EventActorBeginOverlap
  (params (OtherActor :type Actor%20Object%20Reference))
  (|CallParentFunction OtherActor) ; This node is disabled and will not be called.\nDrag off pins to build functionality.
)

(event EventTick
  (params (DeltaSeconds :type Float%20%28single-precision%29))
  (|CallParentFunction DeltaSeconds) ; This node is disabled and will not be called.\nDrag off pins to build functionality.
)

(fn ConstructionScript
  (|CallParentFunction))

(fn ResetSpawner
  (bind _astn_tcrate (Utilities|Casting|CastToTnTCrate (Variables|Default|GetSpawner)))
  (Variables|/Game/Blueprints/Blueprints/Item/TnTCrate.TnTCrate_C|SetAvailable _astn_tcrate false))

(fn Explode
  (bind _self self)
  (bind _explosionradius (Variables|Default|GetExplosionRadius))
  (bind _staticmesh (Variables|Default|GetStaticMesh))
  (bind _returnvalue (Transformation|GetWorldLocation _staticmesh))
  (Components|Sphere|SetSphereRadius _explosionradius (Variables|Default|GetExplosionRadiusSize) true)
  (for _array_element (Collision|GetOverlappingActors _explosionradius 0 :!class /Script/Engine.PrimitiveComponent)
    (if (!= _array_element _self)
      (if (Actor|ActorHasTag _array_element "Player")
        (bind _asbp_player_parent (Utilities|Casting|CastToBP_PlayerParent _array_element))
        (Default|TakeDamage _asbp_player_parent 3e+01 _self)
        (elif (Actor|ActorHasTag _array_element "SpiderWitch")
          (bind _asspider_witch_ch (Utilities|Casting|CastToSpiderWitchCH _array_element))
          (Variables|/Game/Blueprints/AI/SpiderWitch/SpiderWitchAI/SpiderWitchCH.SpiderWitchCH_C|SetHit? _asspider_witch_ch true)
          (Default|TakeDamage _asspider_witch_ch (Variables|Default|GetDamage) (Variables|Default|GetOwningPlayer))
          (elif (Actor|ActorHasTag _array_element "Spider")
            _)))))
  (Effects|SpawnEmitteratLocation "/Game/Art/Particles/Explosion/P_DynamiteExplosion.P_DynamiteExplosion" _returnvalue (Transformation|GetActorRotation) "2.000000,2.000000,2.000000")
  (Audio|PlaySoundatLocation "/Game/Audio/Cues/Interactables/Dynamite/Dynamite_Boom.Dynamite_Boom" _returnvalue "0, 0, 0" 1.0 1.0 0.0 "/Game/Audio/AttenuationSettings/Dynamite-Boom.Dynamite-Boom" 0 0)
  (Actor|DestroyActor))