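; Throwable doll item that acts as bait for the Pregnant Ghost in the Hunt Phase when thrown.
; Using it runs the parent item logic, flags it as bait and expands its range collider to the bait range.
; When the ghost overlaps the pickup collider, the bait switches off and the range shrinks.
; Through its Blackboard, the ghost pauses briefly, then stops being baited and regains chase speed.
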(event OnComponentBeginOverlap(PickupCollider)
  (params (OverlappedComponent :type Primitive%20Component%20Object%20Reference) (OtherActor :type Actor%20Object%20Reference) (OtherComp :type Primitive%20Component%20Object%20Reference) (OtherBodyIndex :type Integer) (bFromSweep :type Boolean) (SweepResult :type Hit%20Result%20Structure%20%28by%20ref%29))
  ;[1 1 1] If Pregnant Ghost reaches the doll when it is a bait, the doll stops being a bait. The ghost is pissed for a second before it stops being baited and then
  (bind _aspregnant_ghost (Utilities|Casting|CastToPregnant_Ghost OtherActor))
  (if (Variables|Default|GetGhostBait)
    (Variables|Default|SetGhostBait false)
    (Components|Sphere|SetSphereRadius (Variables|Default|GetRangeCollider) 32.0 true)
    (AI|Components|Blackboard|SetValueasFloat (AI|GetBlackboard _aspregnant_ghost) (Utilities|Name|MakeLiteralName "Speed") 0.0)
    (Utilities|FlowControl|Delay 2.0)
    (AI|Components|Blackboard|SetValueasBool (AI|GetBlackboard _aspregnant_ghost) (Utilities|Name|MakeLiteralName "Baited?") false)
    (AI|Components|Blackboard|SetValueasFloat (AI|GetBlackboard _aspregnant_ghost) (Utilities|Name|MakeLiteralName "Speed") (Variables|/Game/Blueprints/AI/Pregnant_Ghost/Pregnant_Ghost.Pregnant_Ghost_C|GetChaseSpeed _aspregnant_ghost))))

(event EventBeginPlay
  (|CallParentFunction) ; This node is disabled and will not be called.\nDrag off pins to build functionality.
)

(event Collision|EventActorBeginOverlap
  (params (OtherActor :type Actor%20Object%20Reference))
  (|CallParentFunction OtherActor) ; This node is disabled and will not be called.\nDrag off pins to build functionality.
)

(event EventTick
  (params (DeltaSeconds :type Float%20%28single-precision%29))
  (|CallParentFunction DeltaSeconds) ; This node is disabled and will not be called.\nDrag off pins to build functionality.
)

(fn ConstructionScript
  (|CallParentFunction))

(fn UseItem
  (params (User :type BP%20Player%20Parent%20Object%20Reference))
  ;[1 1 1] Acts as a bait for the Pregnant Ghost in the Hunt Phase when thrown.
  (bind _success (|CallParentFunction User))
  (Variables|Default|SetGhostBait true)
  (Components|Sphere|SetSphereRadius (Variables|Default|GetRangeCollider) (Variables|Default|GetBaitRange) true)
  (return _success))