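; Base pickup item actor with physics impact audio and stub use/passive-effect functions.
; Interact either adds the item to the interactor's inventory and destroys the actor, or, for non-inventory items, attaches the mesh to the player and calls PassiveEffect.
; Hits play item and surface-type sounds at a log-scaled impulse volume, gated by a threshold and cooldown, with optional debug printouts.
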(event EventBeginPlay
  (Audio|Components|Audio|SetSound (Variables|Default|GetItemImpact01) (Variables|Audio|GetItem_Impact_Cue)))

(event Collision|EventHit
  (params (MyComp :type Primitive%20Component%20Object%20Reference) (Other :type Actor%20Object%20Reference) (OtherComp :type Primitive%20Component%20Object%20Reference) (bSelfMoved :type Boolean) (HitLocation :type Vector :default "0, 0, 0") (HitNormal :type Vector :default "0, 0, 0") (NormalImpulse :type Vector :default "0, 0, 0") (Hit :type Hit%20Result%20Structure%20%28by%20ref%29))
  (bind _physmat (Collision|BreakHitResult Hit))
  (bind _returnvalue (Utilities|String|ToString(Vector) HitLocation))
  (bind _returnvalue_2 (Math|Vector|VectorLength NormalImpulse))
  (bind _returnvalue_3 (Math|Vector|VectorLength NormalImpulse))
  (bind _returnvalue_4 (Utilities|GetDisplayName Other))
  (bind _self self)
  (bind _self_2 self)
  (bind _impactthreshold (Variables|Audio|GetImpactThreshold))
  (bind _itemimpact01 (Variables|Default|GetItemImpact01))
  (bind _returnvalue_5 (Utilities|GetDisplayName _self))
  (bind _returnvalue_6 (Utilities|GetDisplayName _physmat))
  (bind _returnvalue_7 (* _returnvalue_3 0.0001))
  (bind _returnvalue_8 (* _returnvalue_2 0.0001))
  (bind _staticmesh (Variables|Default|GetStaticMesh _self_2))
  (bind _returnvalue_9 (Physics|GetMass _staticmesh))
  (bind _returnvalue_10 (Utilities|String|ToString(Float) _returnvalue_8))
  (bind _returnvalue_11 (+ _returnvalue_8 1.0))
  (bind _returnvalue_12 (+ _returnvalue_7 1.0))
  (bind _returnvalue_13 (Utilities|String|ToString(Float) _returnvalue_9))
  (bind _returnvalue_14 (Math|Float|Log _returnvalue_11 2.0))
  (bind _returnvalue_15 (Math|Float|Log _returnvalue_12 2.0))
  (bind _returnvalue_16 (Math|Float|Clamp(Float) _returnvalue_14 0.0 4.0))
  (bind _returnvalue_17 (Math|Float|Clamp(Float) _returnvalue_15 0.0 4.0))
  (bind _returnvalue_18 (Utilities|String|ToString(Float) _returnvalue_16))
  (bind _returnvalue_19 (> _returnvalue_17 _impactthreshold))
  (bind _returnvalue_20 (Utilities|String|Append " 
Actor: " _returnvalue_5 " 
Actor Struck: " _returnvalue_4 " 
Physics Material: " _returnvalue_6 " 
Location: " _returnvalue " 
Impulse: " _returnvalue_10 " 
Output: " _returnvalue_18 " 
Mass: " _returnvalue_13))
  ;[1 1 1] Audio- Impact physics
  (if (Variables|Audio|GetPhysics_Impact_Printout)
    ;;[1 1 1] Debug data
    (if _returnvalue_19
      (Development|PrintString _returnvalue_20)
      (if (Variables|Audio|GetPhysics_Impact_Sound) :!label _label
        (if _returnvalue_19
          (if (Variables|Audio|GetCanPlayImpact)
            (Variables|Audio|SetCanPlayImpact false)
            (Audio|Components|Audio|SetVolumeMultiplier _itemimpact01 _returnvalue_17 :!class /Script/Engine.AudioComponent)
            (Audio|Components|Audio|Play _itemimpact01 0.0)
            (Audio|PlaySoundatLocation (Utilities|Select :Index (Collision|GetSurfaceType Hit) :SurfaceType_Default 0 :SurfaceType1 "/Game/Audio/Cues/Environment/Physics/SurfaceImpact-Wood.SurfaceImpact-Wood" :SurfaceType2 "/Game/Audio/Cues/Environment/Physics/SurfaceImpact-Carpet.SurfaceImpact-Carpet" :SurfaceType3 "/Game/Audio/Cues/Environment/Physics/SurfaceImpact-Tile.SurfaceImpact-Tile" :SurfaceType4 "/Game/Audio/Cues/Environment/Physics/SurfaceImpact-Dirt.SurfaceImpact-Dirt" :SurfaceType5 "/Game/Audio/Cues/Environment/Physics/SurfaceImpact-Metal.SurfaceImpact-Metal" :SurfaceType6 "/Game/Audio/Cues/Environment/Physics/SurfaceImpact-Wood_Small.SurfaceImpact-Wood_Small" :SurfaceType7 "/Game/Audio/Cues/Environment/Physics/SurfaceImpact-Stone.SurfaceImpact-Stone" :SurfaceType8 "/Game/Audio/Cues/Environment/Physics/SurfaceImpact-Cardboard.SurfaceImpact-Cardboard" :SurfaceType9 "/Game/Audio/Cues/Environment/Physics/SurfaceImpact-Fabric.SurfaceImpact-Fabric" :SurfaceType10 "/Game/Audio/Cues/Environment/Physics/SurfaceImpact-Organic.SurfaceImpact-Organic") (.Location (Collision|BreakHitResult Hit)) "0, 0, 0" _returnvalue_17 1.0 0.0 "/Game/Audio/AttenuationSettings/ItemPhysics-01.ItemPhysics-01" 0 0)
            (Utilities|FlowControl|Delay (Variables|Audio|GetDelayBetweenImpacts))
            (Variables|Audio|SetCanPlayImpact true))))
      (elif (Variables|Audio|GetPhysics_Impact_PrintCulled)
        (Development|PrintString _returnvalue_20 true true "(R=1.000000,G=0.082666,B=0.000000,A=1.000000)")))
    (else
      (goto _label))))

(event EventInteract
  (params (Interactor :type Actor%20Object%20Reference) (HitComponent :type Primitive%20Component%20Object%20Reference))
  (bind _asbp_player_parent (Utilities|Casting|CastToBP_PlayerParent Interactor))
  (bind _staticmesh (Variables|Default|GetStaticMesh))
  ;[1 1 1] Item Pickup- Checking with inventory before being picked up
  (if (.non-inventory (Variables|Default|GetItemStructure)) ; Is it a non-inventory item?
    ;[1 1 1] Non-Inventory Item
    (Variables|/Game/Blueprints/Characters/BP_PlayerParent.BP_PlayerParent_C|SetHoldingNonInventoryItem _asbp_player_parent true)
    (Variables|/Game/Blueprints/Characters/BP_PlayerParent.BP_PlayerParent_C|SetNonInventoryItem _asbp_player_parent self)
    (Physics|SetSimulatePhysics _staticmesh false)
    (Collision|SetCollisionEnabled _staticmesh "NoCollision")
    (Transformation|AttachComponentToComponent _staticmesh (Variables|/Game/Blueprints/Characters/BP_PlayerParent.BP_PlayerParent_C|GetNonInventoryItemPlacement _asbp_player_parent) "Item" "SnapToTarget" "KeepRelative" "KeepRelative" true)
    (CallFunction|PassiveEffect _asbp_player_parent)
    (else
      (bind _success (Default|AddtoInventory (Actor|GetComponentbyClass Interactor "/Game/Blueprints/Blueprints/InventoryComponent.InventoryComponent_C") (Utilities|Struct|MakeSlotStructure (Variables|Default|GetItemStructure) (Variables|Default|GetQuantity) (Variables|Default|GetSprayCanJuice))))
      (if _success
        (Default|HUDRefresh (.AsBP%20Player%20Parent (Utilities|Casting|CastToBP_PlayerParent Interactor)))
        (Actor|DestroyActor)))))

(fn ConstructionScript)

(fn UseItem
  (params (User :type BP%20Player%20Parent%20Object%20Reference))
  ;[1 1 1] What the item should do when used by the player
  (return true))

(fn PassiveEffect
  (params (User :type BP%20Player%20Parent%20Object%20Reference))
  (return true))

(fn RemovePassive
  (params (User :type BP%20Player%20Parent%20Object%20Reference)))