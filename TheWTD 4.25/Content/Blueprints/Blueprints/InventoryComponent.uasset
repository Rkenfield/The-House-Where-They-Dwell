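; Inventory component that stores the owning player's items in a slot array sized on BeginPlay.
; AddToInventory tops up a matching partial stack or fills the first empty slot, with stack overflow recursing back into it.
; Separate counters track occupied slots and full slots to gate additions.
; It also sets spray-can state on the BP_PlayerParent owner, triggers passive item effects and refreshes equipped camera and spray checks.
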(event EventBeginPlay
  ;[1 1 1] Initializes the inventory with required size
  (CallFunction|PrepareInventory))

(event EventTick
  (params (DeltaSeconds :type Float%20%28single-precision%29)))

(fn AddtoInventory
  (params (ContentToAdd :type Slot%20Structure%20Structure))
  ;[1 1 1] Checks if inventory has space to add a new item and if yes, checks if item is to be stacked on an existing slot or added to a new slot.
  (Variables|Default|SetCharacter (.AsBP%20Player%20Parent (Utilities|Casting|CastToBP_PlayerParent (Components|GetOwner))))
  (if (< (Variables|Default|GetSlotsFilled) (Variables|Default|GetNoOfSlots)) ; Is SlotsFilled < NoOfSlots
    (if (== (.class (.itemstructure ContentToAdd)) "/Game/Blueprints/Blueprints/Item/BP_Item_Consumable_Spray.BP_Item_Consumable_Spray_C") ; Is it a spray can?
      (Variables|/Game/Blueprints/Characters/BP_PlayerParent.BP_PlayerParent_C|SetHasSprayCan (Variables|Default|GetCharacter) true)
      (if (> (Variables|/Game/Blueprints/Characters/BP_PlayerParent.BP_PlayerParent_C|GetSprayJuice (Variables|Default|GetCharacter)) 0.0) ; Is SprayJuice already > 0?
        _
        (else
          (Variables|/Game/Blueprints/Characters/BP_PlayerParent.BP_PlayerParent_C|SetSprayJuice (Variables|Default|GetCharacter) 1e+02))))
    (if (.isstackable (.itemstructure ContentToAdd)) ; Is the item stackable?
      ;;[1 1 1] Adding Stackable Items
      (bind _stackindex (Utilities|HasStack ContentToAdd)
        (:True
          (CallFunction|AddtoStack ContentToAdd _stackindex)
          (LocalVariables|SetAddSuccess true :!label _label)
          (if (.ispassive (.itemstructure ContentToAdd))
            (bind _asbp_player_parent (Utilities|Casting|CastToBP_PlayerParent (Components|GetOwner)))
            (Default|PassiveItem _asbp_player_parent (.class (.itemstructure ContentToAdd)))))
        (:False
          (if (< (Variables|Default|GetSlotsTaken) (Variables|Default|GetNoOfSlots)) :!label _label_2 ; Is SlotsTaken<NoOfSlots
            (CallFunction|CreateStack ContentToAdd)
            (goto _label)
            (else
              (Development|PrintString "Failure from Inventory Component function \"Add to Inventory\": Full Inventory")
              (LocalVariables|SetAddSuccess false)))))
      (else
        (goto _label_2)))
    (else
      (LocalVariables|SetAddSuccess false)
      (Development|PrintString "Failure from Inventory Component function \"Add to Inventory\": Full Inventory")))
  (Default|CheckEquippedCamera (Variables|Default|GetCharacter))
  (Default|CheckEquippedSpray (Variables|Default|GetCharacter))
  (return (LocalVariables|GetAddSuccess)))

(fn CreateStack
  (params (ContentToAdd :type Slot%20Structure%20Structure))
  (bind _inventory (Variables|Default|GetInventory))
  ;[1 1 1] (Redone by Alex on 1/4/2021): Adding Item to Slot- Finds the first free slot available and adds item to that slot
  (Variables|Default|SetContentToAdd ContentToAdd)
  (bind (_array_element _array_index) (Utilities|Array|ForEachLoopwithBreak (Variables|Default|GetInventory) :!label _label)
    (:LoopBody
      ;;[1 1 1] Finds an empty slot
      (if (<= (.quantity _array_element) 0)
        (LocalVariables|SetHasSpace true)
        (LocalVariables|SetIdentifiedIndex _array_index)
        (goto _label Break)))
    (:Completed
      (if (LocalVariables|GetHasSpace)
        (Utilities|Array|SetArrayElem _inventory (LocalVariables|GetIdentifiedIndex) (Variables|Default|GetContentToAdd))
        (if (or (not (.isstackable (.ItemStructure (Utilities|Struct|BreakSlotStructure (Utilities|Array|Get(acopy) _inventory (LocalVariables|GetIdentifiedIndex)))))) (== (.maxstacksize (.ItemStructure (Utilities|Struct|BreakSlotStructure (Utilities|Array|Get(acopy) _inventory (LocalVariables|GetIdentifiedIndex))))) (.Quantity (Utilities|Struct|BreakSlotStructure (Utilities|Array|Get(acopy) _inventory (LocalVariables|GetIdentifiedIndex)))))) ; Alex 1/22/21: Is the slot at its MaxStackSize or unstackable? To fix a bug
          (bind _output_get (Variables|Default|SetSlotsFilled (+ (Variables|Default|GetSlotsFilled) 1))))
        (bind _output_get_2 (Variables|Default|SetSlotsTaken (+ (Variables|Default|GetSlotsTaken) 1)))
        (return (LocalVariables|GetHasSpace))
        (else
          (return false))))))

(fn PrepareInventory
  ;[1 1 1] Sets the size of the inventory
  (Utilities|Array|Resize (Variables|Default|GetInventory) (Variables|Default|GetNoOfSlots)))

(fn AddtoStack
  (params (SlotStructure :type Slot%20Structure%20Structure) (SlotIndex :type Integer))
  (bind _inventory (Variables|Default|GetInventory))
  (bind _inventory_2 (Variables|Default|GetInventory))
  (bind _maxstacksize (Utilities|Struct|BreakItemStructure (.itemstructure SlotStructure)))
  (bind _output (Utilities|Array|Get(acopy) _inventory SlotIndex))
  ;[1 1 1] Adding Quantity to Stack
  (bind _output_get (LocalVariables|SetCurrentQuantity (.quantity _output)))
  (if (> (+ _output_get (.Quantity (Utilities|Struct|BreakSlotStructure SlotStructure))) (.maxstacksize (.itemstructure _output)))
    ;[1 1 1] If Quantity > Max Stack Size
    (Utilities|Array|SetArrayElem (Variables|Default|GetInventory) SlotIndex (Utilities|Struct|MakeSlotStructure (.itemstructure SlotStructure) _maxstacksize))
    (CallFunction|AddtoInventory (Utilities|Struct|MakeSlotStructure (.itemstructure SlotStructure) (- (.quantity SlotStructure) (- _maxstacksize (LocalVariables|GetCurrentQuantity)))))
    (else
      (if (== (+ _output_get (.Quantity (Utilities|Struct|BreakSlotStructure SlotStructure))) (.maxstacksize (.itemstructure _output))) ; By adding this item to the stack, will the stack now be at its max?
        (Variables|Default|SetSlotsFilled (+ (Variables|Default|GetSlotsFilled) 1)))
      (Utilities|Array|SetArrayElem _inventory_2 SlotIndex (Utilities|Struct|MakeSlotStructure (.itemstructure (Utilities|Array|Get(acopy) _inventory_2 SlotIndex)) (+ _output_get (.Quantity (Utilities|Struct|BreakSlotStructure SlotStructure)))))))
  (return))