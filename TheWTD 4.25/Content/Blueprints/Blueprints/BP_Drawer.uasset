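; Interactable drawer Blueprint that slides open and closed when a BP_PlayerParent interacts with it.
; The Interact event calls OpenDrawer, which toggles IsOpen and plays or reverses the DrawerDriver timeline.
; The timeline's curve lerps the Pivot component's relative location between StartPosition and EndPosition.
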(event Custom|OpenDrawer
  ;[1 1 1] Alex: Event that defines the function that opens the door.
  (Utilities|Casting|CastToBP_PlayerParent (Game|GetPlayerCharacter 0))
  (if (Variables|Default|GetisOpen)
    (Variables|Default|SetisOpen false)
    (bind _drawercurve (Timeline|DrawerDriver Reverse)
      (:Update
        (Transformation|SetRelativeLocation (Variables|Default|GetPivot) (Math|Vector|Lerp(Vector) (Variables|Default|GetstartPosition) (Variables|Default|GetendPosition) _drawercurve) false false)))
    (else
      (Variables|Default|SetisOpen true)
      (Timeline|DrawerDriver Play))))

(event EventBeginPlay)

(event Collision|EventActorBeginOverlap
  (params (OtherActor :type Actor%20Object%20Reference)))

(event EventTick
  (params (DeltaSeconds :type Float%20%28single-precision%29)))

(event EventInteract
  (params (Interactor :type Actor%20Object%20Reference))
  ;[1 1 1] Alex: In Class Settings for this bp, make sure you have BPI_Interaction as one of the implemented interfaces. This event says to execute the OpenDrawer function.
  (Utilities|Casting|CastToBP_PlayerParent Interactor)
  (CallFunction|OpenDrawer))

(fn ConstructionScript)