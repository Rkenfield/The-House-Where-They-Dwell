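; Computer station objective where the player deposits equipment and which must survive damage while uploading data.
; Interacting removes the recorder, camera or held item from the player and increments the GameMode's placed count.
; The third item starts Phase 2 and a timeline-driven upload bar, whose completion triggers Phase 3.
; Scaled damage updates a health widget, and zero health calls Failure on the player.
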(event Custom|TakeDamage
  (params (Damage :type Float%20%28single-precision%29))
  (bind _output_get (Variables|Default|SetCSHealth (- (Variables|Default|GetCSHealth) (* Damage (Variables|Default|GetDamageMultiplier)))))
  (Default|UpdateHealth (Variables|Default|GetComputerStationHealthWidget) _output_get)
  (if (<= (Variables|Default|GetCSHealth) 0.0)
    (bind _asbp_player_parent (Utilities|Casting|CastToBP_PlayerParent (Game|GetPlayerCharacter 0)))
    (Default|Failure _asbp_player_parent)))

(event Custom|Audio-Camera_Setupload
  (bind _camera_setupload (Variables|Default|GetCamera_SetUpload))
  (Audio|Components|Audio|Play _camera_setupload 0.0)
  (Audio|PlaySoundatLocation "/Game/Audio/Cues/Interactables/Camera/Camera_equip.Camera_equip" (Transformation|GetWorldLocation _camera_setupload) "0, 0, 0" 0.1 0.9 0.75 0 0 0))

(event EventBeginPlay
  (Utilities|FlowControl|Sequence
    (:then_0
      (bind _ascomputer_station_health_widget (Utilities|Casting|CastToComputerStationHealthWidget (UserInterface|GetUserWidgetObject (Variables|Default|GetHealthBar))))
      (bind _output_get (Variables|Default|SetComputerStationHealthWidget _ascomputer_station_health_widget))
      (bind _output_get_2 (Variables|Default|SetCSHealth (Variables|/Game/Blueprints/ComputerStationHealthWidget.ComputerStationHealthWidget_C|GetCSWidgetHealth _output_get)))
      (Default|UpdateHealth _output_get _output_get_2))
    (:then_1
      (bind _ascomputer_station_upload_widget (Utilities|Casting|CastToComputerStationUploadWidget (UserInterface|GetUserWidgetObject (Variables|Default|GetUploadBar))))
      (bind _output_get_3 (Variables|Default|SetComputerStationUploadWidget _ascomputer_station_upload_widget))
      (bind _output_get_4 (Variables|Default|SetCSData (Variables|/Game/Blueprints/ComputerStationUploadWidget.ComputerStationUploadWidget_C|GetCSWidgetData _output_get_3)))
      (Default|UpdateUploadBar _output_get_3 _output_get_4))))

(event EventInteract
  (params (Interactor :type Actor%20Object%20Reference) (HitComponent :type Primitive%20Component%20Object%20Reference))
  (bind _asbp_player_parent (Utilities|Casting|CastToBP_PlayerParent Interactor))
  (bind _output_get (Variables|Default|SetCharacter _asbp_player_parent))
  (bind _asbp_wtdgame_mode (Utilities|Casting|CastToBP_WTDGameMode (Game|GetGameMode)))
  (Variables|Default|SetGameMode _asbp_wtdgame_mode)
  (bind (_recorderindex _camindex) (Default|FindEquipment _output_get))
  (if (Variables|/Game/Blueprints/Characters/BP_PlayerParent.BP_PlayerParent_C|GetHasAudioRecorder (Variables|Default|GetCharacter)) ; Does the player have an audio recorder in their inventory?
    (Variables|/Game/Blueprints/Blueprints/InventoryComponent.InventoryComponent_C|SetSlotsFilled (Variables|/Game/Blueprints/Characters/BP_PlayerParent.BP_PlayerParent_C|GetInventoryComponent (Variables|Default|GetCharacter)) (- (Variables|/Game/Blueprints/Blueprints/InventoryComponent.InventoryComponent_C|GetSlotsFilled (Variables|/Game/Blueprints/Characters/BP_PlayerParent.BP_PlayerParent_C|GetInventoryComponent (Variables|Default|GetCharacter))) 1))
    (Utilities|Array|SetArrayElem :TargetArray (Variables|/Game/Blueprints/Blueprints/InventoryComponent.InventoryComponent_C|GetInventory (Variables|/Game/Blueprints/Characters/BP_PlayerParent.BP_PlayerParent_C|GetInventoryComponent (Variables|Default|GetCharacter))) :Index _recorderindex) ; Makes the recorder's slot  blank.
    (Variables|/Game/Blueprints/BP_WTDGameMode.BP_WTDGameMode_C|SetEquipmentPlaced (Variables|Default|GetGameMode) (+ (Variables|/Game/Blueprints/BP_WTDGameMode.BP_WTDGameMode_C|GetEquipmentPlaced (Variables|Default|GetGameMode)) 1))
    (CallFunction|Audio-CameraSetupload)
    (Variables|/Game/Blueprints/Characters/BP_PlayerParent.BP_PlayerParent_C|SetHasAudioRecorder (Variables|Default|GetCharacter) false))
  (if (Variables|/Game/Blueprints/Characters/BP_PlayerParent.BP_PlayerParent_C|GetHasCamera (Variables|Default|GetCharacter)) ; Do you have a camera in your inventory?
    (Variables|/Game/Blueprints/Blueprints/InventoryComponent.InventoryComponent_C|SetSlotsFilled (Variables|/Game/Blueprints/Characters/BP_PlayerParent.BP_PlayerParent_C|GetInventoryComponent (Variables|Default|GetCharacter)) (- (Variables|/Game/Blueprints/Blueprints/InventoryComponent.InventoryComponent_C|GetSlotsFilled (Variables|/Game/Blueprints/Characters/BP_PlayerParent.BP_PlayerParent_C|GetInventoryComponent (Variables|Default|GetCharacter))) 1))
    (Utilities|Array|SetArrayElem :TargetArray (Variables|/Game/Blueprints/Blueprints/InventoryComponent.InventoryComponent_C|GetInventory (Variables|/Game/Blueprints/Characters/BP_PlayerParent.BP_PlayerParent_C|GetInventoryComponent (Variables|Default|GetCharacter))) :Index _camindex)
    (Variables|/Game/Blueprints/BP_WTDGameMode.BP_WTDGameMode_C|SetEquipmentPlaced (Variables|Default|GetGameMode) (+ (Variables|/Game/Blueprints/BP_WTDGameMode.BP_WTDGameMode_C|GetEquipmentPlaced (Variables|Default|GetGameMode)) 1))
    (Variables|/Game/Blueprints/Characters/BP_PlayerParent.BP_PlayerParent_C|SetHasCamera (Variables|Default|GetCharacter) false)
    (Default|CheckEquippedCamera (Variables|Default|GetCharacter))
    (CallFunction|Audio-CameraSetupload))
  (if (Variables|/Game/Blueprints/Characters/BP_PlayerParent.BP_PlayerParent_C|GetHoldingNonInventoryItem (Variables|Default|GetCharacter)) ; Are you holding a non-inventory item?
    (Transformation|DetachFromComponent (Variables|/Game/Blueprints/Blueprints/Item/BP_Item.BP_Item_C|GetStaticMesh (Variables|/Game/Blueprints/Characters/BP_PlayerParent.BP_PlayerParent_C|GetNonInventoryItem (Variables|Default|GetCharacter))) "KeepRelative" "KeepRelative" "KeepRelative" true)
    (Actor|DestroyActor (Variables|/Game/Blueprints/Characters/BP_PlayerParent.BP_PlayerParent_C|GetNonInventoryItem (Variables|Default|GetCharacter)))
    (Variables|/Game/Blueprints/BP_WTDGameMode.BP_WTDGameMode_C|SetEquipmentPlaced (Variables|Default|GetGameMode) (+ (Variables|/Game/Blueprints/BP_WTDGameMode.BP_WTDGameMode_C|GetEquipmentPlaced (Variables|Default|GetGameMode)) 1))
    (Variables|/Game/Blueprints/Characters/BP_PlayerParent.BP_PlayerParent_C|SetHoldingNonInventoryItem (Variables|Default|GetCharacter) false)
    (CallFunction|Audio-CameraSetupload))
  (Default|HUDRefresh (Variables|Default|GetCharacter))
  (if (== (Variables|/Game/Blueprints/BP_WTDGameMode.BP_WTDGameMode_C|GetEquipmentPlaced (Variables|Default|GetGameMode)) 3)
    (Utilities|FlowControl|DoOnce false
      (:Completed
        (Variables|Default|SetAllEquipmentPlaced true)
        (Default|SetPhase2 (Variables|Default|GetGameMode))
        (bind _data (Timeline|UploadBarTimeline Play) ; IMPORTANT NOTE: Time and value of Data timeline should be the same. Also, the length of the timeline should be equal to MaxCSData.
          (:Update
            (bind _output_get_2 (Variables|Default|SetCSData _data))
            (Default|UpdateUploadBar (Variables|Default|GetComputerStationUploadWidget) (/ _output_get_2 (Variables|Default|GetMaxCSData))))
          (:Finished
            (Default|SetPhase3 (Variables|Default|GetGameMode))))))))

(fn ConstructionScript)