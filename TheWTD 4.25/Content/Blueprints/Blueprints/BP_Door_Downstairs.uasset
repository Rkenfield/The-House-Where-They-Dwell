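; Downstairs door actor that swings open or closed each time its OpenDownstairsDoors event runs, after a configurable delay.
; An IsOpen flag picks the direction, playing or reversing a Timeline whose curve lerps the Pivot's relative rotation between start and end rotations.
; Open and close sounds cross-fade so reversals mid-sound blend, and closing also triggers PlayDoorCloseBoom.
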(event Custom|OpenDownstairsDoors
  ;[1 1 1] OpenDownstairsDoors
  (Utilities|FlowControl|Delay (Variables|Default|GetDownstairsDelay))
  (if (Variables|Default|GetIsOpen)
    (Variables|Default|SetIsOpen false) ; If IsOpen is true, set it to false.
    ;;[1 1 1] Audio Cues
    (if (Audio|Components|Audio|IsPlaying (Variables|Default|GetOpen)) ; If still playing open...
      (Audio|Components|Audio|FadeOut (Variables|Default|GetOpen) 0.3 0.0 "SCurve" :!class /Script/Engine.AudioComponent) ; fade open out...
    )
    (Audio|Components|Audio|FadeIn (Variables|Default|GetClose) 0.5 1.0 0.0 "Sin" :!class /Script/Engine.AudioComponent) ; in both cases fade in close
    (CallFunction|PlayDoorCloseBoom)
    (bind _doorcurve (Timeline|Timeline_1 Reverse)
      (:Update
        (Transformation|SetRelativeRotation (Variables|Default|GetPivot) (Math|Rotator|Lerp(Rotator) (Variables|Default|GetStartRotation) (Variables|Default|GetEndRotation) _doorcurve) false false)))
    (else
      (Variables|Default|SetIsOpen true) ; If IsOpen is false, set it to true.
      (if (Audio|Components|Audio|IsPlaying (Variables|Default|GetClose)) ; If still playing close...
        (Audio|Components|Audio|FadeOut (Variables|Default|GetClose) 0.3 0.0 "SCurve" :!class /Script/Engine.AudioComponent) ; fade close out...
      )
      (Audio|Components|Audio|FadeIn (Variables|Default|GetOpen) 0.05 1.0 0.0 "Sin" :!class /Script/Engine.AudioComponent) ; in both cases fade in open
      (Timeline|Timeline_1 Play))))

(event EventBeginPlay
  (|CallParentFunction) ; This node is disabled and will not be called.\nDrag off pins to build functionality.
)

(event Collision|EventActorBeginOverlap
  (params (OtherActor :type Actor%20Object%20Reference)))

(event EventTick
  (params (DeltaSeconds :type Float%20%28single-precision%29)))

(fn ConstructionScript
  (|CallParentFunction))