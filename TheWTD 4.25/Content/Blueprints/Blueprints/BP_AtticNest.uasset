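; BP_AtticNest is a nest actor for the attic that triggers fire propagation in its room when it is about to be destroyed.
; After running the parent Tick, it checks the AboutToBeDestroyed flag each frame.
; While the flag is set, it casts AtticOwner to Room_Attic and calls FirePropogation, repeating every tick with no one-shot guard.
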(event EventBeginPlay
  (|CallParentFunction) ; This node is disabled and will not be called.\nDrag off pins to build functionality.
)

(event Collision|EventActorBeginOverlap
  (params (OtherActor :type Actor%20Object%20Reference))
  (|CallParentFunction OtherActor) ; This node is disabled and will not be called.\nDrag off pins to build functionality.
)

(event EventTick
  (params (DeltaSeconds :type Float%20%28single-precision%29))
  (|CallParentFunction DeltaSeconds)
  (if (Variables|Default|GetAboutToBeDestroyed)
    (bind _asroom_attic (Utilities|Casting|CastToRoom_Attic (Variables|Default|GetAttic_Owner)))
    (Default|FirePropogation _asroom_attic)))

(fn ConstructionScript
  (|CallParentFunction))