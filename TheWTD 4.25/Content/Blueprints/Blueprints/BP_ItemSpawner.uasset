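; Item spawner actor that places one random pickup at its own location and rotation, based on the current game phase.
; On BeginPlay it caches BP_WTDGameMode and calls AttemptToSpawn, which spawns only if its CurrentItem is no longer valid.
; SpawnItem reads CurrentPhase to pick from the Phase 1 or Phase 2/3 class array, the latter adding matchboxes and lighter fluid.
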(event EventBeginPlay
  ;[1 1 1] Sets the value of the variable GameMode and also spawns the first items for the first phase.
  (bind _asbp_wtdgame_mode (Utilities|Casting|CastToBP_WTDGameMode (Game|GetGameMode)))
  (Variables|Default|SetGameMode _asbp_wtdgame_mode)
  (CallFunction|AttempttoSpawn))

(event Collision|EventActorBeginOverlap
  (params (OtherActor :type Actor%20Object%20Reference)))

(event EventTick
  (params (DeltaSeconds :type Float%20%28single-precision%29)))

(fn ConstructionScript)

(fn AttempttoSpawn
  (Utilities|IsValid (Variables|Default|GetCurrentItem) ; Is the item already spawned?
    (:Is%20Valid
      (Development|PrintString "Item already spawned."))
    (:Is%20Not%20Valid
      (CallFunction|SpawnItem))))

(fn SpawnItem
  (bind _gamemode (Variables|Default|GetGameMode)
    (:then
      (if (>= (Variables|/Game/Blueprints/BP_WTDGameMode.BP_WTDGameMode_C|GetCurrentPhase _gamemode) 2) ; Is it Phase 2 or 3?
        ;[1 1 1] If it is Phase 2 or 3, include matchboxes and lighterfluid (uses SpawnableItemsPhase2&3 array)
        (bind _returnvalue (Game|SpawnActorfromClass (Utilities|Array|Get(acopy) (Variables|Default|GetSpawnableItemsPhase2&3) (Math|Random|RandomIntegerinRange 0 (- (Utilities|Array|Length (Variables|Default|GetSpawnableItemsPhase2&3)) 1))) (Math|Transform|MakeTransform (Transformation|GetActorLocation) (Transformation|GetActorRotation)) "AdjustIfPossibleButAlwaysSpawn" 0 0))
        (Variables|Default|SetCurrentItem _returnvalue)
        (else
          ;[1 1 1] If it is Phase 1, exclude matchboxes and lighterfluid (uses SpawnableItemsPhase1 array)
          (bind _returnvalue_2 (Game|SpawnActorfromClass (Utilities|Array|Get(acopy) (Variables|Default|GetSpawnableItemsPhase1) (Math|Random|RandomIntegerinRange 0 (- (Utilities|Array|Length (Variables|Default|GetSpawnableItemsPhase1)) 1))) (Math|Transform|MakeTransform (Transformation|GetActorLocation) (Transformation|GetActorRotation)) "AdjustIfPossibleButAlwaysSpawn" 0 0))
          (Variables|Default|SetCurrentItem _returnvalue_2))))
    (:else)))