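; BPC_MatchFluidSpawner is a scene component that spawns a random item at its own location, named for match fluid pickups.
; On BeginPlay it caches the BP_WTDGameMode and calls AttemptToSpawn, whose logic is not defined in this graph.
; SpawnItem picks a random class from UniqueSpawnableItems, spawns it at the component's transform with unit scale, and stores it as CurrentItem.
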(event EventBeginPlay
  (bind _asbp_wtdgame_mode (Utilities|Casting|CastToBP_WTDGameMode (Game|GetGameMode)))
  (Variables|Default|SetGameMode _asbp_wtdgame_mode)
  (CallFunction|AttempttoSpawn))

(event EventTick
  (params (DeltaSeconds :type Float%20%28single-precision%29))
  (|CallParentFunction DeltaSeconds) ; This node is disabled and will not be called.\nDrag off pins to build functionality.
)

(fn SpawnItem
  (bind _returnvalue (Game|SpawnActorfromClass (Utilities|Array|Get(acopy) (Variables|Default|GetUniqueSpawnableItems) (Math|Random|RandomIntegerinRange 0 (- (Utilities|Array|Length (Variables|Default|GetUniqueSpawnableItems)) 1))) (Math|Transform|MakeTransform (Transformation|GetWorldLocation) (Transformation|GetWorldRotation)) "AdjustIfPossibleButAlwaysSpawn" 0 0))
  (Variables|Default|SetCurrentItem _returnvalue))