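; Interactive drawer actor that toggles open and closed when a ThirdPersonCharacter interacts with it.
; Interact checks the interactor and calls OpenDrawer, which flips IsOpen and plays or reverses the DrawerDriver timeline.
; The timeline update sets the actor's relative location to a fixed zero vector, with no track value feeding the movement.
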(event Custom|OpenDrawer
  (Utilities|Casting|CastToThirdPersonCharacter (Game|GetPlayerCharacter 0))
  (if (Variables|Default|GetIsOpen)
    (Variables|Default|SetIsOpen false)
    (Timeline|DrawerDriver Reverse
      (:Update
        (Transformation|SetActorRelativeLocation "0, 0, 0")))
    (else
      (Variables|Default|SetIsOpen true)
      (Timeline|DrawerDriver Play))))

(event EventBeginPlay)

(event Collision|EventActorBeginOverlap
  (params (OtherActor :type Actor%20Object%20Reference)))

(event EventTick
  (params (DeltaSeconds :type Float%20%28single-precision%29)))

(event EventInteract
  (params (Interactor :type Actor%20Object%20Reference))
  (Utilities|Casting|CastToThirdPersonCharacter Interactor)
  (CallFunction|OpenDrawer))

(fn ConstructionScript)