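; BP_Cradle is an interactable cradle that takes a matching item from the player's inventory and places it in the world.
; On Interact by a ThirdPersonCharacter, TakeItem checks only the first inventory slot of player 0 against the CradleItem name.
; A match spawns that item's class at the mesh's "Object" socket, copies its quantity, decrements SlotsFilled and writes back to the array.
; An unconnected "ForCradle" tag check never runs.
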(event Custom|TakeItem
  (bind _asthird_person_character (Utilities|Casting|CastToThirdPersonCharacter (Game|GetPlayerCharacter 0)))
  (bind _output_get (Variables|Default|SetinventoryComponent (Variables|/Game/Blueprints/Characters/ThirdPersonCharacter.ThirdPersonCharacter_C|GetInventoryComponent _asthird_person_character)))
  (if (Utilities|IsValidClass (.class (.itemstructure (Utilities|Array|Get(acopy) (Variables|/Game/Blueprints/Blueprints/InventoryComponent.InventoryComponent_C|GetInventory _output_get)))))
    (if (Utilities|Enum|Equal(Enum) (.name (.itemstructure (Utilities|Array|Get(acopy) (Variables|/Game/Blueprints/Blueprints/InventoryComponent.InventoryComponent_C|GetInventory _output_get)))) (Variables|Default|GetCradle%20Item)) ; Does the item have the ItemStructureName "Cradle Item"?
      (bind _returnvalue (Game|SpawnActorfromClass (.class (.itemstructure (Utilities|Array|Get(acopy) (Variables|/Game/Blueprints/Blueprints/InventoryComponent.InventoryComponent_C|GetInventory _output_get)))) (Math|Conversions|ToTransform(Vector) (Transformation|GetSocketLocation (Variables|Debug|GetStaticMeshComponent) "Object")) "Undefined" 0 0))
      (Variables|/Game/Blueprints/Blueprints/Item/BP_Item.BP_Item_C|SetQuantity _returnvalue (.quantity (Utilities|Array|Get(acopy) (Variables|/Game/Blueprints/Blueprints/InventoryComponent.InventoryComponent_C|GetInventory _output_get))))
      (Variables|/Game/Blueprints/Blueprints/InventoryComponent.InventoryComponent_C|SetSlotsFilled (Variables|Default|GetinventoryComponent) (- (Variables|/Game/Blueprints/Blueprints/InventoryComponent.InventoryComponent_C|GetSlotsFilled (Variables|Default|GetinventoryComponent)) 1))
      (Utilities|Array|SetArrayElem :TargetArray (Variables|/Game/Blueprints/Blueprints/InventoryComponent.InventoryComponent_C|GetInventory (Variables|Default|GetinventoryComponent))))))

(event EventBeginPlay)

(event Collision|EventActorBeginOverlap
  (params (OtherActor :type Actor%20Object%20Reference)))

(event EventTick
  (params (DeltaSeconds :type Float%20%28single-precision%29)))

(event EventInteract
  (params (Interactor :type Actor%20Object%20Reference))
  (Utilities|Casting|CastToThirdPersonCharacter Interactor)
  (CallFunction|TakeItem))

(fn ConstructionScript)