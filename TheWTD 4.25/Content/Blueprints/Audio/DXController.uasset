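; Dialogue controller that plays voice lines for Vincent (player 1), Laveau (player 2) and a Producer in response to game events.
; DX events select cues by character, location or item, with chance and delay on item lines.
; A shared helper fades out the current line and skips new ones while the Producer speaks, unless overridden.
; Some lines pick a speaker by player count, and the power-outage sequence polls for silence before the Producer talks.
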(event Custom|DX_PowerOff
  ;[1 1 1] DX_PowerOff
  (Audio|PlaySound2D "/Game/Audio/Cues/Environment/Env_Thunder.Env_Thunder" 1.0 1.0 0.0 0 0)
  (Utilities|FlowControl|Delay 1.5)
  (Audio|PlaySound2D "/Game/Audio/Cues/NPC/Spiderwitch_Scream-Thunder-Vox.Spiderwitch_Scream-Thunder-Vox" 1.0 1.0 0.0 0 0)
  (Utilities|FlowControl|Delay 3.0) ; Dialog
  (CallFunction|Audio-PlaybyPlayerCount "/Game/Audio/Dialog/Laveau/CUES/TANGENTS/dx_lav_tan_DIDNTMEANTOTRESPASS.dx_lav_tan_DIDNTMEANTOTRESPASS" "/Game/Audio/Dialog/Vincent/CUES/CALLS/VIN_CALL_MONSTERSOUNDRESPONSE.VIN_CALL_MONSTERSOUNDRESPONSE" true 5e+01)
  (Utilities|FlowControl|Delay 1.0) ; To make sure something's playing by this point
  (Utilities|DelayUntilSilent (Variables|Default|GetVincent) (Variables|Default|GetLaveau))
  (CallFunction|Audio-FadePlayingforNew 0.075 (Variables|Default|GetProducer) "/Game/Audio/Dialog/Producer/dx_pro_CAUSEDAPOWEROUTAGE.dx_pro_CAUSEDAPOWEROUTAGE" 1.75 false))

(event Custom|DX_GetThatFootageUploaded
  ;[1 1 1] DX_GetThatFootageUploaded
  (Utilities|FlowControl|Delay 0.45)
  (CallFunction|Audio-FadePlayingforNew 0.075 (Variables|Default|GetProducer) "/Game/Audio/Dialog/Producer/dx_pro_GETTHATFOOTAGEUPLOADED.dx_pro_GETTHATFOOTAGEUPLOADED" 1.75 true))

(event Custom|DX_LocationCall
  (params (IsPlayer2 :type Boolean) (Enum :type DX_LocationCall%20Enum :default "NewEnumerator1"))
  ;[1 1 1] DX_ItemPickup
  (if IsPlayer2
    (switch Utilities|FlowControl|Switch|SwitchonDX_LocationCall Enum ; Laveau
      (:NewEnumerator1
        (Variables|TempVariables|SetTempLocationCallSound_Lav 0))
      (:NewEnumerator2
        (Variables|TempVariables|SetTempLocationCallSound_Lav "/Game/Audio/Dialog/Laveau/CUES/CALLS/LAV_CALL_LABFOUND.LAV_CALL_LABFOUND"))
      (:NewEnumerator3
        (Variables|TempVariables|SetTempLocationCallSound_Lav 0))
      (:NewEnumerator4
        (Variables|TempVariables|SetTempLocationCallSound_Lav 0))
      (:NewEnumerator14
        (Variables|TempVariables|SetTempLocationCallSound_Lav 0))
      (:NewEnumerator15
        (Variables|TempVariables|SetTempLocationCallSound_Lav 0))
      (:NewEnumerator5
        (Variables|TempVariables|SetTempLocationCallSound_Lav "/Game/Audio/Dialog/Laveau/CUES/CALLS/LAV_CALL_RUINSFOUND.LAV_CALL_RUINSFOUND"))
      (:NewEnumerator6
        (Variables|TempVariables|SetTempLocationCallSound_Lav 0))
      (:NewEnumerator16
        (Variables|TempVariables|SetTempLocationCallSound_Lav 0))
      (:NewEnumerator8
        (Variables|TempVariables|SetTempLocationCallSound_Lav 0))
      (:NewEnumerator9
        (Variables|TempVariables|SetTempLocationCallSound_Lav "/Game/Audio/Dialog/Laveau/CUES/CALLS/LAV_CALL_ATTICFOUND.LAV_CALL_ATTICFOUND"))
      (:NewEnumerator10
        (Variables|TempVariables|SetTempLocationCallSound_Lav "/Game/Audio/Dialog/Laveau/CUES/CALLS/LAV_CALL_ATTICFOUNDBLOCKED.LAV_CALL_ATTICFOUNDBLOCKED"))
      (:NewEnumerator7
        (Variables|TempVariables|SetTempLocationCallSound_Lav "/Game/Audio/Dialog/Laveau/CUES/CALLS/LAV_CALL_SWITCHFOUND.LAV_CALL_SWITCHFOUND")))
    (CallFunction|Audio-FadePlayingforNew 0.075 (Variables|Default|GetLaveau) (Variables|TempVariables|GetTempLocationCallSound_Lav) 1.75 false)
    (else
      (switch Utilities|FlowControl|Switch|SwitchonDX_LocationCall Enum ; Vincent
        (:NewEnumerator1
          (Variables|TempVariables|SetTempLocationCallSound_Vin "/Game/Audio/Dialog/Vincent/CUES/CALLS/VIN_CALL_GAMEROOM.VIN_CALL_GAMEROOM"))
        (:NewEnumerator2
          (Variables|TempVariables|SetTempLocationCallSound_Vin "/Game/Audio/Dialog/Vincent/CUES/CALLS/VIN_CALL_LAB.VIN_CALL_LAB"))
        (:NewEnumerator3
          (Variables|TempVariables|SetTempLocationCallSound_Vin "/Game/Audio/Dialog/Vincent/CUES/CALLS/VIN_CALL_ROOM1.VIN_CALL_ROOM1"))
        (:NewEnumerator4
          (Variables|TempVariables|SetTempLocationCallSound_Vin "/Game/Audio/Dialog/Vincent/CUES/CALLS/VIN_CALL_ROOM2.VIN_CALL_ROOM2"))
        (:NewEnumerator14
          (Variables|TempVariables|SetTempLocationCallSound_Vin "/Game/Audio/Dialog/Vincent/CUES/CALLS/VIN_CALL_ROOM3.VIN_CALL_ROOM3"))
        (:NewEnumerator15
          (Variables|TempVariables|SetTempLocationCallSound_Vin "/Game/Audio/Dialog/Vincent/CUES/CALLS/VIN_CALL_ROOM4.VIN_CALL_ROOM4"))
        (:NewEnumerator5
          (Variables|TempVariables|SetTempLocationCallSound_Vin "/Game/Audio/Dialog/Vincent/CUES/CALLS/VIN_CALL_RUINS.VIN_CALL_RUINS"))
        (:NewEnumerator6
          (Variables|TempVariables|SetTempLocationCallSound_Vin "/Game/Audio/Dialog/Vincent/CUES/CALLS/VIN_CALL_STUDY.VIN_CALL_STUDY"))
        (:NewEnumerator16
          (Variables|TempVariables|SetTempLocationCallSound_Vin "/Game/Audio/Dialog/Vincent/CUES/TANGENTS/VIN_TAN_WORSEPLACESBACKINLA.VIN_TAN_WORSEPLACESBACKINLA"))
        (:NewEnumerator8
          (Variables|TempVariables|SetTempLocationCallSound_Vin "/Game/Audio/Dialog/Vincent/CUES/CALLS/VIN_CALL_TUNNELS.VIN_CALL_TUNNELS"))
        (:NewEnumerator9
          (Variables|TempVariables|SetTempLocationCallSound_Vin "/Game/Audio/Dialog/Vincent/CUES/CALLS/VIN_CALL_ATTIC.VIN_CALL_ATTIC"))
        (:NewEnumerator10
          (Variables|TempVariables|SetTempLocationCallSound_Vin "/Game/Audio/Dialog/Vincent/CUES/CALLS/VIN_CALL_ATTICBLOCKED.VIN_CALL_ATTICBLOCKED"))
        (:NewEnumerator7
          (Variables|TempVariables|SetTempLocationCallSound_Vin "/Game/Audio/Dialog/Vincent/CUES/CALLS/VIN_CALL_SWITCHFOUND.VIN_CALL_SWITCHFOUND")))
      (CallFunction|Audio-FadePlayingforNew 0.075 (Variables|Default|GetVincent) (Variables|TempVariables|GetTempLocationCallSound_Vin) 1.75 false))))

(event Custom|DX_AFK
  ;[1 1 1] DX_AFK
  (if (<= (Variables|Default|GetPhase_Ref) 1)
    (CallFunction|DXIsThatUploaded)))

(event Custom|DX_ItemPickup
  (params (TriggerChance :type Float%20%28single-precision%29) (IsPlayer2 :type Boolean) (ItemName :type String) (DelayBeforeTrigger :type Float%20%28single-precision%29))
  ;[1 1 1] DX_ItemPickup
  (if (Variables|Default|GetDebugMode)
    (Development|PrintString (Utilities|String|Append "Item Name: " ItemName " 
Is Player 2: " (Utilities|String|ToString(Boolean) IsPlayer2) " 
Trigger Chance: " (Utilities|String|ToString(Float) TriggerChance) " 
Delay Before Trigger: " (Utilities|String|ToString(Float) DelayBeforeTrigger) " 
")))
  (if (|RandomChance TriggerChance) ; IfPassesChance...
    (Utilities|FlowControl|Delay DelayBeforeTrigger)
    (if IsPlayer2 ; Per Character
      (switch string ItemName ; Laveau
        (:Default
          (Variables|TempVariables|SetTempPickupCallSound_Lav 0))
        (:BP_Item_Consumable_Spray_C
          (Variables|TempVariables|SetTempPickupCallSound_Lav "/Game/Audio/Dialog/Laveau/CUES/CALLS/LAV_CALL_FOUNDSPRAY.LAV_CALL_FOUNDSPRAY"))
        (:BP_Item_Throwable_Matchbox_C
          (Variables|TempVariables|SetTempPickupCallSound_Lav "/Game/Audio/Dialog/Laveau/CUES/CALLS/LAV_CALL_FOUNDMATCHES.LAV_CALL_FOUNDMATCHES"))
        (:BP_Item_Consumable_LighterFluid_C
          (Variables|TempVariables|SetTempPickupCallSound_Lav "/Game/Audio/Dialog/Laveau/CUES/CALLS/LAV_CALL_FOUNDLIGHTERFLUID.LAV_CALL_FOUNDLIGHTERFLUID"))
        (:BP_Item_Consumable_Camera_C
          (Variables|TempVariables|SetTempPickupCallSound_Lav "/Game/Audio/Dialog/Laveau/CUES/CALLS/LAV_CALL_FOUNDCAMERA.LAV_CALL_FOUNDCAMERA" :!label _label))
        (:BP_Item_Consumable_Camcorder_C
          (goto _label))
        (:BP_Item_Throwable_AudioRecorder_C
          (Variables|TempVariables|SetTempPickupCallSound_Lav 0))
        (:BP_Item_CameraOnTripod_C
          (Variables|TempVariables|SetTempPickupCallSound_Lav "/Game/Audio/Dialog/Laveau/CUES/CALLS/LAV_CALL_FOUNDCAMERA.LAV_CALL_FOUNDCAMERA"))
        (:BP_Item_Consumable_HealthSyringe_C
          (Variables|TempVariables|SetTempPickupCallSound_Lav "/Game/Audio/Dialog/Laveau/CUES/CALLS/LAV_CALL_FOUNDHEAL.LAV_CALL_FOUNDHEAL"))
        (:BP_Item_Throwable_Voodoo_C
          (Variables|TempVariables|SetTempPickupCallSound_Lav "/Game/Audio/Dialog/Laveau/CUES/CALLS/LAV_CALL_FOUNDVOODOO.LAV_CALL_FOUNDVOODOO"))
        (:BP_Item_Throwable_Dynamite_C
          (Variables|TempVariables|SetTempPickupCallSound_Lav "/Game/Audio/Dialog/Laveau/CUES/CALLS/LAV_CALL_FOUNDDYNAMITE.LAV_CALL_FOUNDDYNAMITE")))
      (CallFunction|Audio-FadePlayingforNew 0.075 (Variables|Default|GetLaveau) (Variables|TempVariables|GetTempPickupCallSound_Lav) 1.75 false)
      (else
        (switch string ItemName ; Vincent
          (:Default
            (Variables|TempVariables|SetTempPickupCallSound_Vin "/Game/Audio/Dialog/Vincent/CUES/CALLS/VIN_CALL_FOUNDITEM.VIN_CALL_FOUNDITEM"))
          (:BP_Item_Consumable_Spray_C
            (Variables|TempVariables|SetTempPickupCallSound_Vin "/Game/Audio/Dialog/Vincent/CUES/CALLS/VIN_CALL_FOUNDSPRAY.VIN_CALL_FOUNDSPRAY"))
          (:BP_Item_Throwable_Matchbox_C
            (Variables|TempVariables|SetTempPickupCallSound_Vin "/Game/Audio/Dialog/Vincent/CUES/CALLS/VIN_CALL_FOUNDMATCHES.VIN_CALL_FOUNDMATCHES"))
          (:BP_Item_Consumable_LighterFluid_C
            (Variables|TempVariables|SetTempPickupCallSound_Vin "/Game/Audio/Dialog/Vincent/CUES/CALLS/VIN_CALL_FOUNDLIGHTERFLUID.VIN_CALL_FOUNDLIGHTERFLUID"))
          (:BP_Item_Consumable_Camera_C
            (Variables|TempVariables|SetTempPickupCallSound_Vin "/Game/Audio/Dialog/Vincent/CUES/CALLS/VIN_CALL_FOUNDCAMERA.VIN_CALL_FOUNDCAMERA" :!label _label_2))
          (:BP_Item_Consumable_Camcorder_C
            (goto _label_2))
          (:BP_Item_Throwable_AudioRecorder_C
            (Variables|TempVariables|SetTempPickupCallSound_Vin "/Game/Audio/Dialog/Vincent/CUES/CALLS/VIN_CALL_FOUNDAUDIODEVICE.VIN_CALL_FOUNDAUDIODEVICE"))
          (:BP_Item_CameraOnTripod_C
            (Variables|TempVariables|SetTempPickupCallSound_Vin "/Game/Audio/Dialog/Vincent/CUES/CALLS/VIN_CALL_FOUNDTRIPOD.VIN_CALL_FOUNDTRIPOD"))
          (:BP_Item_Consumable_HealthSyringe_C
            (Variables|TempVariables|SetTempPickupCallSound_Vin "/Game/Audio/Dialog/Vincent/CUES/CALLS/VIN_CALL_FOUNDITEM.VIN_CALL_FOUNDITEM"))
          (:BP_Item_Throwable_Voodoo_C
            (Variables|TempVariables|SetTempPickupCallSound_Vin "/Game/Audio/Dialog/Vincent/CUES/CALLS/VIN_CALL_FOUNDVOODOO.VIN_CALL_FOUNDVOODOO"))
          (:BP_Item_Throwable_Dynamite_C
            (Variables|TempVariables|SetTempPickupCallSound_Vin "/Game/Audio/Dialog/Vincent/CUES/CALLS/VIN_CALL_FOUNDDYNAMITE.VIN_CALL_FOUNDDYNAMITE")))
        (CallFunction|Audio-FadePlayingforNew 0.075 (Variables|Default|GetVincent) (Variables|TempVariables|GetTempPickupCallSound_Vin) 1.75 false)))))

(event Custom|DX_PlayGivenLine
  (params (IsPlayer2 :type Boolean) (Given%20Sound%20Cue :type Sound%20Base%20Object%20Reference))
  ;[1 1 1] DX_PlayGivenLine
  (if IsPlayer2
    (CallFunction|Audio-FadePlayingforNew 0.075 (Variables|Default|GetLaveau) Given%20Sound%20Cue 1.75 false)
    (else
      (CallFunction|Audio-FadePlayingforNew 0.075 (Variables|Default|GetVincent) Given%20Sound%20Cue 1.75 false))))

(event Custom|DX_ItemUse
  (params (TriggerChance :type Float%20%28single-precision%29) (IsPlayer2 :type Boolean) (ItemName :type String) (DelayBeforeTrigger :type Float%20%28single-precision%29))
  ;[1 1 1] DX_ItemUse
  (if (Variables|Default|GetDebugMode)
    (Development|PrintString (Utilities|String|Append "Item Name: " ItemName " 
Is Player 2: " (Utilities|String|ToString(Boolean) IsPlayer2) " 
Trigger Chance: " (Utilities|String|ToString(Float) TriggerChance) " 
Delay Before Trigger: " (Utilities|String|ToString(Float) DelayBeforeTrigger) " 
")))
  (if (|RandomChance_2 TriggerChance) ; IfPassesChance...
    (Utilities|FlowControl|Delay DelayBeforeTrigger)
    (if IsPlayer2 ; Per Character
      (switch string ItemName ; Laveau
        (:BP_Item_Consumable_HealthSyringe_C
          (Variables|TempVariables|SetTempUseCallSound_Lav "/Game/Audio/Dialog/Laveau/CUES/CALLS/LAV_CALL_HEALING.LAV_CALL_HEALING")
          (CallFunction|Audio-FadePlayingforNew 0.075 (Variables|Default|GetLaveau) (Variables|TempVariables|GetTempUseCallSound_Lav) 1.75 false)))
      (else
        (switch string ItemName ; Vincent
          (:BP_Item_Consumable_HealthSyringe_C
            (Variables|TempVariables|SetTempUseCallSound_Vin "/Game/Audio/Dialog/Vincent/CUES/CALLS/VIN_CALL_HEALING.VIN_CALL_HEALING")
            (CallFunction|Audio-FadePlayingforNew 0.075 (Variables|Default|GetVincent) (Variables|TempVariables|GetTempUseCallSound_Vin) 1.75 false)))))))

(event Custom|DX_Death
  (params (IsPlayer2 :type Boolean))
  ;[1 1 1] Death & Downed
  (CallFunction|Audio-PlaybyCharacter IsPlayer2 "/Game/Audio/Dialog/Laveau/CUES/EFFORTS/LAV_EF_DAMAGE.LAV_EF_DAMAGE" "/Game/Audio/Dialog/Vincent/CUES/CALLS/VIN_CALL_DEATH.VIN_CALL_DEATH" true))

(event Custom|DX_BreakerBoxFail
  (params (IsPlayer2 :type Boolean))
  ;[1 1 1] DX_BreakerBox
  (CallFunction|Audio-PlaybyCharacter IsPlayer2 "/Game/Audio/Dialog/Laveau/CUES/CALLS/LAV_CALL_SWITCHFAILED.LAV_CALL_SWITCHFAILED" "/Game/Audio/Dialog/Vincent/CUES/CALLS/VIN_CALL_SWITCHSUCCEED.VIN_CALL_SWITCHSUCCEED" false))

(event Custom|DX_BreakerBoxSuccess
  (params (IsPlayer2 :type Boolean))
  ;[1 1 1] DX_BreakerBox
  (CallFunction|Audio-PlaybyCharacter IsPlayer2 "/Game/Audio/Dialog/Laveau/CUES/CALLS/LAV_FOUND_SWITCHSUCCEED.LAV_FOUND_SWITCHSUCCEED" "/Game/Audio/Dialog/Vincent/CUES/CALLS/VIN_CALL_SWITCHSUCCEED.VIN_CALL_SWITCHSUCCEED" false))

(event Custom|Set_GamePhase
  (params (Phase :type Integer))
  (Variables|Default|SetPhase_Ref Phase))

(event Custom|DX_IsThatUploaded
  ;[1 1 1] DX_IsThatUploaded
  (Utilities|FlowControl|DoOnce false
    (:Completed
      (CallFunction|Audio-FadePlayingforNew 0.075 (Variables|Default|GetProducer) "/Game/Audio/Dialog/Producer/dx_pro_ISTHATUPLOADED.dx_pro_ISTHATUPLOADED" 1.75 true))))

(event Custom|DX_GameStart
  ;[1 1 1] DX_GameStart
  (Utilities|FlowControl|DoOnce false
    (:Completed
      (Utilities|FlowControl|Delay 2.5)
      (CallFunction|Audio-FadePlayingforNew 0.075 (Variables|Default|GetProducer) "/Game/Audio/Dialog/Producer/dx_pro_THATSAWRAP.dx_pro_THATSAWRAP" 1.75 true)
      (CallFunction|Audio-PlaybyPlayerCount "/Game/Audio/Dialog/Laveau/CUES/TANGENTS/Lav_StartingTangent.Lav_StartingTangent" 0 false 5e+01))))

(event Custom|Set_PlayerCount
  (params (PlayerCount :type Integer))
  (Variables|Default|SetPlayerCount PlayerCount))

(event Custom|DX_Downed
  (params (IsPlayer2 :type Boolean))
  ;[1 1 1] Death & Downed
  (CallFunction|Audio-PlaybyCharacter IsPlayer2 "/Game/Audio/Dialog/Laveau/CUES/CALLS/LAV_CALL_DOWNED.LAV_CALL_DOWNED" "/Game/Audio/Dialog/Vincent/CUES/CALLS/VIN_CALL_DOWNED.VIN_CALL_DOWNED" true))

(event EventBeginPlay
  ;[1 1 1] Event BeginPlay
  (if (Variables|Default|GetPlayStart)
    (CallFunction|DXGameStart)
    (bind _asgame_instance_the_wtd (Utilities|Casting|CastToGameInstance_TheWTD (Game|GetGameInstance)))
    (bind _output_get (Variables|Default|SetPlayerCount (Variables|/Game/Blueprints/GameInstance_TheWTD.GameInstance_TheWTD_C|GetDesiredNoOfPlayers _asgame_instance_the_wtd)))
    (Math|Integer|IncrementInt _output_get)))

(fn ConstructionScript)

(fn Audio-FadePlayingforNew
  (params (FadeOutDuration :type Float%20%28single-precision%29) (AudioComponent :type Audio%20Component%20Object%20Reference%20%28by%20ref%29) (New%20Sound :type Sound%20Base%20Object%20Reference) (End%20Multiplier :type Float%20%28single-precision%29) (IgnoreProducer :type Boolean))
  (if IgnoreProducer ; Play while Producer does. Producer must ignore himself
    (Utilities|IsValid New%20Sound :!label _label ; If the new sound has a value...
      (:Is%20Valid
        (if (Audio|Components|Audio|IsPlaying AudioComponent)
          (Audio|Components|Audio|FadeOut AudioComponent FadeOutDuration 0.0 "Linear" :!class /Script/Engine.AudioComponent)
          (Audio|Components|Audio|StopDelayed AudioComponent (* FadeOutDuration End%20Multiplier)))
        (Audio|Components|Audio|SetSound AudioComponent New%20Sound)
        (Audio|Components|Audio|Play AudioComponent 0.0)))
    (elif (not (Audio|Components|Audio|IsPlaying (Variables|Default|GetProducer))) ; If Producer is speaking, don't bother
      (goto _label))))

(fn Audio-PlaybyCharacter
  (params (IsPlayer2 :type Boolean) (LaveauLine :type Sound%20Base%20Object%20Reference) (VincentLine :type Sound%20Base%20Object%20Reference) (IgnoreProducer :type Boolean))
  (if IsPlayer2
    (CallFunction|Audio-FadePlayingforNew 0.075 (Variables|Default|GetLaveau) LaveauLine 1.75 IgnoreProducer)
    (else
      (CallFunction|Audio-FadePlayingforNew 0.075 (Variables|Default|GetVincent) VincentLine 1.75 IgnoreProducer))))

(fn Audio-PlaybyPlayerCount
  (params (Laveau%20Line :type Sound%20Base%20Object%20Reference) (Vincent%20Line :type Sound%20Base%20Object%20Reference) (Ignore%20Producer :type Boolean) (PercentChanceOfVincent :type Float%20%28single-precision%29))
  (if (> (Variables|Default|GetPlayerCount) 1) ; If only one player, default to Vincent
    (if (<= (* (Math|Random|RandomFloat) 1e+02) PercentChanceOfVincent) ; Chose between Vin and Lav
      (CallFunction|Audio-PlaybyCharacter false Laveau%20Line Vincent%20Line Ignore%20Producer :!label _label) ; Vincent
      (else
        (CallFunction|Audio-PlaybyCharacter true Laveau%20Line Vincent%20Line Ignore%20Producer) ; Laveau
      ))
    (else
      (goto _label))))