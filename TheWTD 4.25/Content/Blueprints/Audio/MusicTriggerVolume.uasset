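; Trigger volume that asks the level's SoundController to play music when something overlaps its box.
; An overlap rolls against TriggerChance, and a pass waits briefly before sending MXEnum to the controller if PlayFromEnum is set.
; A failed roll or retriggerable success starts a cooldown between attempts, while a DoOnce limits non-retriggerable volumes to one trigger.
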(event OnComponentBeginOverlap(Box)
  (params (OverlappedComponent :type Primitive%20Component%20Object%20Reference) (OtherActor :type Actor%20Object%20Reference) (OtherComp :type Primitive%20Component%20Object%20Reference) (OtherBodyIndex :type Integer) (bFromSweep :type Boolean) (SweepResult :type Hit%20Result%20Structure%20%28by%20ref%29))
  (if (Variables|Default|GetCanAttempt)
    (if (<= (* (Math|Random|RandomFloat) 1e+02) (Variables|Default|GetTriggerChance)) ; If chance threshold met...
      (if (Variables|Default|GetCanRetrigger) ; If not retriggerable, only do it once...
        (CallFunction|CanAttemptEvent)
        (else
          (Utilities|FlowControl|DoOnce false
            (:Completed
              _))))
      (Utilities|FlowControl|Delay (Variables|Default|GetDelayBeforeTrigger)) ; Slight delay
      (if (Variables|Default|GetPlayFromEnum?) ; Enum is standard
        (Default|MXfromTrigger (Variables|Default|GetSoundController_Ref) (Variables|Default|GetMX_Enum)))
      (else
        (CallFunction|CanAttemptEvent)))))

(event Custom|CanAttempt_Event
  (Variables|Default|SetCanAttempt false) ; Keeps from being triggered repeatedly
  (Utilities|FlowControl|Delay (Variables|Default|GetDelayBetweenAttempts))
  (Variables|Default|SetCanAttempt true))

(event EventBeginPlay
  (bind _returnvalue (Actor|GetActorOfClass "/Game/Blueprints/Audio/SoundController.SoundController_C"))
  (Variables|Default|SetSoundController_Ref _returnvalue))

(fn ConstructionScript)