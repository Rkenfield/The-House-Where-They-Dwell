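; Dialogue trigger volume that plays location-based voice lines for Vincent or Laveau when their player character overlaps its box.
; Overlaps pass a random chance check, an optional DoOnce gate for non-retriggerable volumes, and a short delay.
; A switch on the overlapping actor's class display name picks the character.
; It sends the location enum to DXController, found on BeginPlay, or plays that character's assigned 2D sound directly.
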(event OnComponentBeginOverlap(Box)
  (params (OverlappedComponent :type Primitive%20Component%20Object%20Reference) (OtherActor :type Actor%20Object%20Reference) (OtherComp :type Primitive%20Component%20Object%20Reference) (OtherBodyIndex :type Integer) (bFromSweep :type Boolean) (SweepResult :type Hit%20Result%20Structure%20%28by%20ref%29))
  (bind _returnvalue (Utilities|GetClass OtherActor))
  (bind _locationenum (Variables|Default|GetLocationEnum))
  (bind _dxcontrollerref (Variables|Default|GetDXControllerRef))
  (bind _returnvalue_2 (Utilities|GetClassDisplayName _returnvalue))
  (if (<= (* (Math|Random|RandomFloat) 1e+02) (Variables|Default|GetTriggerChance)) ; If chance threshold met...
    (if (Variables|Default|GetCanRetrigger) ; If not retriggerable, only do it once...
      _
      (else
        (Utilities|FlowControl|DoOnce false
          (:Completed
            _))))
    (Utilities|FlowControl|Delay (Variables|Default|GetDelayBeforeTrigger)) ; Slight delay
    (if (Variables|Default|GetPlayFromEnum?) ; Enum is standard
      (switch string _returnvalue_2 ; Cast to DXController
        (:BP_PlayerChild1
          (Default|DXLocationCall _dxcontrollerref false _locationenum) ; Vincent
        )
        (:BP_PlayerChild2
          (Default|DXLocationCall _dxcontrollerref true _locationenum) ; Laveau
        ))
      (else
        (switch string _returnvalue_2 ; Play from here (just in case)
          (:BP_PlayerChild1
            (Audio|PlaySound2D (Variables|Audio|GetVincentLine) 1.0 1.0 0.0 0 0))
          (:BP_PlayerChild2
            (Audio|PlaySound2D (Variables|Audio|GetLaveauLine) 1.0 1.0 0.0 0 0)))))))

(event EventBeginPlay
  (bind _returnvalue (Actor|GetActorOfClass "/Game/Blueprints/Audio/DXController.DXController_C"))
  (Variables|Default|SetDXControllerRef _returnvalue))

(fn ConstructionScript)