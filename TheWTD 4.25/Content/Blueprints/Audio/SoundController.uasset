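; SoundController directs the game's music and ambience, applying the house base sound mix and starting the ambient bed and game-start cue on BeginPlay.
; After a delay it fades in AmbientMusic, whose Amb_Mode parameter a timeline crossfades toward danger and reverses for calm.
; Other events play the next-phase cue, add a score for high danger, or quickly fade out all five audio components.
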(event Custom|MX_Amb_Start
  (bind _ambientmusic (Variables|Default|GetAmbientMusic))
  (Audio|Parameter|SetFloatParameter _ambientmusic "Amb_Mode" 0.0 :!class /Script/Engine.AudioComponent)
  (Audio|Components|Audio|FadeIn _ambientmusic 2.5 1.0 0.0 "Sin" :!class /Script/Engine.AudioComponent))

(event Custom|MX_Amb_Danger
  (bind _crossfade_value (Timeline|Crossfade Play)
    (:Update
      (Audio|Parameter|SetFloatParameter (Variables|Default|GetAmbientMusic) "Amb_Mode" _crossfade_value :!class /Script/Engine.AudioComponent))))

(event Custom|MX_Amb_Calm
  (bind _crossfade_value (Timeline|Crossfade Reverse)
    (:Update
      (Audio|Parameter|SetFloatParameter (Variables|Default|GetAmbientMusic) "Amb_Mode" _crossfade_value :!class /Script/Engine.AudioComponent))))

(event Custom|MX_Game_Start
  (Audio|Components|Audio|Play (Variables|Default|GetGameStart) 0.0)
  (Utilities|FlowControl|Delay 9.0)
  (CallFunction|MXAmbStart))

(event Custom|MX_Game_NextPhase
  (Audio|Components|Audio|Play (Variables|Default|GetGameNextPhase) 0.0))

(event Custom|MX_Amb_HighDanger
  (Audio|Components|Audio|Play (Variables|Default|GetAmbientScore) 0.0)
  (CallFunction|MXAmbDanger))

(event Custom|MX_StopAll
  (Audio|Components|Audio|FadeOut (Variables|Default|GetAmbientBase) 0.25 0.0 "Linear" :!class /Script/Engine.AudioComponent)
  (Audio|Components|Audio|FadeOut (Variables|Default|GetAmbientMusic) 0.25 0.0 "Linear" :!class /Script/Engine.AudioComponent)
  (Audio|Components|Audio|FadeOut (Variables|Default|GetAmbientScore) 0.25 0.0 "Linear" :!class /Script/Engine.AudioComponent)
  (Audio|Components|Audio|FadeOut (Variables|Default|GetGameStart) 0.25 0.0 "Linear" :!class /Script/Engine.AudioComponent)
  (Audio|Components|Audio|FadeOut (Variables|Default|GetGameNextPhase) 0.25 0.0 "Linear" :!class /Script/Engine.AudioComponent))

(event EventBeginPlay
  (Class|GameplayStatics|SetBaseSoundMix "/Game/Audio/SoundClasses/BaseMix_House.BaseMix_House")
  (Audio|Components|Audio|Play (Variables|Default|GetAmbientBase) 0.0)
  (CallFunction|MXGameStart))

(fn ConstructionScript)