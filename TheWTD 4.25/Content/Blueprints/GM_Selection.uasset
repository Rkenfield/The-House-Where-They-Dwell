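; Game mode for the character selection screen, which sets up four local players and starts the level once four selections are made.
; BeginPlay resets the Game Instance's character indices, disables splitscreen and creates the players.
; Join possesses each controller's selector by controller ID and points player 0's view at a camera actor.
; Selection stores choices in the Game Instance and opens SaisLevel when the count reaches four.
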(event Custom|Join
  (params (Controller :type Player%20Controller%20Object%20Reference))
  (bind _returnvalue (Class|GameplayStatics|GetPlayerControllerID Controller))
  (bind _selectors (Variables|Default|GetSelectors))
  (bind _output (Utilities|Array|Get(acopy) _selectors _returnvalue))
  ;[1 1 1] Join Game event to assign controller to selector.
  (Pawn|Possess Controller _output)
  (Default|Selecting _output)
  (bind _returnvalue_2 (Actor|GetActorOfClass "/Script/Engine.CameraActor"))
  (Game|Player|SetViewTargetwithBlend (Game|GetPlayerController 0) _returnvalue_2 0.0 "VTBlend_Linear" 0.0 false))

(event Custom|Selection
  (params (Controller :type Player%20Controller%20Object%20Reference) (Selection :type Integer))
  ;[1 1 1] Assign Selection to Game Instance
  (bind _asgame_instance_the_wtd (Utilities|Casting|CastToGameInstance_TheWTD (Game|GetGameInstance)))
  (Utilities|Array|SetArrayElem (Variables|/Game/Blueprints/GameInstance_TheWTD.GameInstance_TheWTD_C|GetCharacterIndex _asgame_instance_the_wtd) (Class|GameplayStatics|GetPlayerControllerID Controller) Selection)
  (bind _output_get (Variables|Default|SetSelectionCount (+ (Variables|Default|GetSelectionCount) 1)))
  (Development|PrintString (Utilities|String|ToString(Integer) _output_get))
  (if (== _output_get 4)
    (Game|OpenLevel(byName) "SaisLevel")))

(event EventBeginPlay
  ;[1 1 1] Create players and initalize values.
  (bind _asgame_instance_the_wtd (Utilities|Casting|CastToGameInstance_TheWTD (Game|GetGameInstance)))
  (for (_ _array_index) (Variables|/Game/Blueprints/GameInstance_TheWTD.GameInstance_TheWTD_C|GetCharacterIndex _asgame_instance_the_wtd)
    (Utilities|Array|SetArrayElem (Variables|/Game/Blueprints/GameInstance_TheWTD.GameInstance_TheWTD_C|GetCharacterIndex _asgame_instance_the_wtd) _array_index -1)
    (Class|GameplayStatics|SetForceDisableSplitscreen true)
    (for _index (range 0 3)
      (Class|GameplayStatics|CreatePlayer _index))))

(fn ConstructionScript)