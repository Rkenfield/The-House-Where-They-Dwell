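; Game mode for a local split-screen game that handles player setup, phase progression and level lighting.
; StartGame creates local players from the game instance's desired count and possesses characters chosen in saved character data.
; Phase events reveal nests, open doors, break the lair barrier, start attic minion spawns and cue music.
; LightsOff/LightsOn toggle OnOff-tagged lights; spider witch, win-menu and item-spawn logic is disconnected.
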(event Custom|SpawnCharacters
  ;[1 1 1] Edited by Alex 11-23-20: Creates number of players specified at main menu.
  ;;[1 1 1] Alex: Spawning characters
  (if (== (Variables|/Game/Blueprints/GameInstance_TheWTD.GameInstance_TheWTD_C|GetDesiredNoOfPlayers (Variables|Default|GetGameInstance)) 0)
    (Game|SpawnActorfromClass "/Game/Blueprints/Characters/BP_PlayerChild1.BP_PlayerChild1_C" (Variables|Default|GetTempSpawn1) "Undefined" 0 0)
    (else
      (Game|SpawnActorfromClass "/Game/Blueprints/Characters/BP_PlayerChild1.BP_PlayerChild1_C" (Variables|Default|GetTempSpawn1) "Undefined" 0 0)
      (Game|SpawnActorfromClass "/Game/Blueprints/Characters/BP_PlayerChild2.BP_PlayerChild2_C" (Variables|Default|GetTempSpawn2) "Undefined" 0 0))))

(event Custom|SpawnPlayer
  (params (Controller :type Player%20Controller%20Object%20Reference))
  (bind _returnvalue (Class|GameplayStatics|GetPlayerControllerID Controller))
  (bind _returnvalue_2 (Game|GetPlayerController _returnvalue))
  ;[1 1 1] SpawnPlayer- Allows each player to take control of one of the playable characters when either '1' (keyboard) or 'Special Left Button' (Gamepad) is pressed
  (Utilities|IsValid (Pawn|GetControlledPawn Controller)
    (:Is%20Valid
      (bind _charindex (Class|BPIGameInstance|LoadCharData(Message) (Game|GetGameInstance)))
      (bind _returnvalue_3 (Actor|GetActorOfClass (Utilities|Select :Index (Utilities|Array|Get(acopy) _charindex _returnvalue) :Option%200 (Variables|Default|GetPlayer1) :Option%201 (Variables|Default|GetPlayer2) :Option%202 (Variables|Default|GetPlayer3) :Option%203 (Variables|Default|GetPlayer4))))
      (Utilities|IsValid _returnvalue_2
        (:Is%20Valid
          (Pawn|Possess _returnvalue_2 _returnvalue_3))))))

(event Custom|SetPhase2
  (bind _sound_controller (Variables|Default|GetSound%20Controller))
  ;[1 1 1] Setting Phase 2
  (Variables|Default|SetCurrentPhase 2)
  (bind _outactors (Actor|GetAllActorsOfClass "/Game/Blueprints/Blueprints/BP_Nest.BP_Nest_C"))
  (for _array_element _outactors
    (Development|SetHiddeninGame (Variables|/Game/Blueprints/Blueprints/BP_Nest.BP_Nest_C|GetMesh _array_element) false false)
    (Collision|SetCollisionEnabled (Variables|/Game/Blueprints/Blueprints/BP_Nest.BP_Nest_C|GetSphere _array_element) "QueryAndPhysics"))
  (bind _outactors_2 (Actor|GetAllActorsOfClass "/Game/Blueprints/Blueprints/BP_Door_Downstairs.BP_Door_Downstairs_C"))
  (for _array_element_2 _outactors_2
    (Default|OpenDownstairsDoors _array_element_2))
  (Default|MXGameNextPhase _sound_controller)
  (Default|MXAmbDanger _sound_controller))

(event Custom|SetPhase3
  (bind _sound_controller (Variables|Default|GetSound%20Controller))
  ;[1 1 1] Phase 3
  ;;[1 1 1] Setting Phase 3
  (Variables|Default|SetCurrentPhase 3)
  (Default|MXGameNextPhase _sound_controller)
  (Default|MXAmbCalm _sound_controller)
  ;;;[1 1 1] Destroys the barrier to the spider witch lair.
  (bind _outactors (Actor|GetAllActorsOfClass "/Game/Blueprints/LevelGeneration/Room_SWLair.Room_SWLair_C"))
  (bind _array_element (Utilities|Array|ForEachLoopwithBreak _outactors)
    (:LoopBody
      (Default|DestroyBarrier _array_element))
    (:Completed
      (bind _outactors_2 (Actor|GetAllActorsOfClasswithTag "/Game/Blueprints/Blueprints/BP_Nest.BP_Nest_C" "AtticNest"))
      (bind _array_element_2 (Utilities|Array|ForEachLoopwithBreak _outactors_2)
        (:LoopBody
          (Default|StartSpiderMinionSpawn _array_element_2))))))

(event Custom|StartSpiderWitch
  ;[1 1 1] Phase 3
  ;;[1 1 1] Starting Spider Witch
)

(event Custom|SetPhase4
  ;[1 1 1] SetPhase4
  (Variables|Default|SetCurrentPhase 4))

(event EventStartGame
  ;[1 1 1] Edited by Alex 11-23-20: Creates number of players specified at main menu.
  ;;[1 1 1] Alex: Originally was Event BeginPlay (for the sake of my main menu level).
  (Class|GameplayStatics|SetForceDisableSplitscreen false)
  (while (<= (Variables|Default|GetNoOfPlayers) (Variables|/Game/Blueprints/GameInstance_TheWTD.GameInstance_TheWTD_C|GetDesiredNoOfPlayers (Variables|Default|GetGameInstance)))
    (bind _returnvalue (Class|GameplayStatics|CreatePlayer (Variables|Default|GetNoOfPlayers)))
    (Variables|Default|SetNoOfPlayers (+ (Variables|Default|GetNoOfPlayers) 1)))
  (bind _charindex (Class|BPIGameInstance|LoadCharData(Message) (Game|GetGameInstance)))
  (for (_array_element _array_index) _charindex
    (bind _returnvalue_2 (Actor|GetActorOfClass (Utilities|Select :Index _array_element :Option%200 (Variables|Default|GetPlayer1) :Option%201 (Variables|Default|GetPlayer2) :Option%202 (Variables|Default|GetPlayer3) :Option%203 (Variables|Default|GetPlayer4))))
    (Utilities|IsValid (Game|GetPlayerController _array_index)
      (:Is%20Valid
        (Pawn|Possess (Game|GetPlayerController _array_index) _returnvalue_2)))))

(event EventBeginPlay
  ;[1 1 1] EventBeginPlay
  (bind _asgame_instance_the_wtd (Utilities|Casting|CastToGameInstance_TheWTD (Game|GetGameInstance)))
  (Variables|Default|SetGameInstance _asgame_instance_the_wtd)
  (Utilities|FlowControl|Delay 0.5)
  (bind _returnvalue (Actor|GetActorOfClass "/Game/Blueprints/Audio/SoundController.SoundController_C"))
  (Variables|Default|SetSound%20Controller _returnvalue))

(fn ConstructionScript)

(fn LightsOff
  (Utilities|FlowControl|Sequence
    (:then_0
      ;[1 1 1] All lights in the level with tag OnOff
      (bind _outactors (Actor|GetAllActorsOfClasswithTag "/Script/Engine.Light" "OnOff"))
      (for _array_element _outactors
        (Rendering|SetVisibility (Variables|/Script/Engine.Light|GetLightComponent _array_element) false false)))
    (:then_1
      ;[1 1 1] Chandelier lights with tag OnOff
      (bind _outactors_2 (Actor|GetAllActorsOfClass "/Game/Blueprints/Blueprints/Chadelier.Chadelier_C"))
      (for _array_element_2 _outactors_2
        (for _array_element_3 (Actor|GetComponentsbyTag _array_element_2 "/Script/Engine.LightComponent" "OnOff")
          (Rendering|SetVisibility _array_element_3 false false))))
    (:then_2
      ;[1 1 1] All lights in the rooms bps with tag OnOff
      (bind _outactors_3 (Actor|GetAllActorsOfClass "/Game/Blueprints/LevelGeneration/RoomParent.RoomParent_C"))
      (for _array_element_4 _outactors_3
        (for _array_element_5 (Actor|GetComponentsbyTag _array_element_4 "/Script/Engine.LightComponent" "OnOff")
          (Rendering|SetVisibility _array_element_5 false false))))
    (:then_3
      ;[1 1 1] Computer station lights with tag OnOff
      (bind _outactors_4 (Actor|GetAllActorsOfClass "/Game/Blueprints/Blueprints/BP_ComputerStation.BP_ComputerStation_C"))
      (for _array_element_6 _outactors_4
        (for _array_element_7 (Actor|GetComponentsbyTag _array_element_6 "/Script/Engine.LightComponent" "OnOff")
          (Rendering|SetVisibility _array_element_7 false false))))))

(fn Lightson
  (Utilities|FlowControl|Sequence
    (:then_0
      ;[1 1 1] All lights in the level with tag OnOff
      (bind _outactors (Actor|GetAllActorsOfClasswithTag "/Script/Engine.Light" "OnOff"))
      (for _array_element _outactors
        (Rendering|SetVisibility (Variables|/Script/Engine.Light|GetLightComponent _array_element) true false)))
    (:then_1
      ;[1 1 1] Chandelier lights with tag OnOff
      (bind _outactors_2 (Actor|GetAllActorsOfClass "/Game/Blueprints/Blueprints/Chadelier.Chadelier_C"))
      (for _array_element_2 _outactors_2
        (for _array_element_3 (Actor|GetComponentsbyTag _array_element_2 "/Script/Engine.LightComponent" "OnOff")
          (Rendering|SetVisibility _array_element_3 true false))))
    (:then_2
      ;[1 1 1] All lights in the rooms bps with tag OnOff
      (bind _outactors_3 (Actor|GetAllActorsOfClass "/Game/Blueprints/LevelGeneration/RoomParent.RoomParent_C"))
      (for _array_element_4 _outactors_3
        (for _array_element_5 (Actor|GetComponentsbyTag _array_element_4 "/Script/Engine.LightComponent" "OnOff")
          (Rendering|SetVisibility _array_element_5 true false))))
    (:then_3
      ;[1 1 1] Computer station lights with tag OnOff
      (bind _outactors_4 (Actor|GetAllActorsOfClass "/Game/Blueprints/Blueprints/BP_ComputerStation.BP_ComputerStation_C"))
      (for _array_element_6 _outactors_4
        (for _array_element_7 (Actor|GetComponentsbyTag _array_element_6 "/Script/Engine.LightComponent" "OnOff")
          (Rendering|SetVisibility _array_element_7 true false))))))