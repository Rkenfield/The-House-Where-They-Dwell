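; Game mode for test levels that sets up local multiplayer with a configurable tester player count.
; On BeginPlay it writes the desired count to the game instance, allows splitscreen and creates local players with controllers in a loop.
; It then reads character data from the game instance, maps each entry to one of four player classes and has the matching controller possess that class's actor in the level.
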(event EventBeginPlay
  (|CallParentFunction)
  (Variables|/Game/Blueprints/GameInstance_TheWTD.GameInstance_TheWTD_C|SetDesiredNoOfPlayers (Variables|Default|GetGameInstance) (- (Variables|Default|GetTesterPlayerCount) 1))
  (Class|GameplayStatics|SetForceDisableSplitscreen false)
  (while (<= (Variables|Default|GetNoOfPlayers) (Variables|/Game/Blueprints/GameInstance_TheWTD.GameInstance_TheWTD_C|GetDesiredNoOfPlayers (Variables|Default|GetGameInstance)))
    (bind _returnvalue (Class|GameplayStatics|CreatePlayer (Variables|Default|GetNoOfPlayers)))
    (Variables|Default|SetNoOfPlayers (+ (Variables|Default|GetNoOfPlayers) 1)))
  (bind _charindex (Class|BPIGameInstance|LoadCharData(Message) (Game|GetGameInstance)))
  (for (_array_element _array_index) _charindex
    (bind _returnvalue_2 (Actor|GetActorOfClass (Utilities|Select :Index _array_element :Option%200 (Variables|Default|GetPlayer1) :Option%201 (Variables|Default|GetPlayer2) :Option%202 (Variables|Default|GetPlayer3) :Option%203 (Variables|Default|GetPlayer4))))
    (Utilities|IsValid (Game|GetPlayerController _array_index)
      (:Is%20Valid
        (Pawn|Possess (Game|GetPlayerController _array_index) _returnvalue_2)))))

(event EventTick
  (params (DeltaSeconds :type Float%20%28single-precision%29)))

(fn ConstructionScript
  (|CallParentFunction))