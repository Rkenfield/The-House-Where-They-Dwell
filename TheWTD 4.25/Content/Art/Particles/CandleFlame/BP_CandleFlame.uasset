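; BP_CandleFlame is a candle flame actor that pairs a particle system with a flickering point light.
; On BeginPlay, the CandleFlame_Flicker timeline drives the light's intensity by lerping between MinIntensity and MaxIntensity.
; SetEnabled stores the Enabled flag and toggles visibility of the light and particles, and the construction script applies it.
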(event EventBeginPlay
  (bind _intensity (Timeline|CandleFlame_Flicker Play)
    (:Update
      (Rendering|Components|Light|SetIntensity (Variables|Default|GetPointLight) (Math|Float|Lerp (Variables|Default|GetMinIntensity) (Variables|Default|GetMaxIntensity) _intensity)))))

(event Collision|EventActorBeginOverlap
  (params (OtherActor :type Actor%20Object%20Reference)))

(event EventTick
  (params (DeltaSeconds :type Float%20%28single-precision%29)))

(fn ConstructionScript
  (CallFunction|SetEnabled (Variables|Default|GetEnabled)))

(fn SetEnabled
  (params (Enabled :type Boolean))
  (bind _output_get (Variables|Default|SetEnabled Enabled))
  (Rendering|SetVisibility (Variables|Default|GetPointLight) _output_get false)
  (Rendering|SetVisibility (Variables|Default|GetParticleSystem) _output_get false))